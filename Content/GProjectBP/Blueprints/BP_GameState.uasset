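; GameState for a level that holds its difficulty, spawnable enemy and item lists, and mission objectives.
; LevelInitialize copies the level tree from the GameInstance, filters character and item DataTables by difficulty, and registers each Mission map node as an objective.
; UpdateMissionProgress completes the first open objective of the given type and calls GameMode MissionComplete on authority when none remain.
; Multicast-named events push objective changes to the HUD through player controller 0.
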(event `Level Initialize`
  (params (DifficultiyOfLevel :type Integer))
  (set `self.DifficultiyOfLevel` DifficultiyOfLevel)
  (set `self.ServerLevelTree` (`/Game/GProjectBP/Blueprints/BP_GameInstance.LevelTree` (cast `/Game/GProjectBP/Blueprints/BP_GameInstance` (`GameplayStatics.GetGameInstance`) :!pure true)))
  (`self.Initialize Spawnable Enemy List`)
  (`self.Initialize Spawnable Item List`)
  (for (_array_element _array_index) (`self.ServerLevelTree`)
    (bind _returnvalue (`KismetStringLibrary.Conv_NameToString` (`.MapType` (break `GPMapData` (`.MapData` (break `GPLevelNode` _array_element))))))
    (if (`KismetStringLibrary.StartsWith` _returnvalue "MIssion")
      (bind (_lefts _rights) (`KismetStringLibrary.Split` _returnvalue "_"))
      (`BlueprintMapLibrary.Map_Add` (`self.MissionObject`) _array_index (make `/Game/GProjectBP/Blueprints/MissionStruct` _rights))
      (`self.Multicast Missiom HUD Add` _rights)
      (`/Engine/EditorBlueprintResources/StandardMacros.IncrementInt` (`self.RemainObject`)))))

(event `Multicast Missiom HUD Add`
  (params (Object :type String))
  (`/Game/GProjectBP/Blueprints/BP_PlayerController_Game.Initialize Mission Object HUD` (cast `/Game/GProjectBP/Blueprints/BP_PlayerController_Game` (`GameplayStatics.GetPlayerController` 0) :!pure true) Object))

(event `Multicast Missiom HUD Update`
  (params (inType :type String) (Progress :type "Float (double-precision)") (Complete :type Boolean))
  (`/Game/GProjectBP/Blueprints/BP_PlayerController_Game.Update Mission Object HUD` (cast `/Game/GProjectBP/Blueprints/BP_PlayerController_Game` (`GameplayStatics.GetPlayerController` 0) :!pure true) inType Progress Complete)
  (`KismetSystemLibrary.PrintString` "gs update"))

(event `Update Mission Progress`
  (params (MissionType :type String))
  (bind _missionobject (`self.MissionObject`))
  (bind _values (`BlueprintMapLibrary.Map_Values` (`self.MissionObject`)))
  (for (_array_element _array_index) _values
    (bind (_type _bissuccess) (break `/Game/GProjectBP/Blueprints/MissionStruct` _array_element))
    (if (and (`KismetStringLibrary.EqualEqual_StrStr` _type MissionType) (!= _bissuccess true))
      (bind _keys (`BlueprintMapLibrary.Map_Keys` (`self.MissionObject`)))
      (bind _output (`|GetArrayItem` _keys _array_index))
      (bind (_type_2 _bissuccess_2 _progress) (break `/Game/GProjectBP/Blueprints/MissionStruct` (`BlueprintMapLibrary.Map_Find` _missionobject _output)))
      (`BlueprintMapLibrary.Map_Add` _missionobject _output (make `/Game/GProjectBP/Blueprints/MissionStruct` _type_2 true _progress))
      (`self.Multicast Missiom HUD Update` _type_2 _progress true)
      (`/Engine/EditorBlueprintResources/StandardMacros.DecrementInt` (`self.RemainObject`)
        (:`  `
          (break)))))
  (if (<= (`self.RemainObject`) 0)
    (`KismetSystemLibrary.PrintString` "Complete")
    (if (`self.HasAuthority`)
      (`/Game/GProjectBP/Blueprints/BP_GameMode.Mission Complete` (cast `/Game/GProjectBP/Blueprints/BP_GameMode` (`self.AuthorityGameMode`) :!pure true)))))

(fn `Initialize Spawnable Enemy List`
  (bind _difficultiyoflevel (`self.DifficultiyOfLevel`))
  (bind _outrownames (`DataTableFunctionLibrary.GetDataTableRowNames` "/Game/GProjectBP/DataAsset/CharacterDataTable.CharacterDataTable"))
  (for (_array_element _array_index) _outrownames
    (if (!= _array_index 0)
      (bind _returnvalue (`|GetDataTableRow` "/Game/GProjectBP/DataAsset/CharacterDataTable.CharacterDataTable" _array_element)
        (:`then`
          (bind ((`MinLevel_14_F11CECB641CA9259328D568FD89891AD` _minlevel) (`MaxLevel_4_E45D45B84B2B2F07FDC3F2861DB05F40` _maxlevel)) (break `/Game/GProjectBP/DataAsset/AssetDataStruct` _returnvalue))
          (if (and (<= _minlevel _difficultiyoflevel) (>= _maxlevel _difficultiyoflevel))
            (`KismetArrayLibrary.Array_AddUnique` (`self.Spawnable Enemy List`) _returnvalue)))))))

(fn `Initialize Spawnable Item List`
  (bind _difficultiyoflevel (`self.DifficultiyOfLevel`))
  (bind _outrownames (`DataTableFunctionLibrary.GetDataTableRowNames` "/Game/GProjectBP/DataAsset/ItemDropTable.ItemDropTable"))
  (for _array_element _outrownames
    (bind _returnvalue (`|GetDataTableRow` "/Game/GProjectBP/DataAsset/ItemDropTable.ItemDropTable" _array_element)
      (:`then`
        (bind (_itemid _minstagelevel _maxstagelevel) (break `/Game/GProjectBP/DataAsset/ItemDropStruct` _returnvalue))
        (if (or (and (<= _minstagelevel _difficultiyoflevel) (>= _maxstagelevel _difficultiyoflevel)) (== _minstagelevel -1))
          (`KismetArrayLibrary.Array_AddUnique` (`self.Spawnable Item List`) _returnvalue))))))

(fn `UserConstructionScript`)