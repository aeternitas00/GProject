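; Base character Blueprint on the Gameplay Ability System, handling health, damage, death and hard crowd control.
; Damage and death events forward to multicasts for child hooks and cosmetics, with death also detaching the controller and setting lifespans.
; Multicasts also update HP and ammo widgets and play montages, skipping dedicated servers.
; Helpers activate or cancel weapon and other abilities; a stun tag cancels weapon use and fails the action check.
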(event `self.OnTagUpdated`
  (params (Tag :type "GameplayTag Structure (by ref)") (TagExists :type Boolean))
  ;[1 1 1] For CC Animation
  (if (`BlueprintGameplayTagLibrary.MatchesTag` Tag (struct :`TagName` "Effect.Debuff.Hard"))
    (if TagExists
      (`self.ReceiveCC` Tag)
      (else
        (`self.EndCC` Tag)))))

(event `self.OnHealthChanged`
  (params (DeltaValue :type "Float (single-precision)") (EventTags :type "GameplayTagContainer Structure (by ref)"))
  ;[1 1 1] UI Update
  (`self.Multicast Health UI Update` (/ (`self.GetHealth`) (`self.GetMaxHealth`)) :!label _label))

(event `self.OnMaxHealthChanged`
  (params (DeltaValue :type "Float (single-precision)") (EventTags :type "GameplayTagContainer Structure (by ref)"))
  ;[1 1 1] UI Update
  (goto _label))

(event `self.OnDamaged`
  (params (DamageAmount :type "Float (single-precision)") (HitInfo :type "HitResult Structure (by ref)") (DamageTags :type "GameplayTagContainer Structure (by ref)") (InstigatorCharacter :type "GPCharacterBase Object Reference") (DamageCauser :type "Actor Object Reference"))
  ;[1 1 1] For Damaged Animation
  (`self.Multicast On Damaged` DamageAmount HitInfo DamageTags InstigatorCharacter DamageCauser)
  (if (not (`self.IsAlive`))
    (`/Engine/EditorBlueprintResources/StandardMacros.DoOnce` false
      (:`Completed`
        (`self.OnDeathEvent`)))))

(event `OnDeathEvent`
  (bind _currentweaponactor (`self.CurrentWeaponActor`))
  ;[1 1 1] Server set life span / multicast to play sound,effect or whatever
  (`/Engine/EditorBlueprintResources/StandardMacros.IsValid` _currentweaponactor
    (:`Is Valid`
      (`self.SetLifeSpan` _currentweaponactor 10.0)
      (`self.SetLifeSpan` self 10.0))
    (:`Is Not Valid`
      _))
  (`self.DetachFromControllerPendingDestroy`)
  (`PrimitiveComponent.SetCollisionObjectType` (`self.Mesh`) "ECC_GameTraceChannel3")
  (`self.OnCharacterDeathBP`)
  (`self.Multicast On Death`))

(event `Update Weapon Mag`
  ;[1 1 1] Called by ANS
  (`GPWeaponActorBase.ReloadWeapon` (`self.CurrentWeaponActor`) -1.0))

(event `On Own Attack Hitted`
  (params (Impact :type Boolean)))

(event `On Weapon Fired`
  (`self.OnWeaponFired`))

(event `Multicast On Death`
  ;[1 1 1] Additional Implements by child
  (`SceneComponent.SetVisibility` (`self.HP`) false false)
  (`SceneComponent.SetVisibility` (`self.Ammo`) false false)
  (`PrimitiveComponent.SetCollisionEnabled` (`self.CapsuleComponent`) "NoCollision"))

(event `Multicast On Damaged`
  (params (`Damage Amount` :type "Float (double-precision)") (`Hit Info` :type "HitResult Structure") (`Damage Tags` :type "GameplayTagContainer Structure") (`Instigator Character` :type "GPCharacterBase Object Reference") (`Damage Causer` :type "Actor Object Reference"))
  ;[1 1 1] Additional Implements by child
  (`self.OnDamagedBP`))

(event `Multicast Health UI Update`
  (params (Percent :type "Float (double-precision)"))
  ;[1 1 1] Update UI
  (bind _aswb_hpbar_test (cast `/Game/GProjectBP/Blueprints/WidgetBP/WB_HPBar_Test` (`WidgetComponent.GetUserWidgetObject` (`self.HP`))))
  (`/Game/GProjectBP/Blueprints/WidgetBP/WB_HPBar_Test.Update Progress` _aswb_hpbar_test Percent))

(event `Multicast Mag UI Update`
  (params (Percent :type "Float (double-precision)"))
  ;[1 1 1] Update UI
  (bind _aswb_hpbar_test_2 (cast `/Game/GProjectBP/Blueprints/WidgetBP/WB_HPBar_Test_2` (`WidgetComponent.GetUserWidgetObject` (`self.Ammo`))))
  (`/Game/GProjectBP/Blueprints/WidgetBP/WB_HPBar_Test_2.Update Progress` _aswb_hpbar_test_2 Percent))

(event `Multicast Montage Play`
  (params (MontageToPlay :type "AnimMontage Object Reference") (PlayRate :type "Float (double-precision)" :default 1.0) (StartingPosition :type "Float (double-precision)" :default 0.0) (StartingSection :type Name))
  ;[1 1 1] Clients are playing montage with no actual effect
  (if (not (`KismetSystemLibrary.IsDedicatedServer`))
    (`|PlayMontage` (`self.Mesh`) MontageToPlay PlayRate StartingPosition StartingSection)))

(fn `CanPerformAction`
  (returns (CanPerform :type Boolean))
  (return (not (`BlueprintGameplayTagLibrary.HasAnyTags` (`GameplayTagAssetInterface.GetOwnedGameplayTags` (`AbilitySystemBlueprintLibrary.GetAbilitySystemComponent` self)) (`BlueprintGameplayTagLibrary.MakeLiteralGameplayTagContainer` (struct :`GameplayTags` (struct :`(TagName` "Effect.Debuff.Hard.Stun")))) true))))

(fn `EndCC`
  (params (Tag :type "GameplayTag Structure")))

(fn `Get Slotted Ability Montage Length`
  (params (ItemSlot :type "GPItemSlot Structure"))
  (returns (Length :type "Float (double-precision)"))
  ;[1 1 1] Use by ai only ( may refactor this later )
  (bind _returnvalue (`self.GetSlottedAbilityInstance` ItemSlot))
  (bind _asga_using_montage_base (cast `/Game/GProjectBP/Abilities/GA_UsingMontage_Base` _returnvalue)
    (:`then`
      (bind _returnvalue_2 (`AnimSequenceBase.GetPlayLength` (`/Game/GProjectBP/Abilities/GA_UsingMontage_Base.PlayingMontage` _asga_using_montage_base)))
      (return _returnvalue_2))
    (:`CastFailed`
      (return -1.0))))

(fn `IsAlive`
  (returns (Value :type Boolean))
  (return (> (`self.GetHealth`) 0.0)))

(fn `ReceiveCC`
  (params (Tag :type "GameplayTag Structure"))
  ;[1 1 1] CC React
  (`|SwitchGameplayTag` Tag
    (:`Effect.Debuff.Hard.Stun`
      (`self.StopCurrentWeapon`))))

(fn `StartSpecificAbility`
  (params (InAbilityToActivate :type "GameplayAbility Class Reference"))
  (returns (`Ability Success` :type Boolean))
  (bind _returnvalue (`AbilitySystemComponent.TryActivateAbilityByClass` (`AbilitySystemBlueprintLibrary.GetAbilitySystemComponent` self) InAbilityToActivate true))
  (return _returnvalue))

(fn `StopCurrentWeapon`
  (`GPAbilitySystemComponent.CancelAbilityByClass` (cast `GPAbilitySystemComponent` (`AbilitySystemBlueprintLibrary.GetAbilitySystemComponent` self) :!pure true) "/Game/GProjectBP/Abilities/Character/GA_CharacterUseWeapon.GA_CharacterUseWeapon_C"))

(fn `StopSpecificAbility`
  (params (AbilityClass :type "GameplayAbility Class Reference"))
  (returns (`Successful Cancel` :type Boolean))
  (bind _returnvalue (`GPAbilitySystemComponent.CancelAbilityByClass` (cast `GPAbilitySystemComponent` (`AbilitySystemBlueprintLibrary.GetAbilitySystemComponent` self) :!pure true) AbilityClass))
  (return _returnvalue))

(fn `UseCurrentWeapon`
  (returns (Success :type Boolean))
  (bind _returnvalue (`AbilitySystemComponent.TryActivateAbilityByClass` (`AbilitySystemBlueprintLibrary.GetAbilitySystemComponent` self) "/Game/GProjectBP/Abilities/Character/GA_CharacterUseWeapon.GA_CharacterUseWeapon_C" true))
  (return _returnvalue))

(fn `UserConstructionScript`)