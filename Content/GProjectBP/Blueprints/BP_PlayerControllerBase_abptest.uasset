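; Player controller for BP_PlayerCharacter_abptest that caches the pawn on BeginPlay or possession and handles movement, mouse look, interaction and aiming input.
; Each Tick applies movement along control-yaw vectors when the character can act, sets direction flags, and interpolates body yaw while moving.
; Interaction calls the character's InteractionComponent, while UseOptic plays an aim montage chosen by weapon type and stance, using the Reverse section when already aiming.
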(event `self.ReceiveBeginPlay`
  (if (`self.IsLocalPlayerController`)
    (bind _asbp_player_character_abptest (cast `/Game/GProjectBP/Blueprints/BP_PlayerCharacter_abptest` (`self.K2_GetPawn`)))
    (set `self.PlayerCharacter` _asbp_player_character_abptest) ; TODO 특정 상황에서 중복 배제
  ))

(event `self.ReceiveTick`
  (params (DeltaSeconds :type "Float (single-precision)"))
  (`self.Movement Controll`)
  (if (or (!= (`self.MoveForwardAxis`) 0.0) (!= (`self.MoveRightAxis`) 0.0))
    (`self.RotateYawWhileMoving`)))

(event `self.ReceivePossess`
  (params (PossessedPawn :type "Pawn Object Reference"))
  (bind _asbp_player_character_abptest (cast `/Game/GProjectBP/Blueprints/BP_PlayerCharacter_abptest` PossessedPawn))
  (set `self.PlayerCharacter` _asbp_player_character_abptest) ; TODO 특정 상황에서 중복 배제
)

(event `InputAction|MainInteraction`
  (params (Key :type "Key Structure"))
  (bind _playercharacter (`self.PlayerCharacter`))
  (bind _interactioncomponent (`/Game/GProjectBP/Blueprints/BP_PlayerCharacter_abptest.InteractionComponent` _playercharacter))
  (:`Pressed`
    (`/Engine/EditorBlueprintResources/StandardMacros.IsValid` _playercharacter
      (:`Is Valid`
        (`/Engine/EditorBlueprintResources/StandardMacros.IsValid` _interactioncomponent
          (:`Is Valid`
            (`GPInteractionComponent.PrimaryInteract` _interactioncomponent)))))))

(event `Movement Controll`
  (bind (_forwardvector _rightvector) (`self.GetCharacterVectors`))
  (bind _returnvalue (`self.K2_GetPawn`))
  (bind _returnvalue_2 (`self.GetInputAxisValue`))
  (bind _returnvalue_3 (`self.GetInputAxisValue`))
  (bind _asbp_character_base (cast `/Game/GProjectBP/Blueprints/BP_CharacterBase` _returnvalue :!pure true))
  (`/Engine/EditorBlueprintResources/StandardMacros.IsValid` _asbp_character_base
    (:`Is Valid`
      (if (`/Game/GProjectBP/Blueprints/BP_CharacterBase.CanPerformAction` _asbp_character_base)
        (set `self.MoveForwardAxis` _returnvalue_2)
        (if (!= _returnvalue_2 0.0)
          (`Pawn.AddMovementInput` _returnvalue _forwardvector _returnvalue_2 false)
          (set `self.bMovingForward` (> _returnvalue_2 0.0))
          (set `self.bMovingBackward` (< _returnvalue_2 0.0))
          (else
            (set `self.MoveRightAxis` _returnvalue_3)))
        (if (!= _returnvalue_3 0.0)
          (`Pawn.AddMovementInput` _returnvalue _rightvector _returnvalue_3 false)
          (set `self.bMovingRight` (> _returnvalue_3 0.0))
          (set `self.bMovingLeft` (< _returnvalue_3 0.0)))))))

(event `InputAction|UseOptic`
  (params (Key :type "Key Structure"))
  (bind _bcrouching (`self.bCrouching`))
  (bind _playercharacter (`self.PlayerCharacter`))
  (:`Pressed`
    (`/Engine/EditorBlueprintResources/StandardMacros.IsValid` _playercharacter
      (:`Is Valid`
        (`Character.PlayAnimMontage` _playercharacter (select `/Game/CharactersAssets/MOCAPAnimationPacks/Mobility/ControllerMain/Blueprints/WeaponState` (`/Game/GProjectBP/Blueprints/BPFL_ABP.Get Preper Weapon Anim Flag` (`GPCharacterBase.CurrentWeaponActor` (`self.PlayerCharacter`))) :`NewEnumerator1` (select `bool` _bcrouching :`false` "/Game/GProjectBP/Animation/Montage/MOCAP/AM_Aim_Stand_W1.AM_Aim_Stand_W1" :`true` "/Game/GProjectBP/Animation/Montage/MOCAP/AM_Aim_Crouch_W1.AM_Aim_Crouch_W1" :!type "AnimMontage Object Reference") :`NewEnumerator2` (select `bool` _bcrouching :`false` "/Game/GProjectBP/Animation/Montage/MOCAP/AM_Aim_Stand_W2.AM_Aim_Stand_W2" :`true` "/Game/GProjectBP/Animation/Montage/MOCAP/AM_Aim_Crouch_W2.AM_Aim_Crouch_W2" :!type "AnimMontage Object Reference")) 1.0 (select `bool` (`/Game/GProjectBP/Blueprints/BP_PlayerCharacter_abptest.bUsingOptic` _playercharacter) :`false` "Default" :`true` "Reverse" :!type "Name"))))))

(event `InputAxis|MouseX`
  (params (AxisValue :type "Float (single-precision)"))
  (`Pawn.AddControllerYawInput` (`self.PlayerCharacter`) (* AxisValue 2.5)))

(event `InputAxis|MouseY`
  (params (AxisValue :type "Float (single-precision)"))
  (`Pawn.AddControllerPitchInput` (`self.PlayerCharacter`) (* AxisValue 1.5)))

(event `Multicast Play Montage`
  (params (Character :type "Character Object Reference") (AnimMontage :type "AnimMontage Object Reference") (StartSectionName :type Name))
  (`Character.PlayAnimMontage` Character AnimMontage 1.0 StartSectionName))

(fn `GetCharacterVectors`
  (returns (ForwardVector :type "Vector Structure") (RightVector :type "Vector Structure"))
  (bind _returnvalue (`KismetMathLibrary.MakeRotator` 0.0 0.0 (.yaw (`Pawn.GetControlRotation` (`self.PlayerCharacter`)))))
  (return (`KismetMathLibrary.GetForwardVector` _returnvalue) (`KismetMathLibrary.GetRightVector` _returnvalue)))

(fn `RotateYawWhileMoving`
  (bind _returnvalue (`KismetMathLibrary.RInterpTo_Constant` (`self.K2_GetActorRotation` (`self.PlayerCharacter`)) (`KismetMathLibrary.MakeRotator` 0.0 0.0 (.yaw (`self.GetDesiredRotation`))) (`GameplayStatics.GetWorldDeltaSeconds`) (`KismetMathLibrary.SelectFloat` 140.0 100.0 (`self.bMovingTurn`))))
  (if (`self.bTurnLock`)
    (`self.K2_SetActorRotation` (`self.PlayerCharacter`) (* _returnvalue 0.5) false)
    (else
      (`self.K2_SetActorRotation` (`self.PlayerCharacter`) _returnvalue false)))
  (return))

(fn `UserConstructionScript`)