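; Sublevel boundary actor that streams in a connected sublevel and switches the current sublevel as the player crosses it.
; LoadBoundary overlap asks BP_GameInstance to load the sublevel at the connection's index, rotation and root-relative offset.
; ChangeBoundary tests horizontal player velocity against BoundaryDirection on both overlap begin and end.
; When both checks find movement within 90 degrees of that direction, BP_GameInstance changes the current sublevel.
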(event `self.LoadBoundary.OnComponentBeginOverlap`
  (params (OverlappedComponent :type "PrimitiveComponent Object Reference") (OtherActor :type "Actor Object Reference") (OtherComp :type "PrimitiveComponent Object Reference") (OtherBodyIndex :type Integer) (bFromSweep :type Boolean) (SweepResult :type "HitResult Structure (by ref)"))
  (cast `/Game/GProjectBP/Blueprints/BP_PlayerCharacter` OtherActor)
  (`/Game/GProjectBP/Blueprints/BP_GameInstance.Load Sublevel` (cast `/Game/GProjectBP/Blueprints/BP_GameInstance` (`GameplayStatics.GetGameInstance`) :!pure true) (`self.LocalConnectionIndex`) (`self.GetLocationOfConnection`) (`self.GetRotationOfConnection`)))

(event `self.ChangeBoundary.OnComponentEndOverlap`
  (params (OverlappedComponent :type "PrimitiveComponent Object Reference") (OtherActor :type "Actor Object Reference") (OtherComp :type "PrimitiveComponent Object Reference") (OtherBodyIndex :type Integer))
  (if (and (`self.WorkReady`) (`self.DirectionCheck` OtherActor))
    (`self.Change Level Idx`))
  (set `self.WorkReady` false))

(event `self.ChangeBoundary.OnComponentBeginOverlap`
  (params (OverlappedComponent :type "PrimitiveComponent Object Reference") (OtherActor :type "Actor Object Reference") (OtherComp :type "PrimitiveComponent Object Reference") (OtherBodyIndex :type Integer) (bFromSweep :type Boolean) (SweepResult :type "HitResult Structure (by ref)"))
  (set `self.WorkReady` (`self.DirectionCheck` OtherActor)))

(fn `Change Level Idx`
  (`/Game/GProjectBP/Blueprints/BP_GameInstance.Change Current Sublevel` (cast `/Game/GProjectBP/Blueprints/BP_GameInstance` (`GameplayStatics.GetGameInstance`) :!pure true) self))

(fn `DirectionCheck`
  (params (Character :type "Object Object Reference"))
  (returns (bIsCorrectDirection :type Boolean))
  (bind _asbp_player_character (cast `/Game/GProjectBP/Blueprints/BP_PlayerCharacter` Character)
    (:`then`
      (bind _returnvalue (`KismetMathLibrary.DegAcos` (`KismetMathLibrary.Dot_VectorVector` (`KismetMathLibrary.Normal` (`KismetMathLibrary.GreaterGreater_VectorRotator` (`self.BoundaryDirection`) (`SceneComponent.K2_GetComponentRotation` (`self.Root`)))) (`KismetMathLibrary.Normal` (`KismetMathLibrary.MakeVector` (.x (`self.GetVelocity` _asbp_player_character)) (.y (`self.GetVelocity` _asbp_player_character)))))))
      (return (and (>= _returnvalue -90.0) (<= _returnvalue 90.0))))
    (:`CastFailed`
      (return false))))

(fn `GetLocationOfConnection`
  (returns (`Sublevel Offset` :type "Vector Structure"))
  (bind _root (`self.Root`))
  (return (+ (`KismetMathLibrary.GreaterGreater_VectorRotator` (`self.Offset`) (`SceneComponent.K2_GetComponentRotation` _root)) (`SceneComponent.K2_GetComponentLocation` _root))))

(fn `GetRotationOfConnection`
  (returns (`Sublevel Rotation` :type "Rotator Structure"))
  (return (`SceneComponent.K2_GetComponentRotation` (`self.Root`))))

(fn `UserConstructionScript`)