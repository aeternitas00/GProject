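; Actor that takes a top-down orthographic snapshot of the level, named for use as the minimap image.
; Setup moves it high above a given center, hides space sphere actors from the capture, and applies the ortho width to both the SceneCaptureComponent2D and its Camera.
; Capture renders the scene on demand, prints a debug string, and broadcasts the render target through OnSceneCaptured.
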(event `self.ReceiveTick`
  (params (DeltaSeconds :type "Float (single-precision)")))

(event `Capture`
  (bind _scenecapturecomponent2d (`self.SceneCaptureComponent2D`))
  (`SceneCaptureComponent2D.CaptureScene` _scenecapturecomponent2d)
  (`KismetSystemLibrary.PrintString` "capture")
  (`self.OnSceneCaptured` (`SceneCaptureComponent2D.TextureTarget` _scenecapturecomponent2d)))

(event `Setup`
  (params (Center :type "Vector Structure") (OrthoWidth :type "Float (double-precision)"))
  (bind _outactors (`GameplayStatics.GetAllActorsOfClass` "/Game/GProjectBP/Blueprints/Objects/BP_SpaceSphere_1.BP_SpaceSphere_1_C"))
  (set `SceneCaptureComponent.HiddenActors` _outactors (`self.SceneCaptureComponent2D`))
  (`self.K2_SetActorLocation` (+ Center (0.0 0.0 10000.0)) false true)
  (bind _output_get (set `SceneCaptureComponent2D.OrthoWidth` OrthoWidth (`self.SceneCaptureComponent2D`)))
  (`CameraComponent.SetOrthoWidth` (`self.Camera`) _output_get))

(fn `UserConstructionScript`)