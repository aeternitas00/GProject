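; Actor component that fades its owner's meshes to translucent and back when Begin and End are called.
; BeginPlay creates one shared dynamic translucent material and caches original materials from the root's direct mesh children, or the root itself if childless.
; Begin swaps every slot to that material; Tick lowers its opacity, or raises it after End.
; Reset restores the originals after fade-in, and ticking switches off whenever either fade completes.
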(event `self.ReceiveBeginPlay`
  (bind _returnvalue (`self.GetOwner`))
  (bind _meshs (`self.Meshs`))
  (bind _children (`SceneComponent.GetChildrenComponents` (`Actor.RootComponent` _returnvalue) false))
  (bind _returnvalue_2 (`KismetMaterialLibrary.CreateDynamicMaterialInstance` "/Game/Geometry/Meshes/Transparency_Material_Base_Inst.Transparency_Material_Base_Inst"))
  (set `self.TranslucentMaterial` _returnvalue_2)
  (if (== (`KismetArrayLibrary.Array_Length` _children) 0)
    (bind _asmesh_component (cast `MeshComponent` (`Actor.RootComponent` _returnvalue)))
    (`KismetArrayLibrary.Array_Add` (`self.Meshs`) _asmesh_component)
    (else
      (for _array_element _children
        (bind _asmesh_component_2 (cast `MeshComponent` _array_element))
        (`KismetArrayLibrary.Array_Add` _meshs _asmesh_component_2))))
  (for _array_element_2 _meshs
    (bind _returnvalue_3 (`MeshComponent.GetMaterials` _array_element_2))
    (for _array_element_3 _returnvalue_3
      (`KismetArrayLibrary.Array_Add` (`self.OriginalMaterials`) (cast `MaterialInstance` _array_element_3 :!pure true)))
    (`KismetArrayLibrary.Array_Add` (`self.MaterialsNum`) (`KismetArrayLibrary.Array_Length` _returnvalue_3)))
  (set `self.Amount` 0.7))

(event `self.ReceiveTick`
  (params (DeltaSeconds :type "Float (single-precision)"))
  (bind _returnvalue (* DeltaSeconds 1.0))
  (bind _amount (`self.Amount`))
  (bind _translucentmaterial (`self.TranslucentMaterial`))
  (if (`self.bIsTranslucent`)
    (bind _output_get (set `self.Amount` (`KismetMathLibrary.FClamp` (- _amount _returnvalue) 0.3 0.7)))
    (`MaterialInstanceDynamic.SetScalarParameterValue` _translucentmaterial "Opacity" _output_get)
    (if (<= (`self.Amount`) 0.3)
      (`self.SetComponentTickEnabled` false))
    (else
      (bind _output_get_2 (set `self.Amount` (`KismetMathLibrary.FClamp` (+ _amount _returnvalue) 0.3 0.7)))
      (`MaterialInstanceDynamic.SetScalarParameterValue` _translucentmaterial "Opacity" _output_get_2)
      (if (>= (`self.Amount`) 0.7)
        (`self.Reset`)))))

(event `Begin`
  (if (not (`self.bIsTranslucent`))
    (set `self.Index` 0)
    (for (_array_element _array_index) (`self.Meshs`)
      (for _index (range (`|GetArrayItem` (`self.MaterialsNum`) _array_index))
        (`PrimitiveComponent.SetMaterial` _array_element _index (`self.TranslucentMaterial`))
        (`/Engine/EditorBlueprintResources/StandardMacros.IncrementInt` (`self.Index`))))
    (set `self.bIsTranslucent` true)
    (`self.SetComponentTickEnabled` true)))

(event `End`
  (if (`self.bIsTranslucent`)
    (set `self.bIsTranslucent` false)
    (`self.SetComponentTickEnabled` true)))

(event `Reset`
  (set `self.Index` 0)
  (for (_array_element _array_index) (`self.Meshs`)
    (for _index (range (`|GetArrayItem` (`self.MaterialsNum`) _array_index))
      (`PrimitiveComponent.SetMaterial` _array_element _index (`|GetArrayItem` (`self.OriginalMaterials`) (`self.Index`)))
      (`/Engine/EditorBlueprintResources/StandardMacros.IncrementInt` (`self.Index`))))
  (`self.SetComponentTickEnabled` false)
  (set `self.Amount` 0.9))