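; BP_SkillCaptureActor is a scene capture actor that previews skill montages on a skeletal mesh.
; UpdateCaptureCharacter plays a timeline that drives the capture component's FOV, easing it in when active and reversing it quickly when inactive.
; PreviewMontage plays the given montage and replays it after a timer delay each time it completes.
; StopMontage blends the montage out and clears the stored reference.
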(event `UpdateCaptureCharacter`
  (params (bActive :type Boolean))
  ;[1 1 1] Update Capture Character
  (if bActive
    (`TimelineComponent.SetPlayRate` (`self.FOV_Anim`) 0.8)
    (bind (_direction _fov) (`Timeline|FOV_Anim` :!via `PlayFromStart` :!label _label)
      (:`Update`
        (set `SceneCaptureComponent2D.FOVAngle` (`KismetMathLibrary.MapRangeClamped` _fov 0.0 1.0 30.0 40.0) (`self.SceneCaptureComponent2D`))))
    (else
      (`TimelineComponent.SetPlayRate` (`self.FOV_Anim`) 8.0)
      (goto _label :!via `Reverse`))))

(event `PreviewMontage`
  (params (MontageToPlay :type "AnimMontage Object Reference"))
  (set `self.Montage to Play` MontageToPlay)
  (bind _montage_to_play (`self.Montage to Play`)
    (:`then`
      (`|PlayMontage` (`self.SkeletalMesh`) _montage_to_play :!label _label_2
        (:`OnCompleted`
          (`KismetSystemLibrary.K2_SetTimerDelegate` (delegate `Loop`) (`self.Delay`)))))
    (:`else`)))

(event `Loop`
  (goto _label_2))

(event `Stop Montage`
  (`AnimInstance.Montage_Stop` (`SkeletalMeshComponent.GetAnimInstance` (`self.SkeletalMesh`)) 0.25 (`self.Montage to Play`))
  (set `self.Montage to Play` null))

(fn `UserConstructionScript`)