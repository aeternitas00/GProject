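; Worker actor that makes objects near the player's camera translucent, likely so they do not block the view.
; Each tick, a box trace at the camera, sized by spring arm length, finds hit actors with a BP_TranslucentComponent and calls Begin on them.
; It tracks faded components, calling End on those no longer hit and removing them in reverse index order, or clearing all when nothing is hit.
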(event `self.ReceiveBeginPlay`
  (bind _asbp_player_character (cast `/Game/GProjectBP/Blueprints/BP_PlayerCharacter` (`GameplayStatics.GetPlayerPawn` 0)))
  (set `self.SpringArm1` (`/Game/GProjectBP/Blueprints/BP_PlayerCharacter.SpringArm` _asbp_player_character))
  (set `self.Camera1` (`/Game/GProjectBP/Blueprints/BP_PlayerCharacter.Camera` _asbp_player_character))
  (`self.SetActorTickEnabled` true))

(event `self.ReceiveTick`
  (params (DeltaSeconds :type "Float (single-precision)"))
  (bind _nothidetranslucentcomp (`self.NotHideTranslucentComp`))
  (bind _lasthittranslucentcomp (`self.LastHitTranslucentComp`))
  (bind _returnvalue (`KismetArrayLibrary.Array_LastIndex` _nothidetranslucentcomp))
  (bind _returnvalue_2 (`SceneComponent.K2_GetComponentLocation` (`self.Camera1`)))
  ;[0.0625 0.0625 0.0625] Hide static Mesh
  (bind (_outhits _returnvalue_3) (`KismetSystemLibrary.BoxTraceMultiForObjects` _returnvalue_2 (+ _returnvalue_2 (0.0 0.0 1.0)) (`KismetMathLibrary.MakeVector` 70.0 70.0 (- (`SpringArmComponent.TargetArmLength` (`self.SpringArm1`)) 100.0)) (struct :`Pitch` 30.0) (`|MakeArray` "ObjectTypeQuery7" :!type "EObjectTypeQuery Enum")))
  (if _returnvalue_3
    (`KismetArrayLibrary.Array_Clear` (`self.NewHitTranslucentComp`))
    (for _array_element _outhits
      (bind _returnvalue_4 (`self.GetComponentByClass` (`.HitActor` (`GameplayStatics.BreakHitResult` _array_element)) "/Game/GProjectBP/Blueprints/Workers/BP_TranslucentComponent.BP_TranslucentComponent_C"))
      (`/Engine/EditorBlueprintResources/StandardMacros.IsValid` _returnvalue_4
        (:`Is Valid`
          (bind _output_get (set `self.Translucent Component` _returnvalue_4))
          (`KismetArrayLibrary.Array_Add` (`self.NewHitTranslucentComp`) _output_get)
          ;;[0.08333 0.08333 0.08333] Hide
          (if (not (`/Game/GProjectBP/Blueprints/Workers/BP_TranslucentComponent.bIsTranslucent` (`self.Translucent Component`)))
            (`/Game/GProjectBP/Blueprints/Workers/BP_TranslucentComponent.Begin` (`self.Translucent Component`))
            (`KismetArrayLibrary.Array_AddUnique` (`self.LastHitTranslucentComp`) (`self.Translucent Component`))))))
    ;;[0.08333 0.08333 0.08333] Scan all hiding component and find component to unhide
    (if (`KismetArrayLibrary.Array_IsValidIndex` (`self.LastHitTranslucentComp`))
      (`KismetArrayLibrary.Array_Clear` (`self.NotHideTranslucentComp`))
      (for (_array_element_2 _array_index) (`self.LastHitTranslucentComp`)
        (bind _output_get_2 (set `self.Translucent Component` _array_element_2))
        (if (== (`KismetArrayLibrary.Array_Find` (`self.NewHitTranslucentComp`) _output_get_2) -1)
          (`KismetArrayLibrary.Array_Add` (`self.NotHideTranslucentComp`) _array_index)))
      ;;[0.08333 0.08333 0.08333] Last To First Unhide
      (if (`KismetArrayLibrary.Array_IsValidIndex` _nothidetranslucentcomp)
        (for _index (range (+ _returnvalue 1))
          (bind _output (`|GetArrayItem` (`self.NotHideTranslucentComp`) (- _returnvalue _index)))
          (`/Game/GProjectBP/Blueprints/Workers/BP_TranslucentComponent.End` (`|GetArrayItem` (`self.LastHitTranslucentComp`) _output))
          (`KismetArrayLibrary.Array_Remove` (`self.LastHitTranslucentComp`) _output))))
    (else
      ;;[0.08333 0.08333 0.08333] No targets to hide
      (if (`KismetArrayLibrary.Array_IsValidIndex` _lasthittranslucentcomp)
        (for _array_element_3 _lasthittranslucentcomp
          (`/Game/GProjectBP/Blueprints/Workers/BP_TranslucentComponent.End` _array_element_3))
        (`KismetArrayLibrary.Array_Clear` _lasthittranslucentcomp)))))

(fn `UserConstructionScript`)