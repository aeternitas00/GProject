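; In-game player controller that owns the HUD, inventory screen, consumable menu and the player's item actions.
; It shows a loading screen until level init completes, then builds widgets, loads inventory, and spawns the two slotted weapons hidden on the hand socket with saved attachments.
; Item use branches on granted ability and type to consume, attach or throw, with throws spawning impulse-launched pickups.
; Holding the consumable key opens a selection list, while tapping uses the slotted consumable.
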(event `self.ReceiveBeginPlay`
  (`parent.ReceiveBeginPlay`)
  (bind _asbp_game_state_base (cast `/Game/GProjectBP/Blueprints/BP_GameState_Base` (`GameplayStatics.GetGameState`))
    (:`then`
      (if (`/Game/GProjectBP/Blueprints/BP_GameState_Base.bIsLevelInitialized` _asbp_game_state_base)
        (`self.Post Init Lvl` :!label _label)
        (else
          (add `/Game/GProjectBP/Blueprints/BP_GameState_Base.LvlInitComplete` _asbp_game_state_base (delegate `Post Init Lvl`))
          (`self.DisableInput` self)
          (bind _returnvalue (`|CreateWidget` "/Game/GProjectBP/Blueprints/WidgetBP/WB_LoadingScreen.WB_LoadingScreen_C" (`GameplayStatics.GetPlayerController` 0)))
          (set `self.loadingscr` _returnvalue)
          (`UserWidget.AddToViewport` _returnvalue 0))))
    (:`CastFailed`
      (goto _label))))

(event `Post Init Lvl`
  (bind _quickslotwidget (`self.QuickSlotWidget`))
  (bind _loadingscr (`self.loadingscr`))
  (bind _returnvalue (`|CreateWidget` "/Game/GProjectBP/Blueprints/WidgetBP/Inventory/WB_SkillListMain.WB_SkillListMain_C"))
  (bind _output_get (set `self.QuickSlotWidget` _returnvalue))
  (`UserWidget.AddToViewport` _output_get 0)
  (`Widget.SetVisibility` _quickslotwidget "SelfHitTestInvisible")
  (`/Game/GProjectBP/Blueprints/WidgetBP/Inventory/WB_SkillListMain.Reset Skill List` _quickslotwidget)
  (bind _returnvalue_2 (`|CreateWidget` "/Game/GProjectBP/Blueprints/WidgetBP/HUD/WB_HUD_Main.WB_HUD_Main_C"))
  (bind _output_get_2 (set `self.MainHUD` _returnvalue_2))
  (set `self.ChatWindow` (`/Game/GProjectBP/Blueprints/WidgetBP/HUD/WB_HUD_Main.ChatWidget` _returnvalue_2))
  (`UserWidget.AddToViewport` _output_get_2 0)
  (bind _output_get_3 (set `self.InventoryWidget` (`/Game/GProjectBP/Blueprints/WidgetBP/HUD/WB_HUD_Main.WB_InventoryMain` _returnvalue_2)))
  (`Widget.SetVisibility` _output_get_3 "Collapsed")
  (`self.LoadInventory`)
  (`self.EnableInput` self)
  (`/Engine/EditorBlueprintResources/StandardMacros.IsValid` _loadingscr
    (:`Is Valid`
      (`/Game/GProjectBP/Blueprints/WidgetBP/WB_LoadingScreen.Close Loading Scr` _loadingscr))))

(event `self.InventoryLoaded`
  (bind _inventorydata (`self.InventoryData`))
  (bind _playercharacter (`self.PlayerCharacter`))
  (bind _playercharacter_2 (`self.PlayerCharacter`))
  (bind _keys (`BlueprintMapLibrary.Map_Keys` _inventorydata))
  (for _array_element _keys
    (`self.InventoryItemChanged` _array_element (`BlueprintMapLibrary.Map_Find` _inventorydata _array_element)))
  (for _index (range 2)
    (bind _gpitemslot (make `GPItemSlot` "Weapon" _index))
    (bind _asgpitem_weapon (cast `GPItemWeapon` (`BlueprintMapLibrary.Map_Find` (`self.SlottedItems`) _gpitemslot)))
    (`self.ClientWeaponChanged` _gpitemslot _asgpitem_weapon)
    (bind _asgpweapon_actor_base (castclass `GPWeaponActorBase` (`GPItemWeapon.WeaponActor` _asgpitem_weapon)))
    (bind _returnvalue (`|SpawnActorFromClass` _asgpweapon_actor_base (`KismetMathLibrary.MakeTransform` (0.0 0.0 -500.0)) "Undefined" "OverrideRootScale" _playercharacter _playercharacter))
    (add `GPWeaponActorBase.OnMagSizeChanged_D` _returnvalue (`|CreateDelegate` (`self.PlayerCharacter`) :!event `Weapon OnMagSizeChanged`))
    (add `GPWeaponActorBase.OnCurrentMagChanged_D` _returnvalue (`|CreateDelegate` (`self.PlayerCharacter`) :!event `Weapon OnCurrentMagChanged`))
    (`self.SetActorHiddenInGame` _returnvalue true)
    (`BlueprintMapLibrary.Map_Add` (`/Game/GProjectBP/Blueprints/BP_PlayerCharacter.SlottedWeaponActor` _playercharacter_2) _gpitemslot _returnvalue)
    (`self.K2_AttachToComponent` _returnvalue (`Character.Mesh` _playercharacter_2) "hand_rSoc" "SnapToTarget" "SnapToTarget" "KeepWorld" true) ; Attach the character's hand
    (bind (_value _returnvalue_2) (`BlueprintMapLibrary.Map_Find` (`GPGameInstanceBase.AttachedItems` (cast `/Game/GProjectBP/Blueprints/BP_GameInstance` (`GameplayStatics.GetGameInstance`) :!pure true)) _gpitemslot))
    (if _returnvalue_2
      (bind _values (`BlueprintMapLibrary.Map_Values` (`.Attached` (break `GPWAttachmentedData` _value))))
      (for _array_element_2 _values
        (bind _asgpitem_attachment (cast `GPItemAttachment` (`KismetSystemLibrary.GetObjectFromPrimaryAssetId` _array_element_2) :!pure true))
        (`self.ClientAttachmentChanged` _gpitemslot _asgpitem_attachment)
        (`GPWeaponActorBase.AddAttachment` _returnvalue _asgpitem_attachment))))
  (bind _values_2 (`BlueprintMapLibrary.Map_Values` (`/Game/GProjectBP/Blueprints/BP_PlayerCharacter.SlottedWeaponActor` (`self.PlayerCharacter`))))
  (for _array_element_3 _values_2
    (`GPWeaponActorBase.ReloadWeapon` _array_element_3 -1.0)))

(event `Update Mag HUD`
  (params (bIsCurrent :type Boolean) (Value :type "Float (double-precision)"))
  (bind _mainhud (`self.MainHUD`))
  (bind _ammostatus (`/Game/GProjectBP/Blueprints/WidgetBP/HUD/WB_HUD_Main.AmmoStatus` _mainhud))
  (`/Engine/EditorBlueprintResources/StandardMacros.IsValid` _mainhud
    (:`Is Valid`
      (if bIsCurrent
        (`/Game/GProjectBP/Blueprints/WidgetBP/HUD/WB_HUD_AmmoStatus.Current Mag Update` _ammostatus Value)
        (else
          (`/Game/GProjectBP/Blueprints/WidgetBP/HUD/WB_HUD_AmmoStatus.Max Mag Update` _ammostatus Value))))))

(event `self.InventoryItemChanged`
  (params (Item :type "GPItem Object Reference") (ItemData :type "GPItemData Structure"))
  ;[1 1 1] Inventory Item Change
  (if (not (== (`.Name` (break `PrimaryAssetType` (`GPItem.ItemType` Item))) "Weapon"))
    (`self.ClientInventoryItemChange` Item ItemData)))

(event `Use Selected Consumbale`
  (`/Game/GProjectBP/Blueprints/BP_PlayerCharacter.UseSlottedConsumable` (`self.PlayerCharacter`)))

(event `ClientInventoryItemChange`
  (params (Item :type "GPItem Object Reference") (`Item Data` :type "GPItemData Structure"))
  (bind _inventorywidget (`self.InventoryWidget`))
  ;[1 1 1] Inventory Item Change
  (`/Engine/EditorBlueprintResources/StandardMacros.IsValid` _inventorywidget
    (:`Is Valid`
      (`/Game/GProjectBP/Blueprints/WidgetBP/Inventory/WB_InventoryMain.UpdateItemButton` _inventorywidget Item `Item Data`))))

(event `Server Use Inventory Item`
  (params (Item :type "GPItem Object Reference"))
  (`self.Use Item` Item))

(event `Server Throw Inventory Item`
  (params (Item :type "GPItem Object Reference") (inThrowStack :type Boolean))
  (`self.Throw Item` Item inThrowStack))

(event `self.SlottedItemChanged`
  (params (ItemSlot :type "GPItemSlot Structure") (Item :type "GPItem Object Reference"))
  (bind _playercharacter (`self.PlayerCharacter`))
  (switch `name` (`.Name` (break `PrimaryAssetType` (`.ItemType` (break `GPItemSlot` ItemSlot))))
    (:`Weapon`
      (`/Engine/EditorBlueprintResources/StandardMacros.IsValid` _playercharacter
        (:`Is Valid`
          (set `/Game/GProjectBP/Blueprints/BP_PlayerCharacter.RequestedWeaponSlot` (struct) _playercharacter)
          (`self.Multicast Play Montage` _playercharacter "/Game/GProjectBP/Animation/Montage/AM_SwapWeapon.AM_SwapWeapon" "DrawWeapon")
          (`self.ClientWeaponChanged` ItemSlot (cast `GPItemWeapon` Item :!pure true)))))))

(event `ClientWeaponChanged`
  (params (`Item Slot` :type "GPItemSlot Structure") (Item :type "GPItemWeapon Object Reference"))
  (bind _inventorywidget (`self.InventoryWidget`))
  (`/Engine/EditorBlueprintResources/StandardMacros.IsValid` _inventorywidget
    (:`Is Valid`
      (`/Game/GProjectBP/Blueprints/WidgetBP/Inventory/WB_InventoryMain.UpdateWeaponButton` _inventorywidget Item (`.SlotNumber` (break `GPItemSlot` `Item Slot`))))))

(event `ClientAttachmentChanged`
  (params (`Item Slot` :type "GPItemSlot Structure") (Item :type "GPItemAttachment Object Reference"))
  (bind _inventorywidget (`self.InventoryWidget`))
  (`/Engine/EditorBlueprintResources/StandardMacros.IsValid` _inventorywidget
    (:`Is Valid`
      (`/Game/GProjectBP/Blueprints/WidgetBP/Inventory/WB_InventoryMain.UpdateWeaponAttachment` _inventorywidget Item (`.SlotNumber` (break `GPItemSlot` `Item Slot`))))))

(event `Multicast Play Montage`
  (params (Character :type "Character Object Reference") (AnimMontage :type "AnimMontage Object Reference") (StartSectionName :type Name))
  (`Character.PlayAnimMontage` Character AnimMontage 1.0 StartSectionName))

(event `InputAction|OpenInventory`
  (params (Key :type "Key Structure"))
  (bind _inventorywidget (`self.InventoryWidget`))
  (:`Pressed`
    (if (not (`self.bIsConsumableOpen`))
      (bind _asbp_player_character (cast `/Game/GProjectBP/Blueprints/BP_PlayerCharacter` (`self.K2_GetPawn`)))
      (if (`/Game/GProjectBP/Blueprints/BP_PlayerCharacter.IsAlive` _asbp_player_character)
        (`/Engine/EditorBlueprintResources/StandardMacros.IsValid` _inventorywidget
          (:`Is Valid`
            (if (`self.bIsInventoryOpen`)
              (`Widget.SetVisibility` _inventorywidget "Collapsed")
              (set `self.bIsInventoryOpen` false)
              (set `self.bShowMouseCursor` false)
              (else
                (`Widget.SetVisibility` _inventorywidget "SelfHitTestInvisible")
                (set `self.bIsInventoryOpen` true)
                (set `self.bShowMouseCursor` true)))))))))

(event `InputAction|OpenConsumableMenu`
  (params (Key :type "Key Structure"))
  (:`Pressed`
    (if (not (`self.bIsInventoryOpen`))
      (bind _returnvalue (`KismetSystemLibrary.K2_SetTimerDelegate` (delegate `Open Consumable Menu Ex`) 0.5))
      (set `self.ConsumableTimer` _returnvalue)))
  (:`Released`
    (if (`self.bIsConsumableOpen`)
      (set `self.bIsConsumableOpen` false)
      (`/Game/GProjectBP/Blueprints/WidgetBP/Inventory/WB_ConsumableList.Select Consumable ` (`self.ConsumableWidget`))
      (else
        (`KismetSystemLibrary.K2_ClearAndInvalidateTimerHandle` (`self.ConsumableTimer`))
        (`self.Use Selected Consumbale`)))))

(event `Open Consumable Menu Ex`
  (bind _returnvalue (`|CreateWidget` "/Game/GProjectBP/Blueprints/WidgetBP/Inventory/WB_ConsumableList.WB_ConsumableList_C"))
  (bind _output_get (set `self.ConsumableWidget` _returnvalue))
  (`UserWidget.AddToViewport` _output_get 0)
  (set `self.bIsConsumableOpen` true))

(fn `Throw Item`
  (params (inItem :type "GPItem Object Reference") (inThrowStack :type Boolean))
  (locals (Item :type "GPItem Object Reference") (ThrowStack :type Boolean) (ThrowAmount :type Integer :default 0))
  (bind _returnvalue (`self.GetInventoryItemCount` inItem))
  (bind _throwamount (`local.ThrowAmount`))
  (bind _returnvalue_2 (`self.GetTransform` (`self.PlayerCharacter`)))
  (bind _maxstack (`GPItem.MaxStack` (`local.Item`)))
  (bind _rotation (.rotation _returnvalue_2))
  (set `local.Item` inItem)
  (set `local.ThrowStack` inThrowStack)
  (if (>= _returnvalue 1)
    (if (> _maxstack 0)
      (if (`local.ThrowStack`)
        (set `local.ThrowAmount` (`KismetMathLibrary.Clamp` _returnvalue 1 _maxstack))
        (else
          (set `local.ThrowAmount` 1)))
      (else
        (`KismetSystemLibrary.PrintString` "Hello")
        (set `local.ThrowAmount` _returnvalue)))
    (bind _returnvalue_3 (`|SpawnActorFromClass` (`GPItem.SpawningActor` (`local.Item`)) _returnvalue_2 "AdjustIfPossibleButAlwaysSpawn" "OverrideRootScale" null null))
    (bind _asbp_gppickup_item_base (cast `/Game/GProjectBP/Blueprints/Objects/PickupItems/BP_GPPickupItemBase` _returnvalue_3)
      (:`then`
        (`PrimitiveComponent.AddImpulse` (`/Game/GProjectBP/Blueprints/Objects/PickupItems/BP_GPPickupItemBase.ItemMesh` _asbp_gppickup_item_base) (+ (* (`KismetMathLibrary.GetForwardVector` _rotation) 600.0) (* (`KismetMathLibrary.GetUpVector` _rotation) 200.0)) "None" true)
        (set `/Game/GProjectBP/Blueprints/Objects/PickupItems/BP_GPPickupItemBase.ItemCount` _throwamount _asbp_gppickup_item_base)
        (`self.RemoveInventoryItem` (`local.Item`) _throwamount))
      (:`CastFailed`
        (`KismetSystemLibrary.PrintString` "cf")))))

(fn `Use Item`
  (params (InItem :type "GPItem Object Reference"))
  (locals (Item :type "GPItem Object Reference"))
  (bind _currentweaponactor (`GPCharacterBase.CurrentWeaponActor` (`self.PlayerCharacter`)))
  (bind _output_get (set `local.Item` InItem))
  (if (`KismetSystemLibrary.IsValidClass` (`GPItem.GrantedAbility` _output_get))
    (switch `name` (`.Name` (break `PrimaryAssetType` (`GPItem.ItemType` (`local.Item`))))
      (:`Consumable`
        (`self.SetSlottedItem` (make `GPItemSlot` "Consumable" 1) (`local.Item`))
        (`/Game/GProjectBP/Blueprints/BP_PlayerCharacter.UseSlottedConsumable` (`self.PlayerCharacter`)))
      (:`Attachment`
        (bind _asgpitem_attachment (cast `GPItemAttachment` (`local.Item`)))
        (`KismetSystemLibrary.PrintString` "attachmentclick")
        (bind _returnvalue (`GPWeaponActorBase.AddAttachment` (`GPCharacterBase.CurrentWeaponActor` (`self.PlayerCharacter`)) _asgpitem_attachment))
        (`/Engine/EditorBlueprintResources/StandardMacros.IsValid` _returnvalue ; Add replaced item to inventory
          (:`Is Valid`
            (`KismetSystemLibrary.PrintString` (`KismetSystemLibrary.GetDisplayName` _returnvalue))
            (`self.AddInventoryItem` _returnvalue 1 1 false)))))
    (else
      (switch `name` (`.Name` (break `PrimaryAssetType` (`GPItem.ItemType` (`local.Item`))))
        (:`Default`
          (`self.Throw Item` (`local.Item`) true))
        (:`Attachment`
          (bind _asgpitem_attachment_2 (cast `GPItemAttachment` (`local.Item`)))
          (if (`GPWeaponActorBase.IsAttachableItem` _currentweaponactor _asgpitem_attachment_2)
            (bind _returnvalue_2 (`GPWeaponActorBase.AddAttachment` _currentweaponactor _asgpitem_attachment_2))
            (`self.RemoveInventoryItem` _asgpitem_attachment_2)
            (`self.ClientAttachmentChanged` (`GPCharacterBase.CurrentWeaponSlot` (`self.PlayerCharacter`)) _asgpitem_attachment_2)
            (`/Engine/EditorBlueprintResources/StandardMacros.IsValid` _returnvalue_2 ; Add replaced item to inventory
              (:`Is Valid`
                (`self.AddInventoryItem` _returnvalue_2 1 1 false)))))))))

(fn `UserConstructionScript`)