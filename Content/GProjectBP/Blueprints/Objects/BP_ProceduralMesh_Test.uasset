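; Test actor that breaks a static mesh into chunks at BeginPlay using procedural mesh slicing.
; The construction script copies the static mesh and its materials into a procedural mesh with collision.
; Repeated capped slices cut random chunks, or in even mode cycle through chunks, along enabled axes at random positions, optionally following actor rotation.
; Chunks below minimum size stop being sliced, and each new half receives a random offset.
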(event `self.ReceiveBeginPlay`
  (if (`self.SliceXAxis`)
    (`KismetArrayLibrary.Array_Add` (`self.SliceAxisSelector`)))
  (if (`self.SliceYAxis`)
    (`KismetArrayLibrary.Array_Add` (`self.SliceAxisSelector`) 1))
  (if (`self.SliceZAxis`)
    (`KismetArrayLibrary.Array_Add` (`self.SliceAxisSelector`) 2))
  (if (`self.SliceRandomly`)
    (`self.SliceMeshRandom`)
    (else
      (`self.SliceMeshEven`))))

(fn `SliceMeshEven`
  (locals (SelectedMesh :type "ProceduralMeshComponent Object Reference" :default null) (NewProcMesh :type "ProceduralMeshComponent Object Reference" :default null) (EvenProcMeshArray :type "Array of ProceduralMeshComponent Object Reference") (Rand :type Integer))
  (bind _proceduralmesh (`self.ProceduralMesh`))
  (bind _selectedmesh (`local.SelectedMesh`))
  (bind _newprocmesh (`local.NewProcMesh`))
  (bind (_outitem _outindex) (`KismetArrayLibrary.Array_Random` (`local.EvenProcMeshArray`)))
  (`KismetArrayLibrary.Array_Add` (`self.ProcMeshArray`) _proceduralmesh)
  (`KismetArrayLibrary.Array_Add` (`local.EvenProcMeshArray`) _proceduralmesh)
  (for _ (range (+ (`self.SliceTime`) 1))
    (set `local.SelectedMesh` _outitem :!label _label)
    (if (== _outindex -1)
      (if (== (`KismetArrayLibrary.Array_Length` (`self.ProcMeshArray`)) 0)
        (break)
        (else
          (set `local.EvenProcMeshArray` (`self.ProcMeshArray`))
          (goto _label)))
      (elif (`self.Check Chunk Size` (`local.SelectedMesh`))
        (`KismetArrayLibrary.Array_RemoveItem` (`self.ProcMeshArray`) _selectedmesh)
        (`KismetArrayLibrary.Array_RemoveItem` (`local.EvenProcMeshArray`) _selectedmesh)
        (goto _label)
        (else
          (set `local.Rand` (`KismetArrayLibrary.Array_Random` (`self.SliceAxisSelector`)))
          (bind _outotherhalfprocmesh (`KismetProceduralMeshLibrary.SliceProceduralMesh` (`local.SelectedMesh`) (`self.Random Position extent` (`local.SelectedMesh`)) (`self.Random Slice Plane Normal` (`local.Rand`)) true "CreateNewSectionForCap" "/Game/Geometry/Meshes/XY.XY"))
          (set `local.NewProcMesh` _outotherhalfprocmesh)
          (if (not (`self.Check Chunk Size` (`local.NewProcMesh`)))
            (`KismetArrayLibrary.Array_Add` (`self.ProcMeshArray`) _newprocmesh))
          (`SceneComponent.K2_AddLocalOffset` _newprocmesh (`self.Make Chunk Offset` (`local.Rand`)) false true)
          (`KismetArrayLibrary.Array_RemoveItem` (`local.EvenProcMeshArray`) (`local.SelectedMesh`)))))))

(fn `SliceMeshRandom`
  (locals (SelectedMesh :type "ProceduralMeshComponent Object Reference" :default null) (NewProcMesh :type "ProceduralMeshComponent Object Reference" :default null) (Rand :type Integer))
  (bind _newprocmesh (`local.NewProcMesh`))
  (bind _selectedmesh (`local.SelectedMesh`))
  (bind (_outitem _outindex) (`KismetArrayLibrary.Array_Random` (`self.ProcMeshArray`)))
  (`KismetArrayLibrary.Array_Add` (`self.ProcMeshArray`) (`self.ProceduralMesh`))
  (for _ (range (+ (`self.SliceTime`) 1))
    (set `local.SelectedMesh` _outitem :!label _label)
    (if (== _outindex -1)
      (break)
      (elif (`self.Check Chunk Size` (`local.SelectedMesh`))
        (`KismetArrayLibrary.Array_RemoveItem` (`self.ProcMeshArray`) (`local.SelectedMesh`))
        (goto _label)
        (else
          (set `local.Rand` (`KismetArrayLibrary.Array_Random` (`self.SliceAxisSelector`)))
          (bind _outotherhalfprocmesh (`KismetProceduralMeshLibrary.SliceProceduralMesh` _selectedmesh (`self.Random Position extent` _selectedmesh) (`self.Random Slice Plane Normal` (`local.Rand`)) true "CreateNewSectionForCap" "/Game/Geometry/Meshes/XY.XY"))
          (set `local.NewProcMesh` _outotherhalfprocmesh)
          (if (not (`self.Check Chunk Size` (`local.NewProcMesh`)))
            (`KismetArrayLibrary.Array_Add` (`self.ProcMeshArray`) _newprocmesh))
          (`SceneComponent.K2_AddLocalOffset` _newprocmesh (`self.Make Chunk Offset` (`local.Rand`)) false true))))))

(fn `UserConstructionScript`
  (bind _staticmesh (`self.StaticMesh`))
  (`KismetProceduralMeshLibrary.CopyProceduralMeshFromStaticMeshComponent` _staticmesh 0 (`self.ProceduralMesh`) true)
  (for (_array_element _array_index) (`MeshComponent.GetMaterials` _staticmesh)
    (`PrimitiveComponent.SetMaterial` (`self.ProceduralMesh`) _array_index _array_element)))