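; Interactable setup terminal actor that opens the player's setup UI.
; On BeginPlay it labels its prompt widget "Setup"; interaction events show or hide that prompt.
; Interact reveals the SetupWidget held by BP_PlayerController_Setup, switches input to UI-only and swaps the panel's materials.
; Hiding the prompt also collapses the setup widget, but leaves input mode and materials unchanged.
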(event `self.ReceiveBeginPlay`
  (bind _aswb_hud_interaction_base (cast `/Game/GProjectBP/Blueprints/WidgetBP/Objects/WB_HUD_InteractionBase` (`WidgetComponent.GetWidget` (`self.Text`))))
  (`/Game/GProjectBP/Blueprints/WidgetBP/Objects/WB_HUD_InteractionBase.Set Action Name` _aswb_hud_interaction_base "Setup"))

(event `GPInteractionInterface.Interact`
  (params (InstigatorPawn :type "Pawn Object Reference"))
  (bind _panel (`self.Panel`))
  (bind _asbp_player_controller_setup (cast `/Game/GProjectBP/Blueprints/BP_PlayerController_Setup` (`Pawn.GetController` InstigatorPawn) :!pure true))
  (bind _setup_widget (`/Game/GProjectBP/Blueprints/BP_PlayerController_Setup.Setup Widget` _asbp_player_controller_setup))
  (`WidgetBlueprintLibrary.SetInputMode_UIOnlyEx` _asbp_player_controller_setup _setup_widget)
  (`Widget.SetVisibility` _setup_widget "Visible")
  (`PrimitiveComponent.SetMaterial` _panel 0 "/Game/Geometry/ModularSFPack2/ModularSci_Comm/Materials/MI_Terminal_A_UI_1.MI_Terminal_A_UI_1")
  (`PrimitiveComponent.SetMaterial` _panel 1 "/Game/Geometry/ModularSFPack2/ModularSci_Comm/Materials/MI_Terminal_A_UI_Trim_Pan.MI_Terminal_A_UI_Trim_Pan")
  (`PrimitiveComponent.SetMaterial` _panel 4 "/Game/Geometry/ModularSFPack2/ModularSci_Comm/Materials/MI_Terminal_A_UI_Trim_Pan.MI_Terminal_A_UI_Trim_Pan"))

(event `GPInteractionInterface.ShowInteractUI`
  (params (InstigatorPawn :type "Pawn Object Reference"))
  (`SceneComponent.SetVisibility` (`self.Text`) true true))

(event `GPInteractionInterface.HideInteractUI`
  (params (InstigatorPawn :type "Pawn Object Reference"))
  (`Widget.SetVisibility` (`/Game/GProjectBP/Blueprints/BP_PlayerController_Setup.Setup Widget` (cast `/Game/GProjectBP/Blueprints/BP_PlayerController_Setup` (`Pawn.GetController` InstigatorPawn) :!pure true)) "Collapsed")
  (`SceneComponent.SetVisibility` (`self.Text`) false true))

(fn `GetInteractText`
  (params (InstigatorPawn :type "Pawn Object Reference"))
  (returns (ReturnValue :type Text))
  (return "Terminal"))

(fn `UserConstructionScript`)