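; Interactable setup terminal that opens the mission selection screen for the player.
; Interact toggles Activate and Deactivate, which swap panel materials, lock idle turning, create or remove the WB_MissionSelect_Main widget, and switch cursor and input mode.
; Forward and Backward timelines feed Update to move the player's spring arm in and back out.
; Hiding the interact prompt also deactivates a terminal in use; the world-space widget component path is mostly disconnected.
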(event `InputAxis|MouseX` :consume false
  (params (AxisValue :type "Float (single-precision)")))

(event `InputAxis|MouseY` :consume false
  (params (AxisValue :type "Float (single-precision)")))

(event `self.ReceiveBeginPlay`
  (bind _aswb_hud_interaction_base (cast `/Game/GProjectBP/Blueprints/WidgetBP/Objects/WB_HUD_InteractionBase` (`WidgetComponent.GetWidget` (`self.Text`))))
  (`/Game/GProjectBP/Blueprints/WidgetBP/Objects/WB_HUD_InteractionBase.Set Action Name` _aswb_hud_interaction_base "Select Mission"))

(event `Activate`
  (params (Pawn :type "Pawn Object Reference"))
  (bind _asbp_player_character (cast `/Game/GProjectBP/Blueprints/BP_PlayerCharacter` Pawn :!pure true))
  (bind _panel (`self.Panel`))
  (bind _springarm (`/Game/GProjectBP/Blueprints/BP_PlayerCharacter.SpringArm` _asbp_player_character))
  (bind _asplayer_controller (cast `PlayerController` (`Pawn.GetController` _asbp_player_character) :!pure true))
  (`PrimitiveComponent.SetMaterial` _panel 0 "/Game/Geometry/ModularSFPack2/ModularSci_Comm/Materials/MI_Terminal_A_UI_1.MI_Terminal_A_UI_1")
  (`PrimitiveComponent.SetMaterial` _panel 1 "/Game/Geometry/ModularSFPack2/ModularSci_Comm/Materials/MI_Terminal_A_UI_Trim_Pan.MI_Terminal_A_UI_Trim_Pan")
  (`PrimitiveComponent.SetMaterial` _panel 3 "/Game/Geometry/ModularSFPack2/ModularSci_Comm/Materials/MI_Terminal_A_UI_Trim_Pan.MI_Terminal_A_UI_Trim_Pan")
  (set `self.bUsing` true)
  (set `/Game/GProjectBP/Blueprints/BP_PlayerCharacter.bIdleTurnLock` true _asbp_player_character)
  (set `self.Spring Arm` _springarm)
  (set `self.Relative Location` (`SceneComponent.RelativeLocation` _springarm))
  (set `PlayerController.bShowMouseCursor` true _asplayer_controller)
  (bind _returnvalue (`|CreateWidget` "/Game/GProjectBP/Blueprints/WidgetBP/Objects/MIssionSelector/WB_MissionSelect_Main.WB_MissionSelect_Main_C" _asplayer_controller))
  (`UserWidget.AddToViewport` _returnvalue 0)
  (bind _output_get (set `self.WB_MS` _returnvalue))
  (`WidgetBlueprintLibrary.SetInputMode_GameAndUIEx` _asplayer_controller _output_get "DoNotLock" false)
  (`|ExecutionSequence`
    (:`then_0`
      (bind (_direction _camdist _camoffset _widgetsize) (`Timeline|Forward` :!via `PlayFromStart` :!label _label)
        (:`Update`
          (`self.Update` _camdist _camoffset _widgetsize (`self.AddedComponent`)))))
    (:`then_1`
      (bind (_direction_2 _camdist_2 _camoffset_2 _widgetsize_2) (`Timeline|Backward` :!via `Stop` :!label _label_2)
        (:`Update`
          (`self.Update` _camdist_2 _camoffset_2 _widgetsize_2 (`self.AddedComponent`)))
        (:`Finished`
          (`self.ClearWidgetComp`))))))

(event `Deactivate`
  (params (Object :type "Pawn Object Reference"))
  (bind _asbp_player_character (cast `/Game/GProjectBP/Blueprints/BP_PlayerCharacter` Object :!pure true))
  (bind _panel (`self.Panel`))
  (bind _asplayer_controller (cast `PlayerController` (`Pawn.GetController` _asbp_player_character) :!pure true))
  (`PrimitiveComponent.SetMaterial` _panel 0 "/Game/Geometry/ModularSFPack2/ModularSci_Comm/Materials/MI_Terminal_A_UI_1B.MI_Terminal_A_UI_1B")
  (`PrimitiveComponent.SetMaterial` _panel 1 "/Game/Geometry/ModularSFPack2/ModularSci_Comm/Materials/MI_Terminal_A_UI_TrimB.MI_Terminal_A_UI_TrimB")
  (`PrimitiveComponent.SetMaterial` _panel 3 "/Game/Geometry/ModularSFPack2/ModularSci_Comm/Materials/MI_Terminal_A_UI_TrimB.MI_Terminal_A_UI_TrimB")
  (set `self.bUsing` false)
  (set `/Game/GProjectBP/Blueprints/BP_PlayerCharacter.bIdleTurnLock` false _asbp_player_character)
  (`WidgetBlueprintLibrary.SetInputMode_GameOnly` _asplayer_controller)
  (`/Game/GProjectBP/Blueprints/WidgetBP/Objects/MIssionSelector/WB_MissionSelect_Main.Remove Widget` (`self.WB_MS`))
  (set `PlayerController.bShowMouseCursor` false _asplayer_controller)
  (`|ExecutionSequence`
    (:`then_0`
      (goto _label_2 :!via `PlayFromStart`))
    (:`then_1`
      (goto _label :!via `Stop`))))

(event `GPInteractionInterface.Interact`
  (params (InstigatorPawn :type "Pawn Object Reference"))
  (if (`self.bUsing`)
    (`self.Deactivate` InstigatorPawn)
    (`SceneComponent.SetVisibility` (`self.Text`) true true)
    (else
      (`self.Activate` InstigatorPawn)
      (`SceneComponent.SetVisibility` (`self.Text`) false true)
      (`GameplayStatics.PlaySound2D` "/Game/FXAssets/SFX/SFX_OpenSetupLevel.SFX_OpenSetupLevel" 1.0 1.0 0.0 null InstigatorPawn))))

(event `GPInteractionInterface.ShowInteractUI`
  (params (InstigatorPawn :type "Pawn Object Reference"))
  (`SceneComponent.SetVisibility` (`self.Text`) true true))

(event `GPInteractionInterface.HideInteractUI`
  (params (InstigatorPawn :type "Pawn Object Reference"))
  (if (`self.bUsing`)
    (`self.Deactivate` InstigatorPawn))
  (`SceneComponent.SetVisibility` (`self.Text`) false true))

(fn `GetInteractText`
  (params (InstigatorPawn :type "Pawn Object Reference"))
  (returns (ReturnValue :type Text))
  (return "Terminal"))

(fn `UserConstructionScript`)