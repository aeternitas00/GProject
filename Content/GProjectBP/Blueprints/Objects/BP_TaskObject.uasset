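; Mission task actor with a billboard icon that marks an objective in the world and chains to follow-up task objects.
; The construction script builds a dynamic billboard material from icon, color, emissive power and size.
; Completion fires once, removing the task and marker from the HUD manager.
; If no active mission tasks remain, it waits briefly, activates the next tasks with world markers and optionally shows a tutorial notification.
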(event `UpdateActor`
  (bind _size (`self.Size`))
  (bind _returnvalue (`KismetMaterialLibrary.CreateDynamicMaterialInstance` (`.Material` (break `MaterialSpriteElement` (`|GetArrayItem` (`MaterialBillboardComponent.Elements` (`self.MaterialBillboard`)))))))
  (set `self.DynamicMaterial` _returnvalue)
  (`MaterialInstanceDynamic.SetTextureParameterValue` (`self.DynamicMaterial`) "Texture" (`self.Icon`))
  (`MaterialInstanceDynamic.SetVectorParameterValue` (`self.DynamicMaterial`) "Color" (`self.Color`))
  (`MaterialInstanceDynamic.SetScalarParameterValue` (`self.DynamicMaterial`) "EmissivePower" (`self.EmissivePower`))
  (`MaterialBillboardComponent.SetElements` (`self.MaterialBillboard`) (`|MakeArray` (make `MaterialSpriteElement` :`Material` (`self.DynamicMaterial`) :`BaseSizeX` _size :`BaseSizeY` _size))))

(event `Init task info`
  (for _array_element (`self.NextObjects`)
    (`BlueprintSetLibrary.Set_Add` (`self.NextTaskIdx`) (`/Game/GProjectBP/Blueprints/Objects/BP_TaskObject.TaskIdx` _array_element))))

(event `Task Complete`
  (bind _hud_manager (`/Game/ProHUDV2/Blueprints/Libraries/BP_PHV2_Functions.GetHUDManager`))
  (bind _info (`self.Info`))
  (bind _nexttaskidx (`self.NextTaskIdx`))
  (`/Engine/EditorBlueprintResources/StandardMacros.DoOnce` false
    (:`Completed`
      (`/Game/ProHUDV2/Blueprints/Libraries/BPi_HUDManagerV2.RemoveTask` (`/Game/ProHUDV2/Blueprints/Libraries/BP_PHV2_Functions.GetHUDManager`) (`self.MissionName`) "NewEnumerator0" (`self.TaskIdx`) false null)
      (`/Game/ProHUDV2/Blueprints/Libraries/BPi_HUDManagerV2.RemoveWorldMarker` (`/Game/ProHUDV2/Blueprints/Libraries/BP_PHV2_Functions.GetHUDManager`) (`self.MaterialBillboard`))
      (bind _activetasks (`/Game/ProHUDV2/Blueprints/Libraries/BPi_HUDManagerV2.GetActiveTasks` _hud_manager (`self.MissionName`)))
      (if (and (== (`BlueprintSetLibrary.Set_Length` _activetasks) 0) (!= (`BlueprintSetLibrary.Set_Length` _nexttaskidx) 0))
        (`KismetSystemLibrary.Delay` 3.0)
        (`/Game/ProHUDV2/Blueprints/Libraries/BPi_HUDManagerV2.SetActiveTasks` _hud_manager (`self.MissionName`) _nexttaskidx false)
        (for _array_element (`self.NextObjects`)
          (`/Engine/EditorBlueprintResources/StandardMacros.IsValid` _array_element
            (:`Is Valid`
              (set `/Game/GProjectBP/Blueprints/Objects/BP_TaskObject.Active` true _array_element)
              (`/Game/ProHUDV2/Blueprints/Libraries/BPi_HUDManagerV2.AddOrUpdateWorldMarker` (`/Game/ProHUDV2/Blueprints/Libraries/BP_PHV2_Functions.GetHUDManager`) (`/Game/GProjectBP/Blueprints/Objects/BP_TaskObject.MaterialBillboard` _array_element) (make `/Game/ProHUDV2/Blueprints/Structs/S_WorldMarkerInfo` "/Game/ProHUDV2/Textures/MissionNoti/T_MissionIcon_Active.T_MissionIcon_Active" 1.0 (struct :`R` 1.0 :`G` 0.434589 :`A` 1.0) false (`.ObjectName_23_8198AFFE4B09F234492F5DBDEC0E84C4` (break `/Game/ProHUDV2/Blueprints/Structs/S_Task` (`/Game/GProjectBP/Blueprints/Objects/BP_TaskObject.Task` _array_element))) (struct :`FontInfo` (struct :`OutlineSettings` (struct :`OutlineColor` (struct :`A` 1.0)) :`Size` 24) :`Scale` 1.0 :`ColorAndOpacity` (struct)) true false (struct :`DistanceUnit` "NewEnumerator1" :`DistanceStepskm` 10 :`DistanceStepsm` 1 :`DistanceStepsmi` 10 :`DistanceStepsya` 1) (struct :`FontInfo` (struct :`OutlineSettings` (struct :`OutlineColor` (struct :`A` 1.0)) :`Size` 24) :`Scale` 1.0 :`ColorAndOpacity` (struct)) 0 false true false)))))
        (if (`KismetSystemLibrary.IsValidClass` (`.ContentWidget_5_413FF1F7411F3C5AABEA7BABE8D80ED7` (break `/Game/ProHUDV2/Blueprints/Structs/S_TutNotiInfo` _info)))
          (`/Game/ProHUDV2/Blueprints/Libraries/BPi_HUDManagerV2.CreateTutorialNotification` (`/Game/ProHUDV2/Blueprints/Libraries/BP_PHV2_Functions.GetHUDManager`) _info))))))

(fn `UserConstructionScript`
  (`self.UpdateActor`))