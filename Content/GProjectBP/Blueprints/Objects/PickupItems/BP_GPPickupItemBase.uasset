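; Base pickup item actor that gives its item to a player's inventory on interaction.
; Showing the interact UI either picks up immediately for auto-pickup items or reveals a widget with the item description, which hiding reverses.
; GiveItem adds type, count and level through BP_PlayerController_Game_abptest; on success it sets that controller as owner, calls ClientPickup for the sound and destroys the actor.
; ItemSetup and GetInteractText are empty stubs.
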(event `Client Pickup`
  (`GameplayStatics.PlaySoundAtLocation` (`self.PickupSound`) (`SceneComponent.K2_GetComponentLocation` (`self.ItemMesh`)) (struct) 1.0 1.0 0.0 null null null))

(event `self.Interact`
  (params (InstigatorPawn :type "Pawn Object Reference"))
  (`self.GiveItem` InstigatorPawn))

(event `self.ShowInteractUI`
  (params (InstigatorPawn :type "Pawn Object Reference"))
  (if (`self.bIsAutoPickup`)
    (`self.Interact` InstigatorPawn)
    (elif (not (`self.bIsWidgetVisible`))
      (bind _aswb_hud_pickup_item (cast `/Game/GProjectBP/Blueprints/WidgetBP/HUD/WB_HUD_PickupItem` (`WidgetComponent.GetUserWidgetObject` (`self.Widget`))))
      (`Widget.SetVisibility` (`/Game/GProjectBP/Blueprints/WidgetBP/HUD/WB_HUD_PickupItem.PickupBorder` _aswb_hud_pickup_item) "Visible")
      (set `self.bIsWidgetVisible` true)
      (`TextBlock.SetText` (`/Game/GProjectBP/Blueprints/WidgetBP/HUD/WB_HUD_PickupItem.ItemTextBlock` _aswb_hud_pickup_item) (`GPItem.ItemDescription` (`self.ItemType`))))))

(event `self.HideInteractUI`
  (params (InstigatorPawn :type "Pawn Object Reference"))
  (if (`self.bIsWidgetVisible`)
    (bind _aswb_hud_pickup_item (cast `/Game/GProjectBP/Blueprints/WidgetBP/HUD/WB_HUD_PickupItem` (`WidgetComponent.GetUserWidgetObject` (`self.Widget`))))
    (`Widget.SetVisibility` (`/Game/GProjectBP/Blueprints/WidgetBP/HUD/WB_HUD_PickupItem.PickupBorder` _aswb_hud_pickup_item) "Hidden")
    (set `self.bIsWidgetVisible` false)))

(fn `GetInteractText`
  (params (InstigatorPawn :type "Pawn Object Reference"))
  (returns (ReturnValue :type Text))
  (return ""))

(fn `GiveItem`
  (params (Target :type "Pawn Object Reference"))
  (bind _asbp_player_controller_game_abptest (cast `/Game/GProjectBP/Blueprints/BP_PlayerController_Game_abptest` (`Pawn.GetController` Target) :!pure true))
  (bind _returnvalue (`GProjectPlayerController.AddInventoryItem` _asbp_player_controller_game_abptest (`self.ItemType`) (`self.ItemCount`) (`self.ItemLevel`) true))
  (if _returnvalue
    (`self.SetOwner` _asbp_player_controller_game_abptest)
    (`self.Client Pickup`)
    (`self.K2_DestroyActor`)
    (return)))

(fn `ItemSetup`)

(fn `UserConstructionScript`)