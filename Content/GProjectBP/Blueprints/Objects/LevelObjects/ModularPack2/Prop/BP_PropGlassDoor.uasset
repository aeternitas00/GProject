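; BP_PropGlassDoor is an interactable sliding glass door prop for modular levels.
; Interact toggles IsOpen and plays or reverses a timeline that lerps between the DoorClosed and DoorOpen positions.
; The two static meshes slide as mirrored panels, the second using the negated relative location.
; GetInteractText returns an empty string, so the door supplies no prompt text.
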(event `GPInteractionInterface.Interact`
  (params (InstigatorPawn :type "Pawn Object Reference"))
  (if (`self.bIsOpen`)
    (set `self.bIsOpen` false)
    (bind (_direction _doorposition) (`Timeline|타임라인_0` :!via `Reverse` :!label _label)
      (:`Update`
        (bind _returnvalue (`KismetMathLibrary.VLerp` (`self.DoorClosed`) (`self.DoorOpen`) _doorposition))
        (`SceneComponent.K2_SetRelativeLocation` (`self.StaticMesh`) _returnvalue false false)
        (`SceneComponent.K2_SetRelativeLocation` (`self.StaticMesh1`) (* _returnvalue -1.0) false false)))
    (else
      (set `self.bIsOpen` true)
      (goto _label))))

(fn `GetInteractText`
  (params (InstigatorPawn :type "Pawn Object Reference"))
  (returns (ReturnValue :type Text))
  (return ""))

(fn `UserConstructionScript`)