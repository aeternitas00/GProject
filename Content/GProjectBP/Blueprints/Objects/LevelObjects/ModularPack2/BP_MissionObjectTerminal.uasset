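; BP_MissionObjectTerminal is an interactable mission-object terminal, labelled "Terminal" in its interact text.
; Interact runs the parent logic, then a DoOnce swaps the Panel's screen and trim materials on first use.
; Task start spawns a sound attached to the static mesh and keeps a reference, which task finish uses to stop and destroy it.
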(event `GPInteractionInterface.Interact`
  (params (InstigatorPawn :type "Pawn Object Reference"))
  (bind _panel (`self.Panel`))
  (`parent.Interact` InstigatorPawn)
  (`/Engine/EditorBlueprintResources/StandardMacros.DoOnce` false
    (:`Completed`
      (`PrimitiveComponent.SetMaterial` _panel 0 "/Game/Geometry/ModularSFPack2/ModularSci_Comm/Materials/MI_Terminal_A_UI_1.MI_Terminal_A_UI_1")
      (`PrimitiveComponent.SetMaterial` _panel 1 "/Game/Geometry/ModularSFPack2/ModularSci_Comm/Materials/MI_Terminal_A_UI_Trim_Pan.MI_Terminal_A_UI_Trim_Pan")
      (`PrimitiveComponent.SetMaterial` _panel 4 "/Game/Geometry/ModularSFPack2/ModularSci_Comm/Materials/MI_Terminal_A_UI_Trim_Pan.MI_Terminal_A_UI_Trim_Pan"))))

(event `self.On Task Started`
  (`self.Play Sound`))

(event `Play Sound`
  (bind _returnvalue (`GameplayStatics.SpawnSoundAttached` (`self.Sound`) (`self.StaticMeshComponent`) "None" (0.0 0.0 0.0) (struct) "KeepRelativeOffset" true 1.0 1.0 0.0 null null false))
  (set `self.NewVar_0` _returnvalue))

(event `self.On Task FInished`
  (bind _newvar_0 (`self.NewVar_0`))
  (`AudioComponent.Stop` _newvar_0)
  (`ActorComponent.K2_DestroyComponent` _newvar_0))

(fn `GetInteractText`
  (params (InstigatorPawn :type "Pawn Object Reference"))
  (returns (ReturnValue :type Text))
  (return "Terminal"))

(fn `UserConstructionScript`)