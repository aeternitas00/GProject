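; BP_SciFIDoor is an interactable sci-fi door level object that toggles between open and closed.
; Interact flips IsOpen and plays or reverses a timeline, whose DoorPosition track lerps the relative location of DoorSmallA between DoorClosed and DoorOpen.
; Opening also activates two SteamDoor effect components, while closing does not.
; GetInteractText returns an empty string, so the door supplies no prompt text.
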(event `GPInteractionInterface.Interact`
  (params (InstigatorPawn :type "Pawn Object Reference"))
  (if (`self.bIsOpen`)
    (set `self.bIsOpen` false)
    (bind (_direction _doorposition) (`Timeline|Timeline_0` :!via `Reverse` :!label _label)
      (:`Update`
        (`SceneComponent.K2_SetRelativeLocation` (`self.Door_Small_A`) (`KismetMathLibrary.VLerp` (`self.DoorClosed`) (`self.DoorOpen`) _doorposition) false false)))
    (else
      (set `self.bIsOpen` true)
      (`ActorComponent.Activate` (`self.SteamDoor`) false)
      (`ActorComponent.Activate` (`self.SteamDoor2`) false)
      (goto _label))))

(fn `GetInteractText`
  (params (InstigatorPawn :type "Pawn Object Reference"))
  (returns (ReturnValue :type Text))
  (return ""))

(fn `UserConstructionScript`)