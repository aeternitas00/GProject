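; Spawner component that periodically spawns random enemies at an owner-relative offset, up to a maximum pool size.
; Component activation drives a looping timer; the component deactivates when the pool is full, and a spawned character's death updates the pool and reactivates it.
; The enemy list and drop table come from BP_GameState.
; Each spawn receives randomized drop items, rolled from chance and count ranges matching the level difficulty.
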(event `self.ReceiveBeginPlay`
  (add `self.OnComponentActivated` (delegate `On Spawner Activated`))
  (add `self.OnComponentDeactivated` (delegate `On Spawner Deactivated`))
  (set `self.Spawnable Enemy List` (`self.Get Spawnable List`))
  (`self.Activate` false))

(event `On Spawner Activated` :!signature `self.OnComponentActivated`
  (params (Component :type "ActorComponent Object Reference") (bReset :type Boolean))
  (bind _returnvalue (`KismetSystemLibrary.K2_SetTimerDelegate` (delegate `Spawn Character`) (`self.Spawn Delay`) true)))

(event `On Spawner Deactivated` :!signature `self.OnComponentDeactivated`
  (params (Component :type "ActorComponent Object Reference"))
  (`KismetSystemLibrary.K2_ClearAndInvalidateTimerHandle` (stale `On Spawner Activated` _returnvalue)))

(event `Spawn Character`
  (bind (_spawnable_item_list _difficultiyoflevel) (`self.Get Dropable Item`))
  (bind _spawnable_enemy_list (`self.Spawnable Enemy List`))
  (bind _rotation (.rotation (`Actor.GetTransform` (`self.GetOwner`))))
  (if (>= (`KismetArrayLibrary.Array_Length` (`self.SpawnPool`)) (`self.MaxSpawnNum`))
    (`self.Deactivate`)
    (else
      (if (== (`KismetArrayLibrary.Array_Length` _spawnable_enemy_list) 0)
        (set `self.Spawnable Enemy List` (`self.Get Spawnable List`)))
      (bind _returnvalue (`|SpawnActorFromClass` (`.CharacterClass_9_3CEC45F34AB43E9D72ACBAB532734A1E` (break `/Game/GProjectBP/DataAsset/AssetDataStruct` (`KismetArrayLibrary.Array_Random` _spawnable_enemy_list))) (`KismetMathLibrary.MakeTransform` (+ (`KismetMathLibrary.GreaterGreater_VectorRotator` (`self.Offset`) _rotation) (.location (`Actor.GetTransform` (`self.GetOwner`)))) _rotation (.scale (`Actor.GetTransform` (`self.GetOwner`)))) "AdjustIfPossibleButAlwaysSpawn" "OverrideRootScale" null null))
      (`/Engine/EditorBlueprintResources/StandardMacros.IsValid` _returnvalue
        (:`Is Valid`
          (add `/Game/GProjectBP/Blueprints/BP_CharacterBase.OnCharacterDeathBP` _returnvalue (delegate `Pool Update`))
          (`KismetArrayLibrary.Array_Add` (`self.SpawnPool`) _returnvalue)
          (for _array_element _spawnable_item_list
            (bind ((`ItemID_33_2E11982148EB72D6F81CD893CC5C2527` _itemid) (`DropChance_31_B14BA04645A36CB36BC13C89327B8A6E` _dropchance)) (break `/Game/GProjectBP/DataAsset/ItemDropStruct` _array_element))
            (for _array_element_2 _dropchance
              (bind (_minrangelv _maxrangelv _mindropcount _maxdropcount _dropchance_2) (break `/Game/GProjectBP/DataAsset/ItemDropChanceByLevel` _array_element_2))
              (if (and (>= _difficultiyoflevel _minrangelv) (<= _difficultiyoflevel _maxrangelv))
                (if (>= _dropchance_2 (`KismetMathLibrary.RandomFloat`))
                  (`BlueprintMapLibrary.Map_Add` (`/Game/GProjectBP/Blueprints/BP_CharacterBase.DropItem` _returnvalue) _itemid (make `GPItemData` (`KismetMathLibrary.RandomIntegerInRange` _mindropcount _maxdropcount)))
                  (break)
                  (else
                    (break)))))))))))

(event `Pool Update`
  (`KismetArrayLibrary.Array_RemoveItem` (`self.SpawnPool`) (stale `Spawn Character` _returnvalue))
  (if (not (`self.IsActive`))
    (`self.Activate` false)))