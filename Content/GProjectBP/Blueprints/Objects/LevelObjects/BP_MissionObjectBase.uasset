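; Base interactable level object for missions, completed through a one-time, timed progress sequence.
; On BeginPlay it caches its progress widget, labels the interaction prompt with its MissionType, and registers a HUD task and world marker.
; Interacting hides the prompt and plays a timeline that drives the progress bar, then reports the MissionType to BP_GameState on finish.
; The prompt cannot reappear once the sequence starts.
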(event `self.ReceiveBeginPlay`
  (bind _hud_manager (`/Game/ProHUDV2/Blueprints/Libraries/BP_PHV2_Functions.GetHUDManager`))
  (bind _missiontype (`self.MissionType`))
  (bind _returnvalue (`KismetTextLibrary.Conv_StringToText` _missiontype))
  (bind _aswb_mission_progress_bar (cast `/Game/GProjectBP/Blueprints/WidgetBP/Objects/WB_MissionProgressBar` (`WidgetComponent.GetWidget` (`self.Progress`))))
  (set `self.CaptureProgress` _aswb_mission_progress_bar)
  (bind _aswb_hud_interaction_base (cast `/Game/GProjectBP/Blueprints/WidgetBP/Objects/WB_HUD_InteractionBase` (`WidgetComponent.GetWidget` (`self.Text`))))
  (`/Game/GProjectBP/Blueprints/WidgetBP/Objects/WB_HUD_InteractionBase.Set Action Name` _aswb_hud_interaction_base _missiontype)
  (`/Game/ProHUDV2/Blueprints/Libraries/BPi_HUDManagerV2.AddTask` _hud_manager "Main Object" (`|MakeArray` (make `/Game/ProHUDV2/Blueprints/Structs/S_Task` self _returnvalue _returnvalue)))
  (`/Game/ProHUDV2/Blueprints/Libraries/BPi_HUDManagerV2.AddOrUpdateWorldMarker` :`self` _hud_manager :`MarkerObject` (`self.MaterialBillboard`)))

(event `self.Interact`
  (params (InstigatorPawn :type "Pawn Object Reference"))
  (`/Engine/EditorBlueprintResources/StandardMacros.DoOnce` false
    (:`Completed`
      (`SceneComponent.SetVisibility` (`self.Progress`) true true)
      (set `self.bIsRunning` true)
      (`self.HideInteractUI` null)
      (bind (_direction _percent) (`Timeline|타임라인_0`)
        (:`Update`
          (`/Game/GProjectBP/Blueprints/WidgetBP/Objects/WB_MissionProgressBar.Update Progress` (`self.CaptureProgress`) _percent))
        (:`Finished`
          (`/Game/GProjectBP/Blueprints/BP_GameState.Update Mission Progress` (cast `/Game/GProjectBP/Blueprints/BP_GameState` (`GameplayStatics.GetGameState`) :!pure true) (`self.MissionType`)))))))

(event `self.ShowInteractUI`
  (params (InstigatorPawn :type "Pawn Object Reference"))
  (if (not (`self.bIsRunning`))
    (`SceneComponent.SetVisibility` (`self.Text`) true true)))

(event `self.HideInteractUI`
  (params (InstigatorPawn :type "Pawn Object Reference"))
  (`SceneComponent.SetVisibility` (`self.Text`) false true))

(fn `GetInteractText`
  (params (InstigatorPawn :type "Pawn Object Reference"))
  (returns (ReturnValue :type Text))
  (return ""))

(fn `UserConstructionScript`)