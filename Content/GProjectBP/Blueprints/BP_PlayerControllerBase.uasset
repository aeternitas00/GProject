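; Base player controller that caches the possessed player character and turns player input into movement, interaction and optic use.
; Each tick it feeds forward and right axis values into the controlled pawn as movement input, provided the character can perform actions.
; Input actions trigger the character's interaction component and start or stop optic use on press and release.
; A MulticastPlayMontage event plays a montage section on a given character.
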(event `self.ReceiveBeginPlay`
  (if (`self.IsLocalPlayerController`)
    (bind _asbp_player_character (cast `/Game/GProjectBP/Blueprints/BP_PlayerCharacter` (`self.K2_GetPawn`)))
    (set `self.PlayerCharacter` _asbp_player_character) ; TODO 특정 상황에서 중복 배제
  ))

(event `self.ReceiveTick`
  (params (DeltaSeconds :type "Float (single-precision)"))
  (`self.Movement Controll`))

(event `self.ReceivePossess`
  (params (PossessedPawn :type "Pawn Object Reference"))
  (bind _asbp_player_character (cast `/Game/GProjectBP/Blueprints/BP_PlayerCharacter` PossessedPawn))
  (set `self.PlayerCharacter` _asbp_player_character))

(event `InputAction|MainInteraction`
  (params (Key :type "Key Structure"))
  (bind _playercharacter (`self.PlayerCharacter`))
  (bind _interactioncomponent (`/Game/GProjectBP/Blueprints/BP_PlayerCharacter.InteractionComponent` _playercharacter))
  (:`Pressed`
    (`/Engine/EditorBlueprintResources/StandardMacros.IsValid` _playercharacter
      (:`Is Valid`
        (`/Engine/EditorBlueprintResources/StandardMacros.IsValid` _interactioncomponent
          (:`Is Valid`
            (`GPInteractionComponent.PrimaryInteract` _interactioncomponent)))))))

(event `Movement Controll`
  (bind _returnvalue (`self.K2_GetPawn`))
  (bind _returnvalue_2 (`self.GetInputAxisValue`))
  (bind _returnvalue_3 (`self.GetInputAxisValue`))
  (bind _asbp_character_base (cast `/Game/GProjectBP/Blueprints/BP_CharacterBase` _returnvalue :!pure true))
  (`/Engine/EditorBlueprintResources/StandardMacros.IsValid` _asbp_character_base
    (:`Is Valid`
      (if (`/Game/GProjectBP/Blueprints/BP_CharacterBase.CanPerformAction` _asbp_character_base)
        (if (!= _returnvalue_2 0.0)
          (`Pawn.AddMovementInput` _returnvalue (`KismetMathLibrary.Vector_Forward`) _returnvalue_2 false))
        (if (!= _returnvalue_3 0.0)
          (`Pawn.AddMovementInput` _returnvalue (`KismetMathLibrary.Vector_Right`) _returnvalue_3 false))))))

(event `InputAction|UseOptic`
  (params (Key :type "Key Structure"))
  (bind _playercharacter (`self.PlayerCharacter`))
  (:`Pressed`
    (`/Engine/EditorBlueprintResources/StandardMacros.IsValid` _playercharacter
      (:`Is Valid`
        (`/Game/GProjectBP/Blueprints/BP_PlayerCharacter.StartUsingOptic` _playercharacter))))
  (:`Released`
    (`/Engine/EditorBlueprintResources/StandardMacros.IsValid` _playercharacter
      (:`Is Valid`
        (`/Game/GProjectBP/Blueprints/BP_PlayerCharacter.StopUsingOptic` _playercharacter)))))

(event `Multicast Play Montage`
  (params (Character :type "Character Object Reference") (AnimMontage :type "AnimMontage Object Reference") (StartSectionName :type Name))
  (`Character.PlayAnimMontage` Character AnimMontage 1.0 StartSectionName))

(fn `UserConstructionScript`)