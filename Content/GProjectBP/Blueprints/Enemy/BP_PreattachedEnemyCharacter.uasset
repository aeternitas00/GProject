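; Enemy character Blueprint that activates slotted abilities and reports their montage length.
; ActivatePrioritySkill fires the slot 0 ability, while ActivateSkillBySlot fires any given slot.
; On successful activation, both pass a non-negative montage length to CallMontageDelegate; ActivateSkillBySlot returns true only in that case, whereas ActivatePrioritySkill returns the activation result.
; BeginPlay, Tick, death and construction logic only forward to the parent class.
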(event `self.ReceiveBeginPlay`
  (`parent.ReceiveBeginPlay`))

(event `self.ReceiveTick`
  (params (DeltaSeconds :type "Float (single-precision)"))
  (`parent.ReceiveTick` DeltaSeconds))

(event `self.OnDeathEvent`
  (`parent.OnDeathEvent`))

(fn `ActivatePrioritySkill`
  (returns (Success :type Boolean))
  (bind _gpitemslot (make `GPItemSlot` "Skill" 0))
  (bind _returnvalue (`self.ActivateAbilitiesWithItemSlot` _gpitemslot))
  (if _returnvalue
    (bind _length (`self.Get Slotted Ability Montage Length` _gpitemslot))
    (if (>= _length 0.0)
      (`self.MontageDelegate` _length)))
  (return _returnvalue))

(fn `ActivateSkillBySlot`
  (params (SlotNumber :type Integer))
  (returns (Success :type Boolean))
  (bind _gpitemslot (make `GPItemSlot` "Skill" SlotNumber))
  (bind _returnvalue (`self.ActivateAbilitiesWithItemSlot` _gpitemslot))
  (if _returnvalue
    (bind _length (`self.Get Slotted Ability Montage Length` _gpitemslot))
    (if (>= _length 0.0)
      (`self.MontageDelegate` _length)
      (return true)
      (else
        _)))
  (return false))

(fn `UserConstructionScript`
  (`parent.UserConstructionScript`))