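; Test enemy character Blueprint that adds death visuals on top of its parent class's logic.
; The death event switches the mesh to the Ragdoll collision profile, simulates physics on all bodies and prints a debug message.
; The multicast death event plays one of five random death animations without looping, then ends on a short delay with nothing after it.
; BeginPlay and construction only call the parent.
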(event `self.ReceiveBeginPlay`
  (`parent.ReceiveBeginPlay`))

(event `/Game/GProjectBP/Blueprints/BP_CharacterBase.OnDeathEvent`
  (bind _mesh (`self.Mesh`))
  (`parent.OnDeathEvent`)
  (`PrimitiveComponent.SetCollisionProfileName` _mesh "Ragdoll" true)
  (`SkeletalMeshComponent.SetAllBodiesSimulatePhysics` _mesh true)
  (`KismetSystemLibrary.PrintString` "enemy death event"))

(event `/Game/GProjectBP/Blueprints/BP_CharacterBase.Multicast On Death`
  (`parent.Multicast On Death`)
  (`SkeletalMeshComponent.PlayAnimation` (`self.Mesh`) (select `int` (`KismetMathLibrary.RandomIntegerInRange` 0 4) :`0` "/Game/CharactersAssets/AnimStarterPack/Death_1.Death_1" :`1` "/Game/CharactersAssets/AnimStarterPack/Death_2.Death_2" :`2` "/Game/CharactersAssets/AnimStarterPack/Death_3.Death_3" :`3` "/Game/CharactersAssets/AnimStarterPack/Death_Ironsights_1.Death_Ironsights_1" :`4` "/Game/CharactersAssets/AnimStarterPack/Death_Ironsights_2.Death_Ironsights_2" :!type "AnimationAsset Object Reference") false)
  (`KismetSystemLibrary.Delay` 0.5))

(fn `UserConstructionScript`
  (`parent.UserConstructionScript`))