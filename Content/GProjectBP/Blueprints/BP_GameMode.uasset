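; Mission game mode that runs a mission from start notification and HUD setup through completion and evac.
; Completion fires once, starting a 10-second countdown, then a timeline drives the PC_PixelData Alpha before saving and showing a paused results screen.
; Saving adds attention and a randomized, level-scaled Captain reward message, clears the current stage, and reveals uncleared stages within range, falling back to the nearest.
; The end flow assumes single-player.
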(event `Mission Start Notify`
  (bind _hud_manager (`/Game/ProHUDV2/Blueprints/Libraries/BP_PHV2_Functions.GetHUDManager`))
  (bind _hud_manager_2 (`/Game/ProHUDV2/Blueprints/Libraries/BP_PHV2_Functions.GetHUDManager`))
  (`/Game/ProHUDV2/Blueprints/Libraries/BPi_HUDManagerV2.CreateHUD` _hud_manager 0)
  (`/Game/ProHUDV2/Blueprints/Libraries/BPi_HUDManagerV2.CreatePrimaryNotification` _hud_manager (make `/Game/ProHUDV2/Blueprints/Structs/S_PrimaryNotiInfo` "Mission Start" (make `/Game/ProHUDV2/Blueprints/Structs/S_TextInfo` true (make `SlateFontInfo` "/Game/ProHUDV2/DemoContent/Fonts/BarlowCondensed/F_Barlow_Condensed.F_Barlow_Condensed" null (struct :`OutlineColor` (struct :`A` 1.0)) "FF_BarlowCondensed-Regular" 30) 1.0 (struct :`R` 0.59375 :`G` 0.59375 :`B` 0.59375 :`A` 1.0)) "Complete mission and return" (make `/Game/ProHUDV2/Blueprints/Structs/S_TextInfo` true (make `SlateFontInfo` "/Game/ProHUDV2/DemoContent/Fonts/BarlowCondensed/F_Barlow_Condensed.F_Barlow_Condensed" null (struct :`OutlineColor` (struct :`A` 1.0)) "FF_BarlowCondensed-Regular" 30) 1.0 (struct :`R` 1.0 :`G` 1.0 :`B` 1.0 :`A` 1.0)) (struct :`Transform` (struct :`Translation` (0.0 0.0) :`Scale` (1.0 1.0) :`Shear` (0.0 0.0)) :`IconColor` (struct)) (struct :`R` 1.0 :`G` 1.0 :`B` 1.0 :`A` 0.7) 5.0))
  (`/Game/ProHUDV2/Blueprints/Libraries/BPi_HUDManagerV2.AddCrosshair` _hud_manager_2 "NewEnumerator0" (make `/Game/ProHUDV2/Blueprints/Structs/S_CrosshairInfo` (96.0 96.0) 12.0 (struct :`R` 1.0 :`G` 1.0 :`B` 1.0 :`A` 1.0) (1.0 1.0) 0.1))
  (`/Game/ProHUDV2/Blueprints/Libraries/BPi_HUDManagerV2.Show HP Bar` _hud_manager_2)
  (bind _returnvalue (`GameplayStatics.GetActorOfClass` "/Game/GProjectBP/Blueprints/Workers/MinimapCapture/BP_MinimapCaptureActor.BP_MinimapCaptureActor_C"))
  (`/Game/GProjectBP/Blueprints/Workers/MinimapCapture/BP_MinimapCaptureActor.Capture` _returnvalue)
  (`self.K2_DestroyActor` _returnvalue)
  (`/Game/ProHUDV2/Blueprints/Libraries/BPi_HUDManagerV2.ShowMinimap` _hud_manager_2 0)
  (goto _label :!via `Reset`))

(event `Mission Complete`
  (`/Engine/EditorBlueprintResources/StandardMacros.DoOnce` false :!label _label
    (:`Completed`
      (`/Game/ProHUDV2/Blueprints/Libraries/BPi_HUDManagerV2.CreatePrimaryNotification` (`/Game/ProHUDV2/Blueprints/Libraries/BP_PHV2_Functions.GetHUDManager`) (make `/Game/ProHUDV2/Blueprints/Structs/S_PrimaryNotiInfo` "Mission Complete" (make `/Game/ProHUDV2/Blueprints/Structs/S_TextInfo` true (make `SlateFontInfo` "/Game/ProHUDV2/DemoContent/Fonts/BarlowCondensed/F_Barlow_Condensed.F_Barlow_Condensed" null (struct :`OutlineColor` (struct :`A` 1.0)) "FF_BarlowCondensed-Regular" 30) 1.0 (struct :`R` 0.59375 :`G` 0.59375 :`B` 0.59375 :`A` 1.0)) "10 secs to evac" (make `/Game/ProHUDV2/Blueprints/Structs/S_TextInfo` true (make `SlateFontInfo` "/Game/ProHUDV2/DemoContent/Fonts/BarlowCondensed/F_Barlow_Condensed.F_Barlow_Condensed" null (struct :`OutlineColor` (struct :`A` 1.0)) "FF_BarlowCondensed-Regular" 30) 1.0 (struct :`R` 1.0 :`G` 1.0 :`B` 1.0 :`A` 1.0)) (struct :`Transform` (struct :`Translation` (0.0 0.0) :`Scale` (1.0 1.0) :`Shear` (0.0 0.0)) :`IconColor` (struct)) (struct :`R` 1.0 :`G` 1.0 :`B` 1.0 :`A` 0.7) 5.0))
      (`KismetSystemLibrary.K2_SetTimerDelegate` (delegate `Return to setup`) 10.0)
      (bind _returnvalue (`|CreateWidget` "/Game/GProjectBP/Blueprints/WidgetBP/HUD/WB_HUD_Countdown.WB_HUD_Countdown_C"))
      (`UserWidget.AddToViewport` _returnvalue 0))))

(event `Return to setup`
  (bind _asbp_game_instance (cast `/Game/GProjectBP/Blueprints/BP_GameInstance` (`GameplayStatics.GetGameInstance`) :!pure true))
  (bind _outactors (`GameplayStatics.GetAllActorsOfClass` "/Game/GProjectBP/Blueprints/BP_PlayerCharacter.BP_PlayerCharacter_C"))
  (for _array_element _outactors
    (`PrimitiveComponent.SetRenderCustomDepth` (`Character.Mesh` _array_element) false))
  (bind (_direction _alpha) (`Timeline|Timeline_0` :!via `PlayFromStart`)
    (:`Update`
      (`KismetMaterialLibrary.SetScalarParameterValue` "/Game/FXAssets/PixelSort/Youtube_Tutorial/PC_PixelData.PC_PixelData" "Alpha" _alpha))
    (:`Finished`
      ;[1 1 1] 멀티를 위해 개조 필요
      (`GPGameInstanceBase.SetSavingEnabled` _asbp_game_instance true)
      (bind _asbp_player_controller_game (cast `/Game/GProjectBP/Blueprints/BP_PlayerController_Game` (`GameplayStatics.GetPlayerController` 0)))
      (`self.Mission Reward Message`)
      (`self.SaveStages`)
      (`GProjectPlayerController.SaveInventory` _asbp_player_controller_game)
      (`GPGameInstanceBase.WriteSaveGame` _asbp_game_instance)
      (bind _returnvalue (`|CreateWidget` "/Game/GProjectBP/Blueprints/WidgetBP/WB_MIssionComplete.WB_MIssionComplete_C" _asbp_player_controller_game))
      (`UserWidget.AddToViewport` _returnvalue 0)
      (`WidgetBlueprintLibrary.SetInputMode_UIOnlyEx` _asbp_player_controller_game _returnvalue)
      (set `PlayerController.bShowMouseCursor` true _asbp_player_controller_game)
      (`GameplayStatics.SetGamePaused` true)
      (`GPGameInstanceBase.SetSavingEnabled` _asbp_game_instance false))))

(event `self.ReceiveBeginPlay`)

(fn `Mission Reward Message`
  (bind _stagelevel (break `GPStageInfo` (`.StageInfo` (break `GPStageNode` (`/Game/GProjectBP/Blueprints/BP_GameState_Base.CurrentStageNode` (`/Game/GProjectBP/Blueprints/BPFL_ABP.Get GP GS`))))))
  (bind _returnvalue (`GPGameInstanceBase.GetCurrentSaveGame` (`/Game/GProjectBP/Blueprints/BPFL_ABP.Get GP GI`)))
  (bind _output_get (set `GPSaveGame.SavedAttentionLevel` (+ (`GPSaveGame.SavedAttentionLevel` _returnvalue) (* _stagelevel (`KismetMathLibrary.RandomFloatInRange` 1.0 3.0))) _returnvalue))
  (bind _savedmessages (`GPSaveGame.SavedMessages` _returnvalue))
  (`KismetArrayLibrary.Array_Add` _savedmessages (make `GPMessageInfo` (`KismetArrayLibrary.Array_Length` _savedmessages) false "Captain" "Mission Reward" (`KismetTextLibrary.Conv_StringToText` (`KismetMathLibrary.SelectString` "Good Work, Heres' your cut." (`KismetStringLibrary.Concat_StrStr` "Good Work, Heres' your cut." " \n" "Enemies have put a bounty on you. Be careful.") (>= _output_get 5.0))) (`|MakeMap` "Token:Credit" (make `GPItemData` (* (+ _stagelevel 1) (`KismetMathLibrary.RandomIntegerInRange` 187 299))) :!type "PrimaryAssetId Structure")))
  (set `GPSaveGame.SavedMessages` _savedmessages _returnvalue))

(fn `SaveStages`
  (locals (bIsReachable :type Boolean) (NearestDis :type "Float (double-precision)" :default 999999.0) (NearestNode :type "GPStageNode Structure") (NearestIdx :type Integer))
  (bind _asbp_game_instance (`/Game/GProjectBP/Blueprints/BPFL_ABP.Get GP GI`))
  (bind _asbp_game_instance_2 (`/Game/GProjectBP/Blueprints/BPFL_ABP.Get GP GI`))
  (bind (_stageloc _stageinfo) (break `GPStageNode` (`local.NearestNode`)))
  (bind _stagenodes (`GPGameInstanceBase.StageNodes` _asbp_game_instance))
  (bind _currentstagenode (`GPGameInstanceBase.CurrentStageNode` _asbp_game_instance_2))
  (bind _currentstagenode_2 (`GPGameInstanceBase.CurrentStageNode` _asbp_game_instance))
  (bind _stagenodes_2 (`GPGameInstanceBase.StageNodes` _asbp_game_instance_2))
  (bind ((`StageLoc` _stageloc_2) (`StageInfo` _stageinfo_2)) (break `GPStageNode` _currentstagenode_2))
  (set `local.bIsReachable` false)
  ;[1 1 1] Connected Node Update
  (set `local.NearestDis` 999999.0)
  (for (_array_element _array_index) _stagenodes_2
    (if (!= _array_element _currentstagenode)
      (bind (_stageloc_3 _stageinfo_3 _stagestatus) (break `GPStageNode` _array_element))
      (bind _returnvalue (`KismetMathLibrary.Distance2D` _stageloc_3 (`.StageLoc` (break `GPStageNode` _currentstagenode))))
      (if (<= _returnvalue 400.0)
        (if (`|EnumInequality` _stagestatus "SS_Cleared")
          (`KismetArrayLibrary.Array_Set` _stagenodes_2 _array_index (make `GPStageNode` _stageloc_3 _stageinfo_3 "SS_Info"))
          (set `local.bIsReachable` true))
        (elif (and (< _returnvalue (`local.NearestDis`)) (`|EnumInequality` (`.StageStatus` (break `GPStageNode` _array_element)) "SS_Cleared"))
          (set `local.NearestDis` _returnvalue)
          (set `local.NearestNode` _array_element)
          (set `local.NearestIdx` _array_index)))))
  (if (not (`local.bIsReachable`))
    (`KismetArrayLibrary.Array_Set` (`GPGameInstanceBase.StageNodes` (`/Game/GProjectBP/Blueprints/BPFL_ABP.Get GP GI`)) (`local.NearestIdx`) (make `GPStageNode` _stageloc _stageinfo "SS_Info")))
  (`|VariableSetRef` (`|GetArrayItem` _stagenodes (`KismetArrayLibrary.Array_Find` _stagenodes _currentstagenode_2)) (make `GPStageNode` _stageloc_2 _stageinfo_2 "SS_Cleared"))
  (bind _returnvalue_2 (`GPGameInstanceBase.GetCurrentSaveGame` _asbp_game_instance))
  (set `GPSaveGame.SavedStageNodes` _stagenodes _returnvalue_2))

(fn `UserConstructionScript`)