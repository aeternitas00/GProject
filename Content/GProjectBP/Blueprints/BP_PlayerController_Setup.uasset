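; Player controller for a setup context that prepares the player character and restores its saved defaults and inventory on BeginPlay.
; After the parent logic, it hides the character's HP and Ammo components, shrinks the mesh and sets game-only input.
; It loads from the game instance's current save, or briefly enables saving to load or create one if none is valid.
; A debug print reports the saved attachment count.
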(event `self.ReceiveBeginPlay`
  (bind _asbp_game_instance (`/Game/GProjectBP/Blueprints/BPFL_ABP.Get GP GI`))
  (bind _asbp_game_instance_2 (`/Game/GProjectBP/Blueprints/BPFL_ABP.Get GP GI`))
  (bind _playercharacter (`self.PlayerCharacter`))
  (`parent.ReceiveBeginPlay`)
  (`SceneComponent.SetVisibility` (`/Game/GProjectBP/Blueprints/BP_CharacterBase.HP` _playercharacter) false false)
  (`SceneComponent.SetVisibility` (`/Game/GProjectBP/Blueprints/BP_CharacterBase.Ammo` _playercharacter) false false)
  (`SceneComponent.SetRelativeScale3D` (`Character.Mesh` _playercharacter) (0.85 0.85 0.85))
  (`WidgetBlueprintLibrary.SetInputMode_GameOnly` self)
  (bind _returnvalue (`GPGameInstanceBase.GetCurrentSaveGame` (`/Game/GProjectBP/Blueprints/BPFL_ABP.Get GP GI`)))
  (`/Engine/EditorBlueprintResources/StandardMacros.IsValid` _returnvalue
    (:`Is Valid`
      (`GPGameInstanceBase.LoadDefaults` (`/Game/GProjectBP/Blueprints/BPFL_ABP.Get GP GI`) _returnvalue)
      (`self.LoadInventory`)
      (`KismetSystemLibrary.PrintString` (`KismetStringLibrary.Conv_IntToString` (`BlueprintMapLibrary.Map_Length` (`GPSaveGame.AttachmentData` _returnvalue)))))
    (:`Is Not Valid`
      (`GPGameInstanceBase.SetSavingEnabled` _asbp_game_instance true)
      (`GPGameInstanceBase.LoadOrCreateSaveGame` _asbp_game_instance)
      (`GPGameInstanceBase.SetSavingEnabled` _asbp_game_instance_2 false)
      (bind _returnvalue_2 (`GPGameInstanceBase.GetCurrentSaveGame` _asbp_game_instance_2))
      (`GPGameInstanceBase.LoadDefaults` _asbp_game_instance_2 _returnvalue_2)
      (`self.LoadInventory`)
      (`KismetSystemLibrary.PrintString` (`KismetStringLibrary.Conv_IntToString` (`BlueprintMapLibrary.Map_Length` (`GPSaveGame.AttachmentData` _returnvalue_2)))))))

(fn `UserConstructionScript`)