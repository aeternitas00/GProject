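; AI character Blueprint for an armed combatant that spawns its weapon into a hand socket and drops pickups on death.
; An empty magazine fires an ammo delegate; reloading plays a montage, mirrored on clients via a remote-only event.
; UseCurrentWeapon passes the weapon montage's length to a delegate, failing without ammo or montage.
; Damage from a valid instigator is reported as a damage event while alive, and death flings DropItem pickups out with random impulses.
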(event `self.ReceiveBeginPlay`
  (bind _weaponclass (`self.WeaponClass`))
  (`parent.ReceiveBeginPlay`)
  (`BlueprintGameplayTagLibrary.AddGameplayTag` (`self.TraitsTag`))
  (if (`KismetSystemLibrary.IsValidClass` _weaponclass)
    (bind _returnvalue (`|SpawnActorFromClass` _weaponclass (`KismetMathLibrary.MakeTransform` (0.0 0.0 0.0)) "AlwaysSpawn" "OverrideRootScale" self self))
    (bind _output_get (set `self.CurrentWeaponActor` _returnvalue))
    (`self.K2_AttachToComponent` _output_get (`self.Mesh`) "hand_rSoc" "KeepRelative" "KeepRelative" "KeepRelative" true)
    (add `GPWeaponActorBase.OnCurrentMagChanged_D` _output_get (delegate `OnCurrentMagChanged_D_Event_0`))))

(event `OnCurrentMagChanged_D_Event_0`
  (params (DeltaValue :type "Float (double-precision)") (EventTags :type "GameplayTagContainer Structure (by ref)"))
  (if (== (`GPWeaponActorBase.GetCurrentMag` (`self.CurrentWeaponActor`)) 0.0)
    (`self.AmmoDelegate` true)))

(event `Reload Current Weapon`
  (bind _currentweaponactor (`self.CurrentWeaponActor`))
  ;[1 1 1] AI Reload
  (`/Engine/EditorBlueprintResources/StandardMacros.IsValid` _currentweaponactor
    (:`Is Valid`
      (if (== (`GPWeaponActorBase.GetCurrentMag` _currentweaponactor) 0.0)
        (`GPWeaponActorBase.OnWeaponReloadStart` (`self.CurrentWeaponActor`))
        (`self.Client Play Reload Montage`)
        (`|PlayMontage` (`self.Mesh`) "/Game/GProjectBP/Animation/Montage/AM_ReloadWeapon.AM_ReloadWeapon" (`GPWeaponActorBase.GetReloadSpeed` (`self.CurrentWeaponActor`))
          (:`then`
            (set `self.bIsReloading` true))
          (:`OnCompleted`
            (`self.AmmoDelegate` (== (`GPWeaponActorBase.GetCurrentMag` (`self.CurrentWeaponActor`)) 0.0) :!label _label)
            (set `self.bIsReloading` false))
          (:`OnInterrupted`
            (goto _label)))
        (else
          (`self.AmmoDelegate` false))))))

(event `self.OnDamaged`
  (params (DamageAmount :type "Float (single-precision)") (HitInfo :type "HitResult Structure (by ref)") (DamageTags :type "GameplayTagContainer Structure (by ref)") (InstigatorCharacter :type "GPCharacterBase Object Reference") (DamageCauser :type "Actor Object Reference"))
  (`/Engine/EditorBlueprintResources/StandardMacros.IsValid` InstigatorCharacter
    (:`Is Valid`
      (`parent.OnDamaged` DamageAmount HitInfo DamageTags InstigatorCharacter DamageCauser)
      (if (`self.IsAlive`)
        (`GPAISense_Damage.ReportGPDamageEvent` self InstigatorCharacter DamageAmount (`self.K2_GetActorLocation` InstigatorCharacter) (0.0 0.0 0.0) "Damage")))
    (:`Is Not Valid`
      (`KismetSystemLibrary.PrintString` (`KismetSystemLibrary.GetObjectName` DamageCauser)))))

(event `Client Play Reload Montage`
  (`/Engine/EditorBlueprintResources/ActorMacros.Switch Has Authority`
    (:`Remote`
      (`|PlayMontage` (`self.Mesh`) "/Game/GProjectBP/Animation/Montage/AM_ReloadWeapon.AM_ReloadWeapon"))))

(event `self.OnDeathEvent`
  (bind _dropitem (`self.DropItem`))
  (`parent.OnDeathEvent`)
  (bind _keys (`BlueprintMapLibrary.Map_Keys` _dropitem))
  (for _array_element _keys
    (bind _asgpitem (cast `GPItem` (`KismetSystemLibrary.GetObjectFromPrimaryAssetId` _array_element)))
    (bind _asbp_gppickup_item_base (castclass `/Game/GProjectBP/Blueprints/Objects/PickupItems/BP_GPPickupItemBase` (`GPItem.SpawningActor` _asgpitem)))
    (bind _returnvalue (`|SpawnActorFromClass` _asbp_gppickup_item_base (`self.GetTransform`) "Undefined" "OverrideRootScale" null (`.ItemCount` (break `GPItemData` (`BlueprintMapLibrary.Map_Find` _dropitem _array_element))) null))
    (`PrimitiveComponent.AddImpulse` (`/Game/GProjectBP/Blueprints/Objects/PickupItems/BP_GPPickupItemBase.ItemMesh` _returnvalue) (* (+ (`KismetMathLibrary.RandomUnitVector`) (0.0 0.0 1.2)) 200.0) "None" true)))

(fn `UseCurrentWeapon`
  (returns (Success :type Boolean))
  (bind _currentweaponactor (`self.CurrentWeaponActor`))
  (bind _weaponanimmontage (`GPWeaponActorBase.WeaponAnimMontage` _currentweaponactor))
  (`parent.UseCurrentWeapon`)
  (`/Engine/EditorBlueprintResources/StandardMacros.IsValid` _currentweaponactor
    (:`Is Valid`
      (if (not (== (`GPWeaponActorBase.GetCurrentMag` _currentweaponactor) 0.0))
        (`/Engine/EditorBlueprintResources/StandardMacros.IsValid` _weaponanimmontage
          (:`Is Valid`
            (bind _returnvalue (`AnimSequenceBase.GetPlayLength` _weaponanimmontage))
            (`self.MontageDelegate` _returnvalue)
            (return true))
          (:`Is Not Valid`
            _)))
      (return false))))

(fn `UserConstructionScript`)