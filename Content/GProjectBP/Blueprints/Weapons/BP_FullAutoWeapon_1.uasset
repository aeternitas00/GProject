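; Full-auto rifle weapon Blueprint that adds firing audio to its parent weapon class.
; On activation it calls the parent, then, if not already firing, attaches a one-shot or looping rifle cue to the mesh by fire mode and prints the fire rate.
; On deactivation, if the stored audio is valid, it issues a delayed stop, destroys the component immediately and clears the firing flag.
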(event `self.OnWeaponActivate`
  (`parent.OnWeaponActivate`)
  (if (not (`self.IsFiring`))
    (bind _returnvalue (`GameplayStatics.SpawnSoundAttached` (select `EWFiringMode` (`self.GetCurrentFiringMode`) :`WM_Single` "/Game/WeaponAssets/SciFiWeapDark/Sound/Rifle/RifleA_Fire_Cue.RifleA_Fire_Cue" :`WM_Burst` "/Game/WeaponAssets/SciFiWeapDark/Sound/Rifle/RifleA_Fire_Cue.RifleA_Fire_Cue" :`WM_Auto` "/Game/WeaponAssets/SciFiWeapDark/Sound/Rifle/RifleA_FireLoop_Cue.RifleA_FireLoop_Cue" :!type "SoundBase Object Reference") (`self.SkeletalMesh`) "None" (0.0 0.0 0.0) (struct) "KeepRelativeOffset" false 1.0 1.0 0.0 null null))
    (set `self.Attached Audio` _returnvalue)
    (set `self.IsFiring` true)
    (`KismetSystemLibrary.PrintString` (`KismetStringLibrary.Conv_DoubleToString` (`self.GetFireRate`)))))

(event `self.OnWeaponDeactivate`
  (bind _attached_audio (`self.Attached Audio`))
  (`/Engine/EditorBlueprintResources/StandardMacros.IsValid` _attached_audio
    (:`Is Valid`
      (`AudioComponent.StopDelayed` _attached_audio 0.05)
      (`ActorComponent.K2_DestroyComponent` _attached_audio)
      (set `self.IsFiring` false))))

(fn `UserConstructionScript`)