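; Base Blueprint for an invisible weapon actor that takes its muzzle transform from the "Muzzle" socket on the owning GPCharacterBase's mesh.
; Weapon activate, reload, raise and lower events each forward to a multicast event for animation or sound.
; Raise and lower cues play at the owner's location, skipped on dedicated servers.
; Fire and reload animation events are empty here, with no server check.
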(event `self.OnWeaponActivate`
  ;[1 1 1] Implementation
  (`self.Multicast Play Fire Anim`))

(event `self.OnWeaponReloadStart`
  ;[1 1 1] Implementation
  (`self.Multicast Play Reload Anim`))

(event `self.OnWeaponRaised`
  ;[1 1 1] Implementation
  (`self.Multicast Play Raise Sound`))

(event `self.OnWeaponLowered`
  ;[1 1 1] Implementation
  (`self.Multicast Play Lower Sound`))

(event `Multicast Play Fire Anim`
  ;[1 1 1] Server doesn't have to play anim but it may cause collision async, so we leave it multicast - no authority check ( have to study )
)

(event `Multicast Play Reload Anim`
  ;[1 1 1] Server doesn't have to play anim but it may cause collision async, so we leave it multicast - no authority check ( have to study )
)

(event `Multicast Play Lower Sound`
  ;[1 1 1] Server doesn't have to play sound
  (if (not (`KismetSystemLibrary.IsDedicatedServer`))
    (`GameplayStatics.PlaySoundAtLocation` (`self.LowerCue`) (`self.K2_GetActorLocation` (`self.GetOwner`)) (struct) 1.0 1.0 0.0 null null null)))

(event `Multicast Play Raise Sound`
  ;[1 1 1] Server doesn't have to play sound
  (if (not (`KismetSystemLibrary.IsDedicatedServer`))
    (`GameplayStatics.PlaySoundAtLocation` (`self.RaiseCue`) (`self.K2_GetActorLocation` (`self.GetOwner`)) (struct) 1.0 1.0 0.0 null null null)))

(fn `Get Muzzle Transform`
  (returns (Transform :type "Transform Structure"))
  (bind _asgpcharacter_base (cast `GPCharacterBase` (`self.GetOwner`)))
  (return (`SceneComponent.GetSocketTransform` (`Character.Mesh` _asgpcharacter_base) "Muzzle" "RTS_World")))

(fn `UserConstructionScript`)