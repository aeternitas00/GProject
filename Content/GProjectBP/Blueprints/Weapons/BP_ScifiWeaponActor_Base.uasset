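; Base sci-fi weapon actor that supplies the animation and sound feedback for firing, reloading, raising and lowering.
; Weapon events call multicast events that restart fire or reload animations on the skeletal mesh, with reload play rate driven by GetReloadSpeed.
; Raise and lower cues play at the owner's location except on dedicated servers, while animations run without that check.
; GetMuzzleTransform returns the Muzzle socket's world transform; an unconnected debug chain prints gameplay effect durations.
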(event `self.OnWeaponActivate`
  ;[1 1 1] Implementation
  (`self.Multicast Play Fire Anim`))

(event `self.OnWeaponReloadStart`
  ;[1 1 1] Implementation
  (`self.Multicast Play Reload Anim`))

(event `self.OnWeaponRaised`
  ;[1 1 1] Implementation
  (`self.Multicast Play Raise Sound`))

(event `self.OnWeaponLowered`
  ;[1 1 1] Implementation
  (`self.Multicast Play Lower Sound`))

(event `Multicast Play Fire Anim`
  (bind _skeletalmesh (`self.SkeletalMesh`))
  ;[1 1 1] Server doesn't have to play anim but it may cause collision async, so we leave it multicast - no authority check ( have to study )
  (`SkeletalMeshComponent.SetPosition` _skeletalmesh 0.0 false)
  (`SkeletalMeshComponent.PlayAnimation` _skeletalmesh (`self.FireAnim`) false)
  (`SkeletalMeshComponent.SetPlayRate` _skeletalmesh 1.0))

(event `Multicast Play Reload Anim`
  (bind _skeletalmesh (`self.SkeletalMesh`))
  ;[1 1 1] Server doesn't have to play anim but it may cause collision async, so we leave it multicast - no authority check ( have to study )
  (`SkeletalMeshComponent.SetPosition` _skeletalmesh 0.0 false)
  (`SkeletalMeshComponent.PlayAnimation` _skeletalmesh (`self.ReloadAnim`) false)
  (`SkeletalMeshComponent.SetPlayRate` _skeletalmesh (`self.GetReloadSpeed`)))

(event `Multicast Play Lower Sound`
  ;[1 1 1] Server doesn't have to play sound
  (if (not (`KismetSystemLibrary.IsDedicatedServer`))
    (`GameplayStatics.PlaySoundAtLocation` (`self.LowerCue`) (`self.K2_GetActorLocation` (`self.GetOwner`)) (struct) 1.0 1.0 0.0 null null null)))

(event `Multicast Play Raise Sound`
  ;[1 1 1] Server doesn't have to play sound
  (if (not (`KismetSystemLibrary.IsDedicatedServer`))
    (`GameplayStatics.PlaySoundAtLocation` (`self.RaiseCue`) (`self.K2_GetActorLocation` (`self.GetOwner`)) (struct) 1.0 1.0 0.0 null null null)))

(fn `Get Muzzle Transform`
  (returns (Transform :type "Transform Structure"))
  (return (`SceneComponent.GetSocketTransform` (`self.SkeletalMesh`) "Muzzle" "RTS_World")))

(fn `UserConstructionScript`)