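; BP_TitleMode is the title-screen mode Blueprint that brings up the main menu when play begins.
; On BeginPlay it calls CreateMainMenu, which creates the WB_ProMainMenu widget if the stored reference is invalid, adds it to the viewport and returns it.
; The main-menu player controller then updates its input mode to focus that widget and show the mouse cursor.
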(event `self.ReceiveBeginPlay`
  ;[0 0 0] Beginplay
  (bind _wb_promainmenu (`self.CreateMainMenu`))
  (`/Game/ProMainMenu/Blueprints/MainMenu/BP_PC_MainMenu.UpdateInputMode` (`/Game/ProMainMenu/Blueprints/Libraries/BP_MainMenu_Functions.Get_PC_MainMenu`) true _wb_promainmenu))

(fn `CreateMainMenu`
  (returns (WB_ProMainMenu :type "/Game/ProMainMenu/Widgets/WB_ProMainMenu Object Reference"))
  (`/Engine/EditorBlueprintResources/StandardMacros.IsValid` (`self.WB_ProMainMenu`)
    (:`Is Valid`
      _)
    (:`Is Not Valid`
      (bind _returnvalue (`|CreateWidget` "/Game/ProMainMenu/Widgets/WB_ProMainMenu.WB_ProMainMenu_C"))
      (bind _output_get (set `self.WB_ProMainMenu` _returnvalue))))
  (`UserWidget.AddToViewport` _output_get 0)
  (return (`self.WB_ProMainMenu`)))

(fn `UserConstructionScript`)