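; Blueprint function library of shared UI helpers for popups, item lists, icons and the message box.
; It spawns confirm popups bound to a Yes event, and fills a weapon's attachment list with data objects built from saved slot lookups.
; Other helpers find modifier icons in a data table, return per-type slot brushes, register items with list views and check the game instance for unread messages.
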(fn `Add Item Object to list view`
  (params (Target :type "ListView Object Reference") (Item :type "/Game/GProjectBP/Blueprints/WidgetBP/BP_List_ItemData Object Reference (by ref)"))
  (`ListView.AddItem` Target Item)
  (`KismetArrayLibrary.Array_AddUnique` (`/Game/GProjectBP/Blueprints/WidgetBP/BP_List_ItemData.ParentLists` Item) Target)
  (add `/Game/GProjectBP/Blueprints/WidgetBP/BP_List_ItemData.UpdateAmount` Item (`|CreateDelegate` Item :!event `Listview Amount update`)))

(fn `Create Confirm Widget`
  (params (OwningPlayer :type "PlayerController Object Reference") (Outer :type "/Game/GProjectBP/Blueprints/WidgetBP/Objects/Arsenal/WB_Arsenal_Main Object Reference") (HeaderTextValue :type Text) (ContentTextValue :type Text) (Event :type "Delegate (by ref)"))
  (bind _returnvalue (`|CreateWidget` "/Game/GProjectBP/Blueprints/WidgetBP/Objects/Arsenal/WB_Confirm_Popup.WB_Confirm_Popup_C" OwningPlayer Outer HeaderTextValue ContentTextValue))
  (`UserWidget.AddToViewport` _returnvalue 0)
  (`/Game/GProjectBP/Blueprints/WidgetBP/Objects/Arsenal/WB_Confirm_Popup.Bind Event to Yes Bttn` _returnvalue Event))

(fn `Create Weapon Attachment Slots`
  (params (Weapon :type "GPItemWeapon Object Reference (by ref)") (AttachmentListView :type "ListView Object Reference") (Outer :type "Object Object Reference"))
  (locals (Slot :type "GPItemSlot Structure") (IsEquiped :type Boolean :default false) (Loop_Type :type "EWAttachmentType Enum") (SaveOuter :type "Object Object Reference"))
  (bind _loop_type (`local.Loop_Type`))
  (bind _saveouter (`local.SaveOuter`))
  (bind _asgpitem_attachment (cast `GPItemAttachment` (`KismetSystemLibrary.GetObjectFromPrimaryAssetId` (`BlueprintMapLibrary.Map_Find` (`.Attached` (break `GPWAttachmentedData` (`BlueprintMapLibrary.Map_Find` (`GPGameInstanceBase.AttachedItems` (`/Game/GProjectBP/Blueprints/BPFL_ABP.Get GP GI` null)) (`local.Slot`)))) (`local.Loop_Type`))) :!pure true))
  (set `local.SaveOuter` Outer)
  (`ListView.ClearListItems` AttachmentListView)
  (bind (_exist _slot) (`/Game/GProjectBP/Blueprints/BPFL_ABP.Check Saved Slotted Item` Weapon))
  (if _exist
    (set `local.IsEquiped` true))
  (set `local.Slot` _slot)
  (for _array_element (defaults `Object` (`GPItemWeapon.WeaponActor` Weapon))
    (set `local.Loop_Type` _array_element)
    (if (`local.IsEquiped`)
      (bind _returnvalue (`|GenericCreateObject` _saveouter "/Game/GProjectBP/Blueprints/WidgetBP/Inventory/BP_List_AttachmentData.BP_List_AttachmentData_C" _asgpitem_attachment _loop_type))
      (`ListView.AddItem` AttachmentListView _returnvalue)
      (else
        (bind _returnvalue_2 (`|GenericCreateObject` _saveouter "/Game/GProjectBP/Blueprints/WidgetBP/Inventory/BP_List_AttachmentData.BP_List_AttachmentData_C" _asgpitem_attachment _loop_type))
        (`ListView.AddItem` AttachmentListView _returnvalue_2)))))

(fn `Get Attachment Slot Icon`
  (params (Type :type "EWAttachmentType Enum" :default "WA_Magazine"))
  (returns (Brush :type "SlateBrush Structure"))
  (locals (inType :type "EWAttachmentType Enum" :default "WA_Magazine") (RetVal :type "SlateBrush Structure"))
  (bind _slatecolor (make `SlateColor` (struct :`R` 0.229167 :`G` 0.229167 :`B` 0.229167 :`A` 1.0)))
  (bind _output_get (set `local.inType` Type))
  (switch `EWAttachmentType` _output_get
    (:`WA_Magazine`
      (set `local.RetVal` (make `SlateBrush` "Image" "NoTile" "NoMirror" (struct :`X` 70.0 :`Y` 70.0) (struct) _slatecolor (struct :`CornerRadii` (struct :`W` 1.0) :`Color` (struct :`SpecifiedColor` (struct) :`ColorUseRule` "UseColor_Specified") :`RoundingType` "HalfHeightRadius") "/Game/GProjectBP/UIResource/MagSlot.MagSlot")))
    (:`WA_Barrel`
      (set `local.RetVal` (make `SlateBrush` "Image" "NoTile" "NoMirror" (struct :`X` 70.0 :`Y` 70.0) (struct) _slatecolor (struct :`CornerRadii` (struct :`W` 1.0) :`Color` (struct :`SpecifiedColor` (struct) :`ColorUseRule` "UseColor_Specified") :`RoundingType` "HalfHeightRadius") "/Game/GProjectBP/UIResource/BarrelSlot.BarrelSlot")))
    (:`WA_Stock`
      (set `local.RetVal` (make `SlateBrush` "Image" "NoTile" "NoMirror" (struct :`X` 70.0 :`Y` 70.0) (struct) _slatecolor (struct :`CornerRadii` (struct :`W` 1.0) :`Color` (struct :`SpecifiedColor` (struct) :`ColorUseRule` "UseColor_Specified") :`RoundingType` "HalfHeightRadius") "/Game/GProjectBP/UIResource/StockSlot.StockSlot")))
    (:`WA_Optic`
      (set `local.RetVal` (make `SlateBrush` "Image" "NoTile" "NoMirror" (struct :`X` 70.0 :`Y` 70.0) (struct) _slatecolor (struct :`CornerRadii` (struct :`W` 1.0) :`Color` (struct :`SpecifiedColor` (struct) :`ColorUseRule` "UseColor_Specified") :`RoundingType` "HalfHeightRadius") "/Game/GProjectBP/UIResource/OpticsSlot.OpticsSlot"))))
  (return (`local.RetVal`)))

(fn `Get Modifier Icon`
  (params (Attribute :type "GameplayAttribute Structure"))
  (returns (Brush :type "SlateBrush Structure"))
  (locals (InAtt :type "GameplayAttribute Structure"))
  (set `local.InAtt` Attribute)
  (bind _outrownames (`DataTableFunctionLibrary.GetDataTableRowNames` "/Game/GProjectBP/DataAsset/AttributeIconTable.AttributeIconTable"))
  (for _array_element _outrownames
    (bind _returnvalue (`|GetDataTableRow` "/Game/GProjectBP/DataAsset/AttributeIconTable.AttributeIconTable" _array_element)
      (:`then`
        (bind (_modattribute _icon) (break `/Game/GProjectBP/DataAsset/AttributeIconSet` _returnvalue))
        (if (== (`local.InAtt`) _modattribute)
          (return _icon))))))

(fn `Is New Message in Box`
  (returns (bExist :type Boolean))
  (for _array_element (`GPGameInstanceBase.Messages` (`/Game/GProjectBP/Blueprints/BPFL_ABP.Get GP GI` null))
    (if (== (`.bIsRead` (break `GPMessageInfo` _array_element)) false)
      (return true)))
  (return false))