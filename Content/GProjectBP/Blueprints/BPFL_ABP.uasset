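; Blueprint function library of shared helpers for weapon animation selection, game instance access, saved item slot lookup and float rounding.
; Weapon flag functions match a weapon actor's or class's type against two-handed, then one-handed lists, returning a default flag when invalid or unmatched.
; The slot check scans the game instance's DefaultSlottedItems map for an item's primary asset ID, returning whether it exists and in which slot.
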(fn `Check Saved Slotted Item`
  (params (`Item Data asset` :type "Object Object Reference (by ref)"))
  (returns (Exist :type Boolean) (Slot :type "GPItemSlot Structure"))
  (bind _defaultslotteditems (`GPGameInstanceBase.DefaultSlottedItems` (`self.Get GP GI` null)))
  (bind _keys (`BlueprintMapLibrary.Map_Keys` _defaultslotteditems))
  (for _array_element _keys
    (if (== (`BlueprintMapLibrary.Map_Find` _defaultslotteditems _array_element) (`KismetSystemLibrary.GetPrimaryAssetIdFromObject` `Item Data asset`))
      (return true _array_element)))
  (return false))

(fn `Get GP GI`
  (returns (`AsBP Game Instance` :type "/Game/GProjectBP/Blueprints/BP_GameInstance Object Reference"))
  (return (cast `/Game/GProjectBP/Blueprints/BP_GameInstance` (`GameplayStatics.GetGameInstance` null) :!pure true)))

(fn `Get Preper Weapon Anim Flag`
  (params (WeaponActor :type "GPWeaponActorBase Object Reference"))
  (returns (Flag :type "/Game/CharactersAssets/MOCAPAnimationPacks/Mobility/ControllerMain/Blueprints/WeaponState Enum"))
  (locals (TwoHandedWeapons :type "Array of EWeaponType Enum") (OneHandedWeapons :type "Array of EWeaponType Enum"))
  (bind _weapontype (`GPWeaponActorBase.WeaponType` WeaponActor))
  (`/Engine/EditorBlueprintResources/StandardMacros.IsValid` WeaponActor
    (:`Is Valid`
      (for _array_element (`local.TwoHandedWeapons`)
        (if (`KismetArrayLibrary.Array_Contains` _weapontype _array_element)
          (return "NewEnumerator2")))
      (for _array_element_2 (`local.OneHandedWeapons`)
        (if (`KismetArrayLibrary.Array_Contains` _weapontype _array_element_2)
          (return "NewEnumerator1")))
      (return "NewEnumerator0"))
    (:`Is Not Valid`
      (return "NewEnumerator0"))))

(fn `Get Preper Weapon Anim Flag By Class`
  (params (WeaponActor :type "GPWeaponActorBase Class Reference"))
  (returns (Flag :type "/Game/CharactersAssets/MOCAPAnimationPacks/Mobility/ControllerMain/Blueprints/WeaponState Enum"))
  (locals (TwoHandedWeapons :type "Array of EWeaponType Enum") (OneHandedWeapons :type "Array of EWeaponType Enum"))
  (bind _weapontype (defaults `Object` WeaponActor))
  (if (`KismetSystemLibrary.IsValidClass` WeaponActor)
    (for _array_element (`local.TwoHandedWeapons`)
      (if (`KismetArrayLibrary.Array_Contains` _weapontype _array_element)
        (return "NewEnumerator2")))
    (for _array_element_2 (`local.OneHandedWeapons`)
      (if (`KismetArrayLibrary.Array_Contains` _weapontype _array_element_2)
        (return "NewEnumerator1")))
    (return "NewEnumerator0")
    (else
      (return "NewEnumerator0"))))

(fn `RoundUpToNDemical`
  (params (N :type Integer) (Float :type "Float (double-precision)"))
  (returns (ReturnValue :type "Float (double-precision)"))
  (bind _returnvalue (`KismetMathLibrary.MultiplyMultiply_FloatFloat` 10.0 (`KismetMathLibrary.Conv_IntToDouble` N)))
  (return (/ (`KismetMathLibrary.Conv_IntToDouble` (`KismetMathLibrary.Round` (* _returnvalue Float))) _returnvalue)))