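; BP_TutInteractionObj is a tutorial interactable that appears to be a laptop, bobbing its mesh on a sine wave each Tick.
; While Active, Interact toggles the screen material between mail and off, and its first use completes the task and posts a HUD notification.
; Show and hide interact events toggle the pickup widget border and a custom-depth stencil highlight on the mesh.
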(event `self.ReceiveBeginPlay`
  (set `self.Default` (`SceneComponent.K2_GetComponentLocation` (`self.ItemMesh`))))

(event `self.ReceiveTick`
  (params (DeltaSeconds :type "Float (single-precision)"))
  (`SceneComponent.K2_SetRelativeLocation` (`self.ItemMesh`) (`KismetMathLibrary.MakeVector` 0.0 0.0 (* (`KismetMathLibrary.Sin` (`self.Time`)) 15.0)) false false)
  (bind _output_get (set `self.Time` (+ (`self.Time`) (* DeltaSeconds 2.5))))
  (if (>= _output_get (`KismetMathLibrary.MultiplyByPi` 2.0))
    (set `self.Time` 0.0)))

(event `GPInteractionInterface.Interact`
  (params (InstigatorPawn :type "Pawn Object Reference"))
  (bind _itemmesh (`self.ItemMesh`))
  (if (`self.Active`)
    (`|ExecutionSequence`
      (:`then_0`
        (`/Engine/EditorBlueprintResources/StandardMacros.FlipFlop`
          (:`A`
            (`PrimitiveComponent.SetMaterial` _itemmesh 3 "/Game/Geometry/ModularSFPack2/ModularScifiProps/Materials/MI_Laptop_Mail.MI_Laptop_Mail"))
          (:`B`
            (`PrimitiveComponent.SetMaterial` _itemmesh 3 "/Game/Geometry/ModularSFPack2/ModularScifiProps/Materials/MI_Screen_Lapt_Off.MI_Screen_Lapt_Off"))))
      (:`then_1`
        (`/Engine/EditorBlueprintResources/StandardMacros.DoOnce` false
          (:`Completed`
            (`self.Task Complete`)
            (`/Game/ProHUDV2/Blueprints/Libraries/BPi_HUDManagerV2.CreateUpdateNotification` (`/Game/ProHUDV2/Blueprints/Libraries/BP_PHV2_Functions.GetHUDManager`) (`self.NotInfo`))))))))

(event `GPInteractionInterface.ShowInteractUI`
  (params (InstigatorPawn :type "Pawn Object Reference"))
  (if (`self.Active`)
    (if (not (`self.bIsWidgetVisible`))
      (bind _aswb_hud_pickup_item (cast `/Game/GProjectBP/Blueprints/WidgetBP/HUD/WB_HUD_PickupItem` (`WidgetComponent.GetUserWidgetObject` (`self.Widget`))))
      (`Widget.SetVisibility` (`/Game/GProjectBP/Blueprints/WidgetBP/HUD/WB_HUD_PickupItem.PickupBorder` _aswb_hud_pickup_item) "Visible")
      (set `self.bIsWidgetVisible` true)
      (`TextBlock.SetText` (`/Game/GProjectBP/Blueprints/WidgetBP/HUD/WB_HUD_PickupItem.ItemTextBlock` _aswb_hud_pickup_item) "")
      (`PrimitiveComponent.SetCustomDepthStencilValue` (`self.ItemMesh`) 252)
      (`PrimitiveComponent.SetRenderCustomDepth` (`self.ItemMesh`) true))))

(event `GPInteractionInterface.HideInteractUI`
  (params (InstigatorPawn :type "Pawn Object Reference"))
  (if (`self.Active`)
    (if (`self.bIsWidgetVisible`)
      (bind _aswb_hud_pickup_item (cast `/Game/GProjectBP/Blueprints/WidgetBP/HUD/WB_HUD_PickupItem` (`WidgetComponent.GetUserWidgetObject` (`self.Widget`))))
      (`Widget.SetVisibility` (`/Game/GProjectBP/Blueprints/WidgetBP/HUD/WB_HUD_PickupItem.PickupBorder` _aswb_hud_pickup_item) "Hidden")
      (set `self.bIsWidgetVisible` false)
      (`PrimitiveComponent.SetRenderCustomDepth` (`self.ItemMesh`) false))))

(fn `GetInteractText`
  (params (InstigatorPawn :type "Pawn Object Reference"))
  (returns (ReturnValue :type Text))
  (return ""))

(fn `UserConstructionScript`)