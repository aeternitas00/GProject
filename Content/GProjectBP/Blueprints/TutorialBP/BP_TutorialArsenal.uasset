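; BP_TutorialArsenal is an interactable tutorial terminal that opens the arsenal screen and completes a tutorial task.
; Interacting toggles the WB_Tut_Arsenal widget, cursor, input mode and player idle-turn lock; hiding the interact prompt also closes it.
; Two opposing timelines drive CamMovement, adjusting the player's spring-arm length and offset on open and close.
; Completion calls the parent task logic and swaps direction-marker visibility, while InitTaskInfo gathers next-task indices.
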(event `self.Init task info`
  (for _array_element (`self.NextObjects`)
    (`BlueprintSetLibrary.Set_Add` (`self.NextTaskIdx(Autoset)`) (`/Game/GProjectBP/Blueprints/Objects/BP_TaskObject.TaskIdx(Autoset)` _array_element))))

(event `self.ReceiveBeginPlay`
  (bind _aswb_hud_interaction_base (cast `/Game/GProjectBP/Blueprints/WidgetBP/Objects/WB_HUD_InteractionBase` (`WidgetComponent.GetWidget` (`self.Text`))))
  (`/Game/GProjectBP/Blueprints/WidgetBP/Objects/WB_HUD_InteractionBase.Set Action Name` _aswb_hud_interaction_base "Open arsenal"))

(event `Activate`
  (params (Pawn :type "Pawn Object Reference"))
  (bind _asbp_player_character (cast `/Game/GProjectBP/Blueprints/BP_PlayerCharacter` Pawn :!pure true))
  (bind _springarm (`/Game/GProjectBP/Blueprints/BP_PlayerCharacter.SpringArm` _asbp_player_character))
  (bind _asplayer_controller (cast `PlayerController` (`Pawn.GetController` _asbp_player_character) :!pure true))
  (set `self.bUsing` true)
  (set `/Game/GProjectBP/Blueprints/BP_PlayerCharacter.bIdleTurnLock` true _asbp_player_character)
  (set `self.Spring Arm` _springarm)
  (set `self.Relative Location` (`SceneComponent.RelativeLocation` _springarm))
  (set `PlayerController.bShowMouseCursor` true _asplayer_controller)
  (bind _returnvalue (`|CreateWidget` "/Game/GProjectBP/Blueprints/TutorialBP/WB_Tut_Arsenal.WB_Tut_Arsenal_C" _asplayer_controller))
  (`UserWidget.AddToViewport` _returnvalue 0)
  (bind _output_get (set `self.ArsenalWidget` _returnvalue))
  (set `/Game/GProjectBP/Blueprints/TutorialBP/WB_Tut_Arsenal.Obj` self _output_get)
  (`WidgetBlueprintLibrary.SetInputMode_GameAndUIEx` _asplayer_controller _output_get "DoNotLock" false)
  (`self.Task Complete`)
  (`|ExecutionSequence`
    (:`then_0`
      (bind (_direction _camdist _camoffset) (`Timeline|Timeline_0` :!via `PlayFromStart` :!label _label)
        (:`Update`
          (`self.CamMovement` _camdist _camoffset))))
    (:`then_1`
      (bind (_direction_2 _camdist_2 _camoffset_2) (`Timeline|Timeline_1` :!via `Stop` :!label _label_2)
        (:`Update`
          (`self.CamMovement` _camdist_2 _camoffset_2))))))

(event `Deactivate`
  (params (Object :type "Pawn Object Reference"))
  (bind _asplayer_controller (cast `PlayerController` (`Pawn.GetController` Object) :!pure true))
  (set `self.bUsing` false)
  (set `/Game/GProjectBP/Blueprints/BP_PlayerCharacter.bIdleTurnLock` false (cast `/Game/GProjectBP/Blueprints/BP_PlayerCharacter` Object :!pure true))
  (`/Game/ProHUDV2/Blueprints/Libraries/BPi_HUDManagerV2.RemoveCrosshair` (`/Game/ProHUDV2/Blueprints/Libraries/BP_PHV2_Functions.GetHUDManager`))
  (`WidgetBlueprintLibrary.SetInputMode_GameOnly` _asplayer_controller)
  (`/Game/GProjectBP/Blueprints/TutorialBP/WB_Tut_Arsenal.Remove Widget` (`self.ArsenalWidget`))
  (set `PlayerController.bShowMouseCursor` false _asplayer_controller)
  (`|ExecutionSequence`
    (:`then_0`
      (goto _label_2 :!via `PlayFromStart`))
    (:`then_1`
      (goto _label :!via `Stop`))))

(event `self.Task Complete`
  (`parent.Task Complete`)
  (for _array_element (`self.HideDirectioner`)
    (`self.SetActorHiddenInGame` _array_element true))
  (for _array_element_2 (`self.ShowDirectioner`)
    (`self.SetActorHiddenInGame` _array_element_2 false)))

(event `GPInteractionInterface.Interact`
  (params (InstigatorPawn :type "Pawn Object Reference"))
  (if (`self.bUsing`)
    (`self.Deactivate` InstigatorPawn)
    (`SceneComponent.SetVisibility` (`self.Text`) true true)
    (else
      (`self.Activate` InstigatorPawn)
      (`SceneComponent.SetVisibility` (`self.Text`) false true))))

(event `GPInteractionInterface.ShowInteractUI`
  (params (InstigatorPawn :type "Pawn Object Reference"))
  (`SceneComponent.SetVisibility` (`self.Text`) true true))

(event `GPInteractionInterface.HideInteractUI`
  (params (InstigatorPawn :type "Pawn Object Reference"))
  (if (`self.bUsing`)
    (`self.Deactivate` InstigatorPawn))
  (`SceneComponent.SetVisibility` (`self.Text`) false true))

(fn `GetInteractText`
  (params (InstigatorPawn :type "Pawn Object Reference"))
  (returns (ReturnValue :type Text))
  (return "Terminal"))

(fn `UserConstructionScript`)