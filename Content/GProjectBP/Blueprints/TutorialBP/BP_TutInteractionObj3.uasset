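; Tutorial interactable with a hinged Glass component that highlights through custom depth while the interact UI shows.
; When active, the first interaction completes the tutorial task and posts a HUD notification.
; Each interaction, unless locked, toggles the glass open or closed by playing or reversing a timeline that lerps its yaw, with collision disabled during the swing.
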(event `GPInteractionInterface.ShowInteractUI`
  (params (InstigatorPawn :type "Pawn Object Reference"))
  (if (`self.Active`)
    (`PrimitiveComponent.SetCustomDepthStencilValue` (`self.Glass`) 252)
    (`PrimitiveComponent.SetRenderCustomDepth` (`self.Glass`) true)))

(event `GPInteractionInterface.HideInteractUI`
  (params (InstigatorPawn :type "Pawn Object Reference"))
  (if (`self.Active`)
    (`PrimitiveComponent.SetRenderCustomDepth` (`self.Glass`) false)))

(event `GPInteractionInterface.Interact`
  (params (InstigatorPawn :type "Pawn Object Reference"))
  (bind _isopened (`self.IsOpened`))
  (bind _returnvalue (not _isopened))
  (if (`self.Active`)
    (`|ExecutionSequence`
      (:`then_0`
        (`/Engine/EditorBlueprintResources/StandardMacros.DoOnce` false
          (:`Completed`
            (`self.Task Complete`)
            (`/Game/ProHUDV2/Blueprints/Libraries/BPi_HUDManagerV2.CreateUpdateNotification` (`/Game/ProHUDV2/Blueprints/Libraries/BP_PHV2_Functions.GetHUDManager`) (`self.NotInfo`)))))
      (:`then_1`
        (if (`self.IsLocked`)
          _
          (elif _isopened
            (set `self.IsOpened` _returnvalue)
            (`PrimitiveComponent.SetCollisionEnabled` (`self.Glass`) "NoCollision")
            (bind (_direction _offset) (`Timeline|ToggleGlass` :!via `Reverse` :!label _label)
              (:`Update`
                (`SceneComponent.K2_SetRelativeRotation` (`self.Glass`) (`KismetMathLibrary.MakeRotator` (.x (`KismetMathLibrary.VLerp` (0.0 0.0 0.0) (0.0 0.0 120.0) _offset)) (.y (`KismetMathLibrary.VLerp` (0.0 0.0 0.0) (0.0 0.0 120.0) _offset)) (.z (`KismetMathLibrary.VLerp` (0.0 0.0 0.0) (0.0 0.0 120.0) _offset))) false false))
              (:`Finished`
                (`PrimitiveComponent.SetCollisionEnabled` (`self.Glass`) "QueryAndPhysics")))
            (else
              (set `self.IsOpened` _returnvalue)
              (`PrimitiveComponent.SetCollisionEnabled` (`self.Glass`) "NoCollision")
              (goto _label))))))))

(fn `GetInteractText`
  (params (InstigatorPawn :type "Pawn Object Reference"))
  (returns (ReturnValue :type Text))
  (return ""))

(fn `UserConstructionScript`)