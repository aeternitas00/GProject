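; Interactable tutorial terminal that toggles a world-space mission-select widget when the player interacts with it.
; Activation locks idle turning, shows a crosshair and plays a timeline that moves the player's spring arm while scaling the widget.
; Mouse axes slide the widget component, so it moves relative to the crosshair.
; Deactivating or hiding the interact UI while in use plays a separate Backward timeline, then destroys the widget.
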(event `InputAxis|MouseX` :consume false
  (params (AxisValue :type "Float (single-precision)"))
  (bind _addedcomponent (`self.AddedComponent`))
  (`/Engine/EditorBlueprintResources/StandardMacros.IsValid` _addedcomponent
    (:`Is Valid`
      (`SceneComponent.K2_AddLocalOffset` _addedcomponent (`KismetMathLibrary.MakeVector` 0.0 (* AxisValue -16.0)) false false))))

(event `self.ReceiveBeginPlay`
  (bind _aswb_hud_interaction_base (cast `/Game/GProjectBP/Blueprints/WidgetBP/Objects/WB_HUD_InteractionBase` (`WidgetComponent.GetWidget` (`self.Text`))))
  (`/Game/GProjectBP/Blueprints/WidgetBP/Objects/WB_HUD_InteractionBase.Set Action Name` _aswb_hud_interaction_base "Replicate"))

(event `InputAxis|MouseY` :consume false
  (params (AxisValue :type "Float (single-precision)"))
  (bind _addedcomponent (`self.AddedComponent`))
  (`/Engine/EditorBlueprintResources/StandardMacros.IsValid` _addedcomponent
    (:`Is Valid`
      (`SceneComponent.K2_AddLocalOffset` _addedcomponent (`KismetMathLibrary.MakeVector` 0.0 0.0 (* AxisValue -8.0)) false false))))

(event `Activate`
  (params (Pawn :type "Pawn Object Reference"))
  (bind _asbp_player_character (cast `/Game/GProjectBP/Blueprints/BP_PlayerCharacter` Pawn :!pure true))
  (bind _springarm (`/Game/GProjectBP/Blueprints/BP_PlayerCharacter.SpringArm` _asbp_player_character))
  (set `self.bUsing` true)
  (set `/Game/GProjectBP/Blueprints/BP_PlayerCharacter.bIdleTurnLock` true _asbp_player_character)
  (set `self.Spring Arm` _springarm)
  (`/Game/ProHUDV2/Blueprints/Libraries/BPi_HUDManagerV2.AddCrosshair` (`/Game/ProHUDV2/Blueprints/Libraries/BP_PHV2_Functions.GetHUDManager`) "NewEnumerator1" (make `/Game/ProHUDV2/Blueprints/Structs/S_CrosshairInfo` (96.0 96.0) 12.0 (struct :`R` 1.0 :`G` 1.0 :`B` 1.0 :`A` 1.0)))
  (set `self.Relative Location` (`SceneComponent.RelativeLocation` _springarm))
  (`/Engine/EditorBlueprintResources/StandardMacros.IsValid` (`self.AddedComponent`)
    (:`Is Valid`
      (`self.ClearWidgetComp`))
    (:`Is Not Valid`
      _))
  (bind _returnvalue (`AddComponent|NODE_AddWidgetComponent-0` :`self` self))
  (bind _output_get (set `self.AddedComponent` _returnvalue))
  (set `/Game/GProjectBP/Blueprints/TutorialBP/WB_Tut_MissionSelect.Obj` self (cast `/Game/GProjectBP/Blueprints/TutorialBP/WB_Tut_MissionSelect` (`WidgetComponent.GetWidget` _output_get) :!pure true))
  (`|ExecutionSequence`
    (:`then_0`
      (bind (_direction _camdist _camoffset _widgetsize) (`Timeline|Forward` :!via `PlayFromStart` :!label _label)
        (:`Update`
          (`self.Update` _camdist _camoffset _widgetsize (`self.AddedComponent`)))))
    (:`then_1`
      (bind (_direction_2 _camdist_2 _camoffset_2 _widgetsize_2) (`Timeline|Backward` :!via `Stop` :!label _label_2)
        (:`Update`
          (`self.Update` _camdist_2 _camoffset_2 _widgetsize_2 (`self.AddedComponent`)))
        (:`Finished`
          (`self.ClearWidgetComp`))))))

(event `Deactivate`
  (params (Object :type "Pawn Object Reference"))
  (set `self.bUsing` false)
  (set `/Game/GProjectBP/Blueprints/BP_PlayerCharacter.bIdleTurnLock` false (cast `/Game/GProjectBP/Blueprints/BP_PlayerCharacter` Object :!pure true))
  (`/Game/ProHUDV2/Blueprints/Libraries/BPi_HUDManagerV2.RemoveCrosshair` (`/Game/ProHUDV2/Blueprints/Libraries/BP_PHV2_Functions.GetHUDManager`))
  (`|ExecutionSequence`
    (:`then_0`
      (goto _label_2 :!via `PlayFromStart`))
    (:`then_1`
      (goto _label :!via `Stop`))))

(event `GPInteractionInterface.Interact`
  (params (InstigatorPawn :type "Pawn Object Reference"))
  (if (`self.bUsing`)
    (`self.Deactivate` InstigatorPawn)
    (`SceneComponent.SetVisibility` (`self.Text`) true true)
    (else
      (`self.Activate` InstigatorPawn)
      (`SceneComponent.SetVisibility` (`self.Text`) false true))))

(event `GPInteractionInterface.ShowInteractUI`
  (params (InstigatorPawn :type "Pawn Object Reference"))
  (`SceneComponent.SetVisibility` (`self.Text`) true true))

(event `GPInteractionInterface.HideInteractUI`
  (params (InstigatorPawn :type "Pawn Object Reference"))
  (if (`self.bUsing`)
    (`self.Deactivate` InstigatorPawn))
  (`SceneComponent.SetVisibility` (`self.Text`) false true))

(fn `GetInteractText`
  (params (InstigatorPawn :type "Pawn Object Reference"))
  (returns (ReturnValue :type Text))
  (return "Terminal"))

(fn `UserConstructionScript`)