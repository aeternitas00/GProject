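; Tutorial pickup item that, on interaction, gives the player a test weapon and ammo.
; Tick bobs the mesh on a sine wave, and the interact UI events toggle a custom depth stencil highlight while the item is active.
; Interact posts a HUD notification, then once completes the task, adds items through the player controller, adds a crosshair, and hides and deactivates the actor.
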(event `self.ReceiveBeginPlay`
  (set `self.Default` (`SceneComponent.K2_GetComponentLocation` (`self.ItemMesh`))))

(event `self.ReceiveTick`
  (params (DeltaSeconds :type "Float (single-precision)"))
  (`SceneComponent.K2_SetRelativeLocation` (`self.ItemMesh`) (`KismetMathLibrary.MakeVector` 0.0 0.0 (* (`KismetMathLibrary.Sin` (`self.Time`)) 15.0)) false false)
  (bind _output_get (set `self.Time` (+ (`self.Time`) (* DeltaSeconds 2.5))))
  (if (>= _output_get (`KismetMathLibrary.MultiplyByPi` 2.0))
    (set `self.Time` 0.0)))

(event `GPInteractionInterface.Interact`
  (params (InstigatorPawn :type "Pawn Object Reference"))
  (if (`self.Active`)
    (`/Game/ProHUDV2/Blueprints/Libraries/BPi_HUDManagerV2.CreateUpdateNotification` (`/Game/ProHUDV2/Blueprints/Libraries/BP_PHV2_Functions.GetHUDManager`) (`self.NotInfo`))
    (`/Engine/EditorBlueprintResources/StandardMacros.DoOnce` false
      (:`Completed`
        (`self.Task Complete`)
        (bind _asbp_player_character (cast `/Game/GProjectBP/Blueprints/BP_PlayerCharacter` InstigatorPawn))
        (`self.GiveItem` _asbp_player_character)
        (`/Game/ProHUDV2/Blueprints/Libraries/BPi_HUDManagerV2.V1_AddCrosshair` (`/Game/ProHUDV2/Blueprints/Libraries/BP_PHV2_Functions.GetHUDManager`) "NewEnumerator0" (struct :`R` 1.0 :`G` 1.0 :`B` 1.0 :`A` 1.0) false)))))

(event `GPInteractionInterface.ShowInteractUI`
  (params (InstigatorPawn :type "Pawn Object Reference"))
  (if (`self.Active`)
    (`PrimitiveComponent.SetCustomDepthStencilValue` (`self.ItemMesh`) 252)
    (`PrimitiveComponent.SetRenderCustomDepth` (`self.ItemMesh`) true)))

(event `GPInteractionInterface.HideInteractUI`
  (params (InstigatorPawn :type "Pawn Object Reference"))
  (if (`self.Active`)
    (`PrimitiveComponent.SetRenderCustomDepth` (`self.ItemMesh`) false)))

(fn `GetInteractText`
  (params (InstigatorPawn :type "Pawn Object Reference"))
  (returns (ReturnValue :type Text))
  (return ""))

(fn `GiveItem`
  (params (Target :type "Pawn Object Reference"))
  (bind _asbp_player_controller_game (cast `/Game/GProjectBP/Blueprints/BP_PlayerController_Game` (`Pawn.GetController` Target) :!pure true))
  (`GProjectPlayerController.AddInventoryItem` _asbp_player_controller_game "/Game/GProjectBP/DataAsset/Items/Weapon/Weapon_Test1.Weapon_Test1" 1 1 true)
  (`GProjectPlayerController.AddInventoryItem` _asbp_player_controller_game "/Game/GProjectBP/DataAsset/Items/Token/Ammo_Test1.Ammo_Test1" 10000 1 true)
  (`self.SetActorHiddenInGame` true)
  (set `self.Active` false)
  (return))

(fn `UserConstructionScript`)