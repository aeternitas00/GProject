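; Tutorial interactable double sliding door that completes a task and posts a HUD notification on its first active interaction, even if locked.
; While active, it highlights both panels through custom depth stencil when the interact UI shows.
; Interacting toggles the unlocked door through a timeline that lerps the panels apart or back, with an optional timer to auto-close it.
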(event `GPInteractionInterface.HideInteractUI`
  (params (InstigatorPawn :type "Pawn Object Reference"))
  (if (`self.Active`)
    (`PrimitiveComponent.SetRenderCustomDepth` (`self.Door`) false)
    (`PrimitiveComponent.SetRenderCustomDepth` (`self.Door_02`) false)))

(event `GPInteractionInterface.ShowInteractUI`
  (params (InstigatorPawn :type "Pawn Object Reference"))
  (if (`self.Active`)
    (`PrimitiveComponent.SetCustomDepthStencilValue` (`self.Door_02`) 252)
    (`PrimitiveComponent.SetCustomDepthStencilValue` (`self.Door`) 252)
    (`PrimitiveComponent.SetRenderCustomDepth` (`self.Door`) true)
    (`PrimitiveComponent.SetRenderCustomDepth` (`self.Door_02`) true)))

(event `GPInteractionInterface.Interact`
  (params (InstigatorPawn :type "Pawn Object Reference"))
  (bind _isopened (`self.IsOpened`))
  (bind _returnvalue (not _isopened))
  (if (`self.Active`)
    (`|ExecutionSequence`
      (:`then_0`
        (if (`self.IsLocked`)
          _
          (elif _isopened
            (set `self.IsOpened` _returnvalue)
            (bind (_direction _offset) (`Timeline|ToggleDoor` :!via `Reverse` :!label _label)
              (:`Update`
                (`SceneComponent.K2_SetRelativeLocation` (`self.Door`) (`KismetMathLibrary.VLerp` (0.0 0.0 0.0) (-110.0 0.0 0.0) _offset) false false)
                (`SceneComponent.K2_SetRelativeLocation` (`self.Door_02`) (`KismetMathLibrary.VLerp` (400.0 0.0 0.0) (510.0 0.0 0.0) _offset) false false)))
            (else
              (set `self.IsOpened` _returnvalue)
              (if (`self.UseAutoClose`)
                (`KismetSystemLibrary.K2_SetTimerDelegate` (delegate `AutoClose`) (`self.AutoCloseDelay`))
                (goto _label)
                (else
                  (goto _label)))))))
      (:`then_1`
        (`/Engine/EditorBlueprintResources/StandardMacros.DoOnce` false
          (:`Completed`
            (`self.Task Complete`)
            (`/Game/ProHUDV2/Blueprints/Libraries/BPi_HUDManagerV2.CreateUpdateNotification` (`/Game/ProHUDV2/Blueprints/Libraries/BP_PHV2_Functions.GetHUDManager`) (`self.NotInfo`))))))))

(event `AutoClose`
  (bind _isopened (`self.IsOpened`))
  (if _isopened
    (set `self.IsOpened` (not _isopened))
    (goto _label :!via `Reverse`)))

(fn `GetInteractText`
  (params (InstigatorPawn :type "Pawn Object Reference"))
  (returns (ReturnValue :type Text))
  (return ""))

(fn `UserConstructionScript`)