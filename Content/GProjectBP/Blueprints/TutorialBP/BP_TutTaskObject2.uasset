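; Tutorial task object that completes its task after being shot by projectiles five times.
; While active, skeletal mesh hits from GPProjectileBase actors increment a counter, and reaching the threshold fires a one-time completion.
; Completion calls TaskComplete and switches the mesh to simulated ragdoll physics.
; After a tiny delay, it launches the bodies below the struck bone with an impulse along the hit normal.
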(event `self.SkeletalMesh.OnComponentHit`
  (params (HitComponent :type "PrimitiveComponent Object Reference") (OtherActor :type "Actor Object Reference") (OtherComp :type "PrimitiveComponent Object Reference") (NormalImpulse :type "Vector Structure") (Hit :type "HitResult Structure (by ref)"))
  (bind (_bblockinghit _binitialoverlap _time _distance _location _impactpoint _normal _impactnormal _physmat _hitactor _hitcomponent _hitbonename) (`GameplayStatics.BreakHitResult` Hit))
  (bind _skeletalmesh (`self.SkeletalMesh`))
  (cast `GPProjectileBase` OtherActor)
  (if (`self.Active`)
    (bind _result (`/Engine/EditorBlueprintResources/StandardMacros.IncrementInt` (`self.HitCount`))
      (:`  `
        (if (>= _result 5)
          (`/Engine/EditorBlueprintResources/StandardMacros.DoOnce` false
            (:`Completed`
              (`self.Task Complete`)
              (`PrimitiveComponent.SetCollisionProfileName` _skeletalmesh "Ragdoll" true)
              (`SkeletalMeshComponent.SetAllBodiesSimulatePhysics` _skeletalmesh true)
              (`KismetSystemLibrary.Delay` 0.01)
              (`SkeletalMeshComponent.AddImpulseToAllBodiesBelow` (`self.SkeletalMesh`) (* _normal 3000.0) _hitbonename true true))))))))

(fn `UserConstructionScript`)