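; Player controller for the tutorial level, which switches input to game-only when play begins.
; Its PostInitLvl event enables input, shows the HUD through the HUD manager and posts the first timed tutorial notification.
; It then hides the player character's HP and Ammo components and closes the loading screen.
; The Tick event is disabled and a minimap call is left unconnected.
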(event `self.ReceiveBeginPlay`
  (`parent.ReceiveBeginPlay`)
  (`WidgetBlueprintLibrary.SetInputMode_GameOnly` self))

(event `self.Post Init Lvl`
  (bind _hud_manager (`/Game/ProHUDV2/Blueprints/Libraries/BP_PHV2_Functions.GetHUDManager`))
  (`self.EnableInput` self)
  (`/Game/ProHUDV2/Blueprints/Libraries/BPi_HUDManagerV2.ShowHUD` _hud_manager)
  (`/Game/ProHUDV2/Blueprints/Libraries/BPi_HUDManagerV2.CreateTutorialNotification` _hud_manager (make `/Game/ProHUDV2/Blueprints/Structs/S_TutNotiInfo` 60.0 "/Game/GProjectBP/Blueprints/WidgetBP/Tutorial/WB_TutNoti1.WB_TutNoti1_C" (struct :`R` 0.057292 :`G` 0.057292 :`B` 0.057292 :`A` 1.0)))
  (`SceneComponent.SetVisibility` (`/Game/GProjectBP/Blueprints/BP_CharacterBase.HP` (`self.PlayerCharacter`)) false false)
  (`SceneComponent.SetVisibility` (`/Game/GProjectBP/Blueprints/BP_CharacterBase.Ammo` (`self.PlayerCharacter`)) false false)
  (`/Game/GProjectBP/Blueprints/WidgetBP/WB_LoadingScreen.Close Loading Scr` (`self.loadingscr`)))

(fn `UserConstructionScript`
  (`parent.UserConstructionScript`))