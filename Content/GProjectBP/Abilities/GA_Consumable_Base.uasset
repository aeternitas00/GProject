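; Base gameplay ability for consumable items, which applies an item's effects and uses up one unit from the player's inventory.
; On activation it commits, then builds and applies the effect container tagged Ability.Item.
; It then removes one of the item in slot number 1 through BP_PlayerController_Game.
; Only a failed commit calls EndAbility here; the success path does not end the ability in this graph.
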(event `self.K2_ActivateAbility`
  (bind (_returnvalue_owneractor _returnvalue_avataractor _returnvalue_playercontroller) (break `GameplayAbilityActorInfo` (`self.GetActorInfo`)))
  (`parent.K2_ActivateAbility`)
  (bind _returnvalue (`self.K2_CommitAbility`))
  (if _returnvalue
    (bind _returnvalue_2 (`self.MakeEffectContainerSpec` (struct :`TagName` "Ability.Item")))
    (`self.ApplyEffectContainerSpec` _returnvalue_2)
    (bind _asbp_player_controller_game (cast `/Game/GProjectBP/Blueprints/BP_PlayerController_Game` _returnvalue_playercontroller))
    (`GProjectPlayerController.RemoveInventoryItem` _asbp_player_controller_game (`GProjectPlayerController.GetSlottedItem` _asbp_player_controller_game (make `GPItemSlot` "Consumable" 1)) 1)
    (else
      (`self.K2_EndAbility`))))