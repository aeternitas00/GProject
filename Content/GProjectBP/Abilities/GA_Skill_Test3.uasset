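; Test gameplay ability that knocks targets away from its owner with an explosion-style radial impulse.
; On AbilityWork it prints a debug label and resolves target actors from every entry in its effect container map.
; Each target's mesh components receive a velocity-change radial impulse centered on the owner; the graph applies no gameplay effects from the containers.
; It then spawns an explosion emitter at the owner's location and ends immediately.
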(event `self.Ability Work`
  (params (Tag :type "GameplayTag Structure") (`Event data` :type "GameplayEventData Structure"))
  (bind _returnvalue (`Actor.K2_GetActorLocation` (`.OwnerActor` (break `GameplayAbilityActorInfo` (`self.GetActorInfo`)))))
  (`KismetSystemLibrary.PrintText` "Skill_Test3")
  (bind _values (`BlueprintMapLibrary.Map_Values` (`self.EffectContainerMap`)))
  (for _array_element _values
    (bind (_outhitresults _outtargetactors _returnvalue_2) (`self.GetTargetsFromEffectContainer` _array_element (make `GameplayEventData` (struct))))
    (if _returnvalue_2
      (for (_array_element_2 _array_index) _outtargetactors
        (for _array_element_3 (`Actor.K2_GetComponentsByClass` _array_element_2 "/Script/Engine.MeshComponent")
          (`PrimitiveComponent.AddRadialImpulse` _array_element_3 _returnvalue 500.0 2000.0 "RIF_Linear" true)))))
  (`GameplayStatics.SpawnEmitterAtLocation` "/Game/WeaponAssets/SciFiWeapDark/FX/Particles/P_RocketLauncher_Explosion_Dark.P_RocketLauncher_Explosion_Dark" _returnvalue)
  (`self.K2_EndAbility`))