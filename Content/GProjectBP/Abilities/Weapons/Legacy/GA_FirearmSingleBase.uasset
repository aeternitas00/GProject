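; Legacy base gameplay ability for single-shot firearms, exposing ammo item and magazine size.
; On commit it multicasts the weapon's fire animation, plays a montage and spawns a muzzle projectile on the montage event.
; Dedicated servers and non-authority instances hide that bullet and multicast an effectless copy from the muzzle with a yaw offset, working around double spawning.
; Non-dedicated authority, intended for single-player testing, spawns only the normal bullet.
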(event `self.K2_ActivateAbility`
  (bind _returnvalue (`self.K2_CommitAbility`))
  (if _returnvalue
    (bind _asgpcharacter_base (cast `GPCharacterBase` (`self.GetOwningActorFromActorInfo`))
      (:`then`
        (bind _asbp_scifi_weapon_actor_base (cast `/Game/GProjectBP/Blueprints/Weapons/BP_ScifiWeaponActor_Base` (`GPCharacterBase.CurrentWeaponActor` _asgpcharacter_base))
          (:`then`
            (`/Game/GProjectBP/Blueprints/Weapons/BP_ScifiWeaponActor_Base.Multicast Play Fire Anim` _asbp_scifi_weapon_actor_base)
            (bind (_asynctaskproxy _eventtag _eventdata) (`GPAbilityTask_PlayMontage.PlayMontageAndWaitForEvent` "None" (`self.PlayingMontage`) (struct :`GameplayTags` (struct :`(TagName` "Event.Montage"))))
              (:`EventReceived`
                ;[1 1 1] Logic like below comment box causes double projectile spawn when player fire this ability. so i changed to this
                (if (`KismetSystemLibrary.IsDedicatedServer`)
                  (bind _proj (`/Game/GProjectBP/Abilities/Weapons/GPGAMacroLibrary.Spawn a Bullet at Muzzle` _eventtag _eventdata (`self.ProjectileClass`) :!label _label)
                    (:`Out`
                      (`Actor.SetActorHiddenInGame` _proj true)
                      (bind _asgpcharacter_base_2 (cast `GPCharacterBase` (`self.GetOwningActorFromActorInfo`))
                        (:`then`
                          (bind _asbp_scifi_weapon_actor_base_2 (cast `/Game/GProjectBP/Blueprints/Weapons/BP_ScifiWeaponActor_Base` (`GPCharacterBase.CurrentWeaponActor` _asgpcharacter_base_2))
                            (:`then`
                              (`self.Multicast Spawn Bulet` (`self.ProjectileClass`) (`KismetMathLibrary.MakeTransform` (.location (`/Game/GProjectBP/Blueprints/Weapons/BP_ScifiWeaponActor_Base.Get Muzzle Transform` _asbp_scifi_weapon_actor_base_2)) (`KismetMathLibrary.MakeRotator` (.roll (.rotation (`/Game/GProjectBP/Blueprints/Weapons/BP_ScifiWeaponActor_Base.Get Muzzle Transform` _asbp_scifi_weapon_actor_base_2))) (.pitch (.rotation (`/Game/GProjectBP/Blueprints/Weapons/BP_ScifiWeaponActor_Base.Get Muzzle Transform` _asbp_scifi_weapon_actor_base_2))) (- (.yaw (.rotation (`/Game/GProjectBP/Blueprints/Weapons/BP_ScifiWeaponActor_Base.Get Muzzle Transform` _asbp_scifi_weapon_actor_base_2))) 5.0)) (.scale (`/Game/GProjectBP/Blueprints/Weapons/BP_ScifiWeaponActor_Base.Get Muzzle Transform` _asbp_scifi_weapon_actor_base_2))) _asgpcharacter_base_2)
                              (`self.K2_EndAbility`))
                            (:`CastFailed`
                              (`KismetSystemLibrary.PrintString` "weapon failed"))))
                        (:`CastFailed`
                          (`KismetSystemLibrary.PrintString` "get char failed")))))
                  (else
                    ;;[1 1 1] For Single play Test
                    (`self.K2_HasAuthority`
                      (:`True`
                        (`/Game/GProjectBP/Abilities/Weapons/GPGAMacroLibrary.Spawn a Bullet at Muzzle` _eventtag _eventdata (`self.ProjectileClass`)
                          (:`Out`
                            (`self.K2_EndAbility`))))
                      (:`False`
                        (goto _label))))))))
          (:`CastFailed`
            (`KismetSystemLibrary.PrintString` "Get weapon actor failed"))))
      (:`CastFailed`
        (`KismetSystemLibrary.PrintString` "get character failed")))
    (else
      (`self.K2_EndAbility`))))

(event `Multicast Spawn Bulet`
  (params (Projectile :type "GPProjectileBase Class Reference") (inTransform :type "Transform Structure") (inInstigator :type "Character Object Reference"))
  (`/Game/GProjectBP/Abilities/Weapons/GPGAMacroLibrary.Spawn a Effectless Bullet` Projectile inTransform inInstigator))

(event `GPMagAbilityInterface.SetMagSize`
  (params (inMagSize :type "Float (single-precision)"))
  (set `self.MagSize` inMagSize))

(fn `GetAmmoItem`
  (returns (ReturnValue :type "GPItem Object Reference"))
  (return (`self.AmmoItem`)))

(fn `GetMagSize`
  (returns (ReturnValue :type "Float (double-precision)"))
  (return (`self.MagSize`)))