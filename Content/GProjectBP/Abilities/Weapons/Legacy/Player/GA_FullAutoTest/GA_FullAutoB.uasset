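; Legacy test gameplay ability for full-auto weapon fire, built as a toggle ability with ammo and magazine accessors.
; Each work cycle plays a montage whose event spawns a muzzle projectile, with DoOnce guarding against double-fired notifies.
; Dedicated servers hide their bullet and multicast an effectless copy with a yaw-offset muzzle transform; otherwise authority spawns directly.
; A looping rifle sound starts at setup and stops on ability end, skipped on dedicated servers.
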(event `self.OnToggleWorkBegin`
  (bind (_asynctaskproxy _eventtag _eventdata) (`GPAbilityTask_PlayMontage.PlayMontageAndWaitForEvent` "None" (`self.Montage to Play`) (struct :`GameplayTags` (struct :`(TagName` "Event.Montage"))))
    (:`then`
      (goto _label :!via `Reset`))
    (:`EventReceived`
      (`/Engine/EditorBlueprintResources/StandardMacros.DoOnce` false :!label _label ; ANS Bug ( if it is too fast, event received called twice )
        (:`Completed`
          (if (`KismetSystemLibrary.IsDedicatedServer`)
            (bind _proj (`/Game/GProjectBP/Abilities/Weapons/GPGAMacroLibrary.Spawn a Bullet at Muzzle` _eventtag _eventdata (`self.ProjectileClass`))
              (:`Out`
                (`Actor.SetActorHiddenInGame` _proj true)
                (bind _asgpcharacter_base (cast `GPCharacterBase` (`self.GetOwningActorFromActorInfo`))
                  (:`then`
                    (bind _asbp_scifi_weapon_actor_base (cast `/Game/GProjectBP/Blueprints/Weapons/BP_ScifiWeaponActor_Base` (`GPCharacterBase.CurrentWeaponActor` _asgpcharacter_base))
                      (:`then`
                        (`self.Multicast Spawn Bulet` (`self.ProjectileClass`) (`KismetMathLibrary.MakeTransform` (.location (`/Game/GProjectBP/Blueprints/Weapons/BP_ScifiWeaponActor_Base.Get Muzzle Transform` _asbp_scifi_weapon_actor_base)) (`KismetMathLibrary.MakeRotator` (.roll (.rotation (`/Game/GProjectBP/Blueprints/Weapons/BP_ScifiWeaponActor_Base.Get Muzzle Transform` _asbp_scifi_weapon_actor_base))) (.pitch (.rotation (`/Game/GProjectBP/Blueprints/Weapons/BP_ScifiWeaponActor_Base.Get Muzzle Transform` _asbp_scifi_weapon_actor_base))) (- (.yaw (.rotation (`/Game/GProjectBP/Blueprints/Weapons/BP_ScifiWeaponActor_Base.Get Muzzle Transform` _asbp_scifi_weapon_actor_base))) 5.0)) (.scale (`/Game/GProjectBP/Blueprints/Weapons/BP_ScifiWeaponActor_Base.Get Muzzle Transform` _asbp_scifi_weapon_actor_base))) _asgpcharacter_base))
                      (:`CastFailed`
                        (`KismetSystemLibrary.PrintString` "weapon failed"))))
                  (:`CastFailed`
                    (`KismetSystemLibrary.PrintString` "get char failed")))))
            (else
              ;[1 1 1] For Single play Test
              (`self.K2_HasAuthority`
                (:`True`
                  (`/Game/GProjectBP/Abilities/Weapons/GPGAMacroLibrary.Spawn a Bullet at Muzzle` _eventtag _eventdata (`self.ProjectileClass`)))))))))))

(event `Cleanup Sound`
  ;[1 1 1] Sound work
  (if (and (not (`KismetSystemLibrary.IsDedicatedServer`)) (`KismetSystemLibrary.IsValid` (`self.LoopSound`)))
    (`AudioComponent.StopDelayed` (`self.LoopSound`) 0.03)
    (`KismetSystemLibrary.PrintString` "Cleanup Sound succ")))

(event `Multicast Spawn Sound Attached`
  (params (`Firing actor` :type "Actor Object Reference"))
  ;[1 1 1] Sound work
  (if (not (`KismetSystemLibrary.IsDedicatedServer`))
    (`/Engine/EditorBlueprintResources/StandardMacros.IsValid` (`self.LoopSound`)
      (:`Is Not Valid`
        (bind _returnvalue (`GameplayStatics.SpawnSoundAttached` "/Game/SciFiWeapDark/Sound/Rifle/RifleA_FireLoop_Cue.RifleA_FireLoop_Cue" (`Actor.RootComponent` `Firing actor`) "None" (0.0 0.0 0.0) (struct) "KeepRelativeOffset" true 1.0 1.0 0.0 null null))
        (set `self.LoopSound` _returnvalue)
        (`KismetSystemLibrary.PrintString` "play sound")))))

(event `self.K2_OnEndAbility`
  (params (bWasCancelled :type Boolean))
  (`self.Cleanup Sound`)
  (`parent.K2_OnEndAbility` bWasCancelled))

(event `GPMagAbilityInterface.SetMagSize`
  (params (inMagSize :type "Float (single-precision)"))
  (set `self.MagSize` inMagSize))

(event `Multicast Spawn Bulet`
  (params (Projectile :type "GPProjectileBase Class Reference") (inTransform :type "Transform Structure") (inInstigator :type "Character Object Reference"))
  (`/Game/GProjectBP/Abilities/Weapons/GPGAMacroLibrary.Spawn a Effectless Bullet` Projectile inTransform inInstigator))

(fn `GetAmmoItem`
  (returns (ReturnValue :type "GPItem Object Reference"))
  (return (`self.AmmoItem`)))

(fn `GetMagSize`
  (returns (ReturnValue :type "Float (double-precision)"))
  (return (`self.MagSize`)))

(fn `OnRep_LoopSound`)

(fn `Setup Toggle Ability`
  (`parent.Setup Toggle Ability`)
  (`self.Multicast Spawn Sound Attached` (`self.GetOwningActorFromActorInfo`)))