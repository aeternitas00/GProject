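; Legacy test player weapon ability that fires a shotgun-style burst of spread projectiles.
; On commit it multicasts the weapon fire animation and plays a montage, whose event spawns the bullets at the muzzle before ending the ability.
; A dedicated server hides its projectiles and multicasts copies to clients with the owning character as instigator.
; Other authority instances spawn visible bullets only, for single-play testing, while non-authority ones reuse the server path.
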(event `self.K2_ActivateAbility`
  (bind _returnvalue (`self.K2_CommitAbility`))
  (if _returnvalue
    (bind _asgpcharacter_base (cast `GPCharacterBase` (`self.GetOwningActorFromActorInfo`))
      (:`then`
        (bind _asbp_scifi_weapon_actor_base (cast `/Game/GProjectBP/Blueprints/Weapons/BP_ScifiWeaponActor_Base` (`GPCharacterBase.CurrentWeaponActor` _asgpcharacter_base))
          (:`then`
            (`/Game/GProjectBP/Blueprints/Weapons/BP_ScifiWeaponActor_Base.Multicast Play Fire Anim` _asbp_scifi_weapon_actor_base)
            (bind (_asynctaskproxy _eventtag _eventdata) (`GPAbilityTask_PlayMontage.PlayMontageAndWaitForEvent` "None" (`self.PlayingMontage`) (struct :`GameplayTags` (struct :`(TagName` "Event.Montage"))))
              (:`EventReceived`
                ;[1 1 1] Multiple Bullet
                (if (`KismetSystemLibrary.IsDedicatedServer`)
                  (for _ (range 4) :!label _label
                    (bind _proj (`/Game/GProjectBP/Abilities/Weapons/GPGAMacroLibrary.Spawn a Bullet at Muzzle` _eventtag _eventdata (`self.ProjectileClass`))
                      (:`Out`
                        (`/Game/GProjectBP/Abilities/Weapons/GPGAMacroLibrary.Spread Bullet` _proj 5.0)
                        (`Actor.SetActorHiddenInGame` _proj true)
                        (bind _asgpcharacter_base_2 (cast `GPCharacterBase` (`self.GetOwningActorFromActorInfo`)))
                        (`self.Multicast Spawn Bulet` (`self.ProjectileClass`) (`Actor.GetTransform` _proj) _asgpcharacter_base_2))))
                  (`self.K2_EndAbility`)
                  (else
                    ;;[1 1 1] For Single play Test
                    (`self.K2_HasAuthority`
                      (:`True`
                        (for _ (range 4)
                          (bind _proj_2 (`/Game/GProjectBP/Abilities/Weapons/GPGAMacroLibrary.Spawn a Bullet at Muzzle` _eventtag _eventdata (`self.ProjectileClass`))
                            (:`Out`
                              (`/Game/GProjectBP/Abilities/Weapons/GPGAMacroLibrary.Spread Bullet` _proj_2 5.0))))
                        (`self.K2_EndAbility`))
                      (:`False`
                        (goto _label))))))))
          (:`CastFailed`
            (`KismetSystemLibrary.PrintString` "Get weapon actor failed"))))
      (:`CastFailed`
        (`KismetSystemLibrary.PrintString` "get character failed")))
    (else
      (`self.K2_EndAbility`))))