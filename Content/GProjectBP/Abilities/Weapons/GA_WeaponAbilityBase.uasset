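; Base Gameplay Ability for weapon abilities, with the weapon actor expected as the ability's owning actor.
; Activation commits the ability and, on success, calls AbilityWork, an empty event that serves as the hook for child abilities.
; Ending the ability calls CallOnAbilityEnded.
; Helper functions cast the owning actor to GPWeaponActorBase and that weapon's owner to GPCharacterBase.
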(event `self.K2_ActivateAbility`
  (bind _returnvalue (`self.K2_CommitAbility`))
  (if _returnvalue
    (`self.Ability Work`)))

(event `Ability Work`)

(event `self.K2_OnEndAbility`
  (params (bWasCancelled :type Boolean))
  (`self.OnAbilityEnded`))

(fn `GetOwningWeapon`
  (returns (Weapon :type "GPWeaponActorBase Object Reference"))
  (return (cast `GPWeaponActorBase` (`self.GetOwningActorFromActorInfo`) :!pure true)))

(fn `GetWeaponOwner`
  (returns (`AsGPCharacter Base` :type "GPCharacterBase Object Reference"))
  (return (cast `GPCharacterBase` (`Actor.GetOwner` (`self.GetOwningWeapon`)) :!pure true)))