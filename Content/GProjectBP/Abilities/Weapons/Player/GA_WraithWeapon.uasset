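; Player weapon gameplay ability for the Wraith weapon that supplies a muzzle transform with random horizontal spread.
; GetMuzzleTransform reads the muzzle transform from the owning BP_InvisWeaponActor_Base and adds a small random yaw offset, divided by weapon accuracy.
; Location, pitch, roll and scale pass through unchanged.
; ActivateAbility is only a disabled parent-call stub, so activation logic is not defined in this graph.
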(fn `GetMuzzleTransform`
  (returns (Transform :type "Transform Structure"))
  (return (`KismetMathLibrary.MakeTransform` (.location (`/Game/GProjectBP/Blueprints/Weapons/BP_InvisWeaponActor_Base.Get Muzzle Transform` (cast `/Game/GProjectBP/Blueprints/Weapons/BP_InvisWeaponActor_Base` (`self.GetOwningWeapon`) :!pure true))) (`KismetMathLibrary.MakeRotator` (.roll (.rotation (`/Game/GProjectBP/Blueprints/Weapons/BP_InvisWeaponActor_Base.Get Muzzle Transform` (cast `/Game/GProjectBP/Blueprints/Weapons/BP_InvisWeaponActor_Base` (`self.GetOwningWeapon`) :!pure true)))) (.pitch (.rotation (`/Game/GProjectBP/Blueprints/Weapons/BP_InvisWeaponActor_Base.Get Muzzle Transform` (cast `/Game/GProjectBP/Blueprints/Weapons/BP_InvisWeaponActor_Base` (`self.GetOwningWeapon`) :!pure true)))) (+ (.yaw (.rotation (`/Game/GProjectBP/Blueprints/Weapons/BP_InvisWeaponActor_Base.Get Muzzle Transform` (cast `/Game/GProjectBP/Blueprints/Weapons/BP_InvisWeaponActor_Base` (`self.GetOwningWeapon`) :!pure true)))) (/ (`KismetMathLibrary.RandomFloatInRange` -5.0 5.0) (`GPWeaponActorBase.GetAccuracy` (`self.GetOwningWeapon`))))) (.scale (`/Game/GProjectBP/Blueprints/Weapons/BP_InvisWeaponActor_Base.Get Muzzle Transform` (cast `/Game/GProjectBP/Blueprints/Weapons/BP_InvisWeaponActor_Base` (`self.GetOwningWeapon`) :!pure true))))))