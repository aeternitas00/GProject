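; Base player sci-fi weapon ability that fires a projectile from the owning weapon's muzzle and then ends.
; AbilityWork builds an effect container spec from a montage event tag and passes it to the spawned projectile, which the owner's capsule ignores when moving.
; GetMuzzleTransform reads the weapon actor's muzzle and adds random yaw divided by weapon accuracy.
; SpreadBullet, uncalled here, randomly rotates a projectile and its velocity in pitch and yaw.
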(event `self.Ability Work`
  (`KismetSystemLibrary.PrintString` "ScifiWeap")
  (bind _projectile (`self.SpawnProjectileFromMuzzle` (struct :`TagName` "Event.Montage.Shared.Weapon") (make `GameplayEventData` (struct)) (`self.ProjectileClass`)))
  (`KismetSystemLibrary.PrintString` (`KismetSystemLibrary.GetObjectName` _projectile))
  (`self.K2_EndAbility`))

(event `self.K2_OnEndAbility`
  (params (bWasCancelled :type Boolean))
  (`parent.K2_OnEndAbility` bWasCancelled))

(fn `GetMuzzleTransform`
  (returns (Transform :type "Transform Structure"))
  (return (`KismetMathLibrary.MakeTransform` (.location (`/Game/GProjectBP/Blueprints/Weapons/BP_ScifiWeaponActor_Base.Get Muzzle Transform` (cast `/Game/GProjectBP/Blueprints/Weapons/BP_ScifiWeaponActor_Base` (`self.GetOwningWeapon`) :!pure true))) (`KismetMathLibrary.MakeRotator` (.roll (.rotation (`/Game/GProjectBP/Blueprints/Weapons/BP_ScifiWeaponActor_Base.Get Muzzle Transform` (cast `/Game/GProjectBP/Blueprints/Weapons/BP_ScifiWeaponActor_Base` (`self.GetOwningWeapon`) :!pure true)))) (.pitch (.rotation (`/Game/GProjectBP/Blueprints/Weapons/BP_ScifiWeaponActor_Base.Get Muzzle Transform` (cast `/Game/GProjectBP/Blueprints/Weapons/BP_ScifiWeaponActor_Base` (`self.GetOwningWeapon`) :!pure true)))) (+ (.yaw (.rotation (`/Game/GProjectBP/Blueprints/Weapons/BP_ScifiWeaponActor_Base.Get Muzzle Transform` (cast `/Game/GProjectBP/Blueprints/Weapons/BP_ScifiWeaponActor_Base` (`self.GetOwningWeapon`) :!pure true)))) (/ (`KismetMathLibrary.RandomFloatInRange` -5.0 5.0) (`GPWeaponActorBase.GetAccuracy` (`self.GetOwningWeapon`))))) (.scale (`/Game/GProjectBP/Blueprints/Weapons/BP_ScifiWeaponActor_Base.Get Muzzle Transform` (cast `/Game/GProjectBP/Blueprints/Weapons/BP_ScifiWeaponActor_Base` (`self.GetOwningWeapon`) :!pure true))))))

(fn `SpawnProjectileFromMuzzle`
  (params (ContainerTag :type "GameplayTag Structure") (EventData :type "GameplayEventData Structure (by ref)") (ProjectileClass :type "GPProjectileBase Class Reference"))
  (returns (Projectile :type "GPProjectileBase Object Reference"))
  (bind _asgpcharacter_base (`self.GetWeaponOwner`))
  ;[1 1 1] Projectile's validation check
  (bind _returnvalue (`self.MakeEffectContainerSpec` ContainerTag EventData))
  (if (`GPBPFuncLibrary.DoesEffectContainerSpecHaveEffects` _returnvalue)
    (if (`KismetSystemLibrary.IsValidClass` ProjectileClass)
      ;[1 1 1] Make transform for spawning projectile ( firearm's muzzle )
      (bind _returnvalue_2 (`|SpawnActorFromClass` ProjectileClass (`self.GetMuzzleTransform`) "AlwaysSpawn" "OverrideRootScale" _asgpcharacter_base _returnvalue _asgpcharacter_base))
      (`PrimitiveComponent.IgnoreActorWhenMoving` (`Character.CapsuleComponent` _asgpcharacter_base) _returnvalue_2 true)
      (return _returnvalue_2)
      (else
        (`KismetSystemLibrary.PrintString` "Proj class is not valid class")))
    (else
      (`KismetSystemLibrary.PrintString` "Spec failed"))))

(fn `SpreadBullet`
  (params (Projectile :type "GPProjectileBase Object Reference") (SpreadScale :type "Float (double-precision)"))
  (bind _returnvalue (* -1 SpreadScale))
  (bind _projmovementcomp (`GPProjectileBase.ProjMovementComp` Projectile))
  (bind _returnvalue_2 (`KismetMathLibrary.MakeRotator` 0.0 (`KismetMathLibrary.RandomFloatInRange` _returnvalue SpreadScale) (`KismetMathLibrary.RandomFloatInRange` _returnvalue SpreadScale)))
  (`Actor.K2_AddActorWorldRotation` Projectile _returnvalue_2 false false)
  (set `MovementComponent.Velocity` (`KismetMathLibrary.GreaterGreater_VectorRotator` (`MovementComponent.Velocity` _projmovementcomp) _returnvalue_2) _projmovementcomp))