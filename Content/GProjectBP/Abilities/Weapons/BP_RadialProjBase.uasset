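; Base radial-damage weapon projectile that, on its first valid hit, applies gameplay effects and physics impulses within an effect radius.
; Hits on move-ignored actors are skipped; otherwise one sphere trace gathers targets for the effect container spec, notifying a character owner when effects apply.
; A second trace applies linear-falloff radial impulses to hit components.
; It then plays impact FX and sound, ends trails, disables collision and expires after a short lifespan.
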(event `self.ReceiveHit`
  (params (MyComp :type "PrimitiveComponent Object Reference") (Other :type "Actor Object Reference") (OtherComp :type "PrimitiveComponent Object Reference") (bSelfMoved :type Boolean) (HitLocation :type "Vector Structure") (HitNormal :type "Vector Structure") (NormalImpulse :type "Vector Structure") (Hit :type "HitResult Structure (by ref)"))
  (bind _returnvalue (`PrimitiveComponent.CopyArrayOfMoveIgnoreActors` (`self.SphereCollision`)))
  (if (`KismetArrayLibrary.Array_Contains` _returnvalue Other)
    _
    (elif (not (`self.bIsWaitingToKill`))
      ;[1 1 1] Gameplay Effect
      (bind _outhits (`KismetSystemLibrary.SphereTraceMultiForObjects` :`Start` HitLocation :`End` HitLocation :`Radius` (`self.EffectRadius`) :`ObjectTypes` (`self.GETypes`) :`DrawTime` 1.0))
      (for _array_element _outhits
        (`KismetArrayLibrary.Array_AddUnique` (`self.HitTempActors`) (`.HitActor` (`GameplayStatics.BreakHitResult` _array_element))))
      (bind _returnvalue_2 (`GPBPFuncLibrary.AddTargetsToEffectContainerSpec` :`ContainerSpec` (`self.EffectContainerSpec`) :`TargetActors` (`self.HitTempActors`)))
      (bind _returnvalue_3 (`GPBPFuncLibrary.ApplyExternalEffectContainerSpec` _returnvalue_2))
      (if (> (`KismetArrayLibrary.Array_Length` _returnvalue_3) 0)
        (bind _asbp_character_base (cast `/Game/GProjectBP/Blueprints/BP_CharacterBase` (`self.GetOwner`))
          (:`then`
            (`/Game/GProjectBP/Blueprints/BP_CharacterBase.Own Attack Hitted` _asbp_character_base))
          (:`CastFailed`
            _)))
      ;[1 1 1] Physics
      (bind _outhits_2 (`KismetSystemLibrary.SphereTraceMultiForObjects` :`Start` HitLocation :`End` HitLocation :`Radius` (`self.EffectRadius`) :`ObjectTypes` (`self.PhysicsTypes`) :`DrawTime` 1.0))
      (for _array_element_2 _outhits_2
        (`PrimitiveComponent.AddRadialImpulse` (`.HitComponent` (`GameplayStatics.BreakHitResult` _array_element_2)) HitLocation (`self.EffectRadius`) (`self.ImpulseStrength`) "RIF_Linear" false))
      ;[1 1 1] Cleanup
      (`GameplayStatics.SpawnEmitterAtLocation` (`self.EmitterTemplate`) HitLocation (`KismetMathLibrary.Conv_VectorToRotator` HitNormal))
      (`GameplayStatics.PlaySoundAtLocation` (`self.HitSound`) HitLocation (struct) 1.0 1.0 0.0 null null null)
      (`ParticleSystemComponent.EndTrails` (`self.ParticleSystem`))
      (set `self.bIsWaitingToKill` true)
      (`self.SetLifeSpan` (`self.LifespanAfterHit`))
      (`PrimitiveComponent.SetCollisionEnabled` (`self.SphereCollision`) "NoCollision"))))

(fn `UserConstructionScript`
  (`parent.UserConstructionScript`))