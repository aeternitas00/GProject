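; BP_TestWeaponProj3 is a test weapon projectile that keeps speeding up horizontally while in flight.
; Each Tick adds a fixed, frame-time-scaled acceleration to the movement component's velocity along its normalized XY direction, leaving vertical velocity untouched.
; Its audio starts shortly after BeginPlay and stops on hit, with both events also calling the parent class's logic.
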(event `self.ReceiveTick`
  (params (DeltaSeconds :type "Float (single-precision)"))
  (bind _projmovementcomp (`self.ProjMovementComp`))
  (bind _velocity (`MovementComponent.Velocity` _projmovementcomp))
  (set `MovementComponent.Velocity` (+ _velocity (* (`KismetMathLibrary.Normal` (`KismetMathLibrary.MakeVector` (.x _velocity) (.y _velocity))) (* DeltaSeconds 5000.0))) _projmovementcomp))

(event `self.ReceiveHit`
  (params (MyComp :type "PrimitiveComponent Object Reference") (Other :type "Actor Object Reference") (OtherComp :type "PrimitiveComponent Object Reference") (bSelfMoved :type Boolean) (HitLocation :type "Vector Structure") (HitNormal :type "Vector Structure") (NormalImpulse :type "Vector Structure") (Hit :type "HitResult Structure (by ref)"))
  (`AudioComponent.Stop` (`self.Audio`))
  (`parent.ReceiveHit` MyComp Other OtherComp bSelfMoved HitLocation HitNormal NormalImpulse Hit))

(event `self.ReceiveBeginPlay`
  (`parent.ReceiveBeginPlay`)
  (`KismetSystemLibrary.Delay` 0.1)
  (`AudioComponent.Play` (`self.Audio`) 0.0))

(fn `UserConstructionScript`)