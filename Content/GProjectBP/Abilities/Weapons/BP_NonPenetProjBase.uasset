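; Base weapon projectile that does not penetrate, destroying itself on impact with any actor outside its collision sphere's move-ignore list.
; On such a hit it spawns an impact emitter along the surface normal and calls ProjectileHit.
; If that succeeds on a skeletal mesh, it notifies the owning BP_CharacterBase through OnOwnAttackHitted, flagging headshots when the bone closest to the impact is "head" or its child.
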(event `self.ReceiveHit`
  (params (MyComp :type "PrimitiveComponent Object Reference") (Other :type "Actor Object Reference") (OtherComp :type "PrimitiveComponent Object Reference") (bSelfMoved :type Boolean) (HitLocation :type "Vector Structure") (HitNormal :type "Vector Structure") (NormalImpulse :type "Vector Structure") (Hit :type "HitResult Structure (by ref)"))
  (bind _returnvalue (`PrimitiveComponent.CopyArrayOfMoveIgnoreActors` (`self.SphereCollision`)))
  (if (not (`KismetArrayLibrary.Array_Contains` _returnvalue Other))
    (`GameplayStatics.SpawnEmitterAtLocation` (`self.HitEmitter`) HitLocation (`KismetMathLibrary.Conv_VectorToRotator` HitNormal))
    (bind _returnvalue_2 (`self.ProjectileHit` self Other))
    (if _returnvalue_2
      (bind _asbp_character_base (cast `/Game/GProjectBP/Blueprints/BP_CharacterBase` (`self.GetOwner`))
        (:`then`
          (bind _asskeletal_mesh_component (cast `SkeletalMeshComponent` OtherComp)
            (:`then`
              (bind (_bonelocation _returnvalue_3) (`SkinnedMeshComponent.FindClosestBone_K2` _asskeletal_mesh_component HitLocation 0.0 false))
              (`/Game/GProjectBP/Blueprints/BP_CharacterBase.On Own Attack Hitted` _asbp_character_base (or (`SkinnedMeshComponent.BoneIsChildOf` _asskeletal_mesh_component _returnvalue_3 "head") (== _returnvalue_3 "head"))))
            (:`CastFailed`
              _)))
        (:`CastFailed`
          _)))
    (`self.K2_DestroyActor`)))

(fn `UserConstructionScript`)