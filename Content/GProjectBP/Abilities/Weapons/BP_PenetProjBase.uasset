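; Base projectile Blueprint for weapons that pass through overlapped actors and end on a blocking hit.
; Each overlap spawns a hit emitter and runs ProjectileHit; on success the owning BP_CharacterBase gets OnOwnAttackHitted with a headshot flag.
; Headshots are detected by whether the skeletal mesh bone closest to the projectile is the head or its child.
; Blocking hits spawn the emitter along the surface normal, then destroy the projectile immediately or after LifespanAfterHit.
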(event `self.ReceiveActorBeginOverlap`
  (params (OtherActor :type "Actor Object Reference"))
  (bind _returnvalue (`self.GetComponentByClass` OtherActor "/Script/Engine.SkeletalMeshComponent"))
  (bind _returnvalue_2 (`self.K2_GetActorLocation` self))
  (bind (_bonelocation _returnvalue_3) (`SkinnedMeshComponent.FindClosestBone_K2` _returnvalue _returnvalue_2 0.0 false))
  (bind _returnvalue_4 (`self.ProjectileHit` self OtherActor))
  (`GameplayStatics.SpawnEmitterAtLocation` (`self.HitEmitter`) _returnvalue_2 (* (`self.K2_GetActorRotation` self) -1.0))
  (if _returnvalue_4
    (bind _asbp_character_base (cast `/Game/GProjectBP/Blueprints/BP_CharacterBase` (`self.GetOwner`)))
    (`/Engine/EditorBlueprintResources/StandardMacros.IsValid` _returnvalue
      (:`Is Valid`
        (`/Game/GProjectBP/Blueprints/BP_CharacterBase.On Own Attack Hitted` _asbp_character_base (or (`SkinnedMeshComponent.BoneIsChildOf` _returnvalue _returnvalue_3 "head") (== _returnvalue_3 "head"))))
      (:`Is Not Valid`
        (`/Game/GProjectBP/Blueprints/BP_CharacterBase.On Own Attack Hitted` _asbp_character_base false)))))

(event `self.ReceiveHit`
  (params (MyComp :type "PrimitiveComponent Object Reference") (Other :type "Actor Object Reference") (OtherComp :type "PrimitiveComponent Object Reference") (bSelfMoved :type Boolean) (HitLocation :type "Vector Structure") (HitNormal :type "Vector Structure") (NormalImpulse :type "Vector Structure") (Hit :type "HitResult Structure (by ref)"))
  (bind _lifespanafterhit (`self.LifespanAfterHit`))
  (`GameplayStatics.SpawnEmitterAtLocation` (`self.HitEmitter`) HitLocation (`KismetMathLibrary.Conv_VectorToRotator` HitNormal))
  (if (`KismetMathLibrary.NearlyEqual_FloatFloat` _lifespanafterhit)
    (`self.K2_DestroyActor`)
    (else
      (`self.SetLifeSpan` _lifespanafterhit))))

(fn `UserConstructionScript`)