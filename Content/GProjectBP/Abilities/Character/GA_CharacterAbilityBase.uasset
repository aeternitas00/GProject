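; Base gameplay ability for characters, providing a commit, montage and work flow with an overridable AbilityWork hook.
; After a successful commit, it multicasts any montage from the server and runs a montage task that fires AbilityWork once, on the first Event.Montage event.
; Without a montage, AbilityWork runs immediately.
; The ability ends after work, montage completion, cancellation or failed commit unless EndSpecified is set, while the montage can outlive it.
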(event `self.K2_ActivateAbility`
  (bind _returnvalue (`self.K2_CommitAbility`))
  (set `self.bActive` _returnvalue)
  (if _returnvalue
    (`/Engine/EditorBlueprintResources/StandardMacros.IsValid` (`self.PlayingMontage`)
      (:`Is Valid`
        (`self.K2_HasAuthority`
          (:`True`
            (`/Game/GProjectBP/Blueprints/BP_CharacterBase.Multicast Montage Play` (`self.GetOwningCharacter`) (`self.PlayingMontage`) 1.0 0.0 "None"))
          (:`False`
            _))
        (bind (_asynctaskproxy _eventtag _eventdata) (`GPAbilityTask_PlayMontage.PlayMontageAndWaitForEvent` (`KismetStringLibrary.Conv_StringToName` (`KismetSystemLibrary.GetObjectName` self)) (`self.PlayingMontage`) (struct :`GameplayTags` (struct :`(TagName` "Event.Montage"))) 1.0 "None" false)
          (:`then`
            (goto _label :!via `Reset`))
          (:`OnCompleted`
            _)
          (:`OnCancelled`
            _)
          (:`EventReceived`
            (`/Engine/EditorBlueprintResources/StandardMacros.DoOnce` false :!label _label
              (:`Completed`
                (`self.Ability Work` _eventtag _eventdata :!label _label_2))))))
      (:`Is Not Valid`
        (goto _label_2))))
  (if (not (`self.bEndSpecified`))
    (`self.K2_EndAbility`)))

(event `self.K2_OnEndAbility`
  (params (bWasCancelled :type Boolean))
  (`self.OnAbilityEnded`))

(event `Ability Work`
  (params (Tag :type "GameplayTag Structure") (`Event data` :type "GameplayEventData Structure")))

(fn `GetOwningCharacter`
  (returns (Character :type "/Game/GProjectBP/Blueprints/BP_CharacterBase Object Reference"))
  (return (cast `/Game/GProjectBP/Blueprints/BP_CharacterBase` (`self.GetOwningActorFromActorInfo`) :!pure true)))