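; Player Pulse Bomb skill ability that throws a grenade from the character's left hand along the control rotation.
; On AbilityWork it builds an effect container spec from the tag and event data and passes it, with the aim direction as impulse, to a spawned BP_GrenadeBase_Child.
; The grenade's mesh and collision sphere ignore the owner while moving, and the ability ends immediately after spawning.
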(event `self.Ability Work`
  (params (Tag :type "GameplayTag Structure") (`Event data` :type "GameplayEventData Structure"))
  (bind _character (`self.GetOwningCharacter`))
  (bind _returnvalue (`Pawn.GetControlRotation` _character))
  (bind _returnvalue_2 (`self.MakeEffectContainerSpec` Tag `Event data`))
  (bind _returnvalue_3 (`|SpawnActorFromClass` "/Game/GProjectBP/Abilities/Character/Player/Skill/PulseBomb/BP_GrenadeBase_Child.BP_GrenadeBase_Child_C" (`KismetMathLibrary.MakeTransform` (`SceneComponent.GetSocketLocation` (`Character.Mesh` _character) "hand_lSoc") _returnvalue) "AlwaysSpawn" "OverrideRootScale" _character (`KismetMathLibrary.Conv_RotatorToVector` _returnvalue) _returnvalue_2 _character))
  (`PrimitiveComponent.IgnoreActorWhenMoving` (`/Game/GProjectBP/Abilities/Weapons/BP_RadialProjBase.StaticMesh` _returnvalue_3) (`self.GetOwningCharacter`) true)
  (`PrimitiveComponent.IgnoreActorWhenMoving` (`GPProjectileBase.SphereCollision` _returnvalue_3) (`self.GetOwningCharacter`) true)
  (`self.K2_EndAbility`))