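; Grenade projectile for the player's Pulse Bomb skill, derived from a grenade base class.
; On BeginPlay it launches its static mesh with a velocity-change impulse scaled by the projectile movement's initial speed.
; Projectile bounces with enough vertical speed spawn a small particle effect aligned to the surface.
; Detonation is tied to EndPlay, calling Explosion at the mesh's location with an upward normal.
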(event `self.ReceiveBeginPlay`
  (`parent.ReceiveBeginPlay`)
  (`PrimitiveComponent.AddImpulse` (`self.StaticMesh`) (* (`self.Impulse`) (`ProjectileMovementComponent.InitialSpeed` (`self.ProjMovementComp`))) "None" true))

(event `self.ReceiveTick`
  (params (DeltaSeconds :type "Float (single-precision)"))
  (`parent.ReceiveTick` DeltaSeconds))

(event `self.ReceiveEndPlay`
  (params (EndPlayReason :type "EEndPlayReason Enum" :default "Destroyed"))
  (`self.Explosion` (`SceneComponent.K2_GetComponentLocation` (`self.StaticMesh`)) (0.0 0.0 1.0)))

(event `self.ProjMovementComp.OnProjectileBounce`
  (params (ImpactResult :type "HitResult Structure (by ref)") (ImpactVelocity :type "Vector Structure (by ref)"))
  (bind (_bblockinghit _binitialoverlap _time _distance _location _impactpoint _normal _impactnormal) (`GameplayStatics.BreakHitResult` ImpactResult))
  (if (> (`KismetMathLibrary.Abs` (.z ImpactVelocity)) 300.0)
    (`GameplayStatics.SpawnEmitterAtLocation` "/Game/WeaponAssets/Temp/P_GrenadeBounce.P_GrenadeBounce" _location (`KismetMathLibrary.Conv_VectorToRotator` _impactnormal) (0.3 0.3 0.3))))

(fn `UserConstructionScript`
  (`parent.UserConstructionScript`))