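; Gameplay ability that lets a character use their current weapon, ending immediately if the weapon is missing or cannot activate.
; Single and Burst modes trigger the weapon once and end.
; Auto mode loops by waiting out the weapon's cooldown tag duration, playing its montage and re-firing once per montage event until activation fails.
; Ending the ability deactivates the weapon.
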(event `self.K2_ActivateAbility`
  (bind _currentweaponactor (`GPCharacterBase.CurrentWeaponActor` (`self.GetOwningCharacter`)))
  (`/Engine/EditorBlueprintResources/StandardMacros.IsValid` _currentweaponactor
    (:`Is Valid`
      (if (`GPWeaponActorBase.CanActivateWeapon` _currentweaponactor)
        (set `self.PlayingMontage` (`GPWeaponActorBase.WeaponAnimMontage` _currentweaponactor))
        (`parent.K2_ActivateAbility`)
        (else
          (`self.K2_EndAbility` :!label _label))))
    (:`Is Not Valid`
      (goto _label))))

(event `self.Ability Work`
  (params (Tag :type "GameplayTag Structure") (`Event data` :type "GameplayEventData Structure"))
  (bind _currentweaponactor (`GPCharacterBase.CurrentWeaponActor` (`self.GetOwningCharacter`)))
  (switch `EWFiringMode` (`GPWeaponActorBase.GetCurrentFiringMode` _currentweaponactor)
    (:`WM_Single`
      (`GPWeaponActorBase.TryActivateWeapon` _currentweaponactor :!label _label_2)
      (`self.K2_EndAbility`))
    (:`WM_Burst`
      (goto _label_2))
    (:`WM_Auto`
      (bind _returnvalue (`GPWeaponActorBase.TryActivateWeapon` _currentweaponactor))
      (`/Engine/EditorBlueprintResources/StandardMacros.IsValid` _returnvalue
        (:`Is Valid`
          (bind (_timeremaining _cooldownduration) (`GPAbilitySystemComponent.GetCooldownRemainingForTag` (cast `GPAbilitySystemComponent` (`AbilitySystemBlueprintLibrary.GetAbilitySystemComponent` _currentweaponactor) :!pure true) (struct :`GameplayTags` (struct :`(TagName` "Ability.Weapon")))))
          (`KismetSystemLibrary.Delay` _cooldownduration :!label _label_3)
          (`self.Client Play Montage`)
          (`GPAbilityTask_PlayMontage.PlayMontageAndWaitForEvent` "None" (`self.PlayingMontage`) (struct :`GameplayTags` (struct :`(TagName` "Event.Montage")))
            (:`then`
              (goto _label_4 :!via `Reset`))
            (:`EventReceived`
              (`/Engine/EditorBlueprintResources/StandardMacros.DoOnce` false :!label _label_4
                (:`Completed`
                  (bind _returnvalue_2 (`GPWeaponActorBase.TryActivateWeapon` (`GPCharacterBase.CurrentWeaponActor` (`self.GetOwningCharacter`))))
                  (`/Engine/EditorBlueprintResources/StandardMacros.IsValid` _returnvalue_2
                    (:`Is Valid`
                      (goto _label_3))
                    (:`Is Not Valid`
                      (`self.K2_EndAbility`))))))))
        (:`Is Not Valid`
          (`self.K2_EndAbility`))))))

(event `self.K2_OnEndAbility`
  (params (bWasCancelled :type Boolean))
  (bind _currentweaponactor (`GPCharacterBase.CurrentWeaponActor` (`self.GetOwningCharacter`)))
  (`/Engine/EditorBlueprintResources/StandardMacros.IsValid` _currentweaponactor
    (:`Is Valid`
      (`GPWeaponActorBase.DeactivateWeapon` _currentweaponactor))))