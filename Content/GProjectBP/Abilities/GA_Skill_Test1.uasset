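; GA_Skill_Test1 is a test gameplay ability that produces a radial blast around its owner.
; Once committed, it prints a debug message, gathers targets from each effect container and applies a radial velocity-change impulse to their mesh components.
; It spawns an explosion emitter at the owner's location and ends immediately, applying no gameplay effects from the containers to targets.
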(event `self.K2_ActivateAbility`
  (bind _returnvalue (`Actor.K2_GetActorLocation` (`.OwnerActor` (break `GameplayAbilityActorInfo` (`self.GetActorInfo`)))))
  (bind _returnvalue_2 (`self.K2_CommitAbility`))
  (if _returnvalue_2
    (`KismetSystemLibrary.PrintText` "Skill_Test1")
    (bind _values (`BlueprintMapLibrary.Map_Values` (`self.EffectContainerMap`)))
    (for _array_element _values
      (bind (_outhitresults _outtargetactors _returnvalue_3) (`self.GetTargetsFromEffectContainer` _array_element (make `GameplayEventData` (struct))))
      (if _returnvalue_3
        (for (_array_element_2 _array_index) _outtargetactors
          (for _array_element_3 (`Actor.K2_GetComponentsByClass` _array_element_2 "/Script/Engine.MeshComponent")
            (`PrimitiveComponent.AddRadialImpulse` _array_element_3 _returnvalue 500.0 2000.0 "RIF_Linear" true)))))
    (`GameplayStatics.SpawnEmitterAtLocation` "/Game/WeaponAssets/SciFiWeapDark/FX/Particles/P_RocketLauncher_Explosion_Dark.P_RocketLauncher_Explosion_Dark" _returnvalue)
    (`self.K2_EndAbility`)
    (else
      (`self.K2_EndAbility`))))