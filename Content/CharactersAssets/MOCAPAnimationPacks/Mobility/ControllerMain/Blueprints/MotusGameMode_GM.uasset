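; Game mode that handles mission start and completion presentation for the Motus controller content.
; On BeginPlay it uses the HUD manager to show the HP bar, crosshair and a "Mission start" notification.
; MissionComplete shows a countdown widget and sets a timer to ReturnToSetup.
; That event turns off custom depth on player meshes, animates the PC_PixelData Alpha parameter via timeline, then creates a black screen, with no level travel here.
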(event `self.ReceiveBeginPlay`
  (bind _hud_manager (`/Game/ProHUDV2/Blueprints/Libraries/BP_PHV2_Functions.GetHUDManager`))
  (message `/Game/ProHUDV2/Blueprints/Libraries/BPi_HUDManagerV2.CreateHUD` (`KismetSystemLibrary.Conv_InterfaceToObject` _hud_manager) 0)
  (`/Game/ProHUDV2/Blueprints/Libraries/BPi_HUDManagerV2.Show HP Bar` _hud_manager)
  (`self.Multicast Mission Start noti`))

(event `Multicast Mission Start noti`
  (bind _hud_manager (`/Game/ProHUDV2/Blueprints/Libraries/BP_PHV2_Functions.GetHUDManager`))
  (bind _hud_manager_2 (`/Game/ProHUDV2/Blueprints/Libraries/BP_PHV2_Functions.GetHUDManager`))
  (`/Game/ProHUDV2/Blueprints/Libraries/BPi_HUDManagerV2.CreateHUD` _hud_manager_2 0)
  (`/Game/ProHUDV2/Blueprints/Libraries/BPi_HUDManagerV2.CreatePrimaryNotification` _hud_manager_2 (make `/Game/ProHUDV2/Blueprints/Structs/S_PrimaryNotiInfo` "Mission start" (make `/Game/ProHUDV2/Blueprints/Structs/S_TextInfo` true (make `SlateFontInfo` "/Game/ProHUDV2/DemoContent/Fonts/BarlowCondensed/F_Barlow_Condensed.F_Barlow_Condensed" null (struct :`OutlineColor` (struct :`A` 1.0)) "FF_BarlowCondensed-Regular" 30) 1.0 (struct :`R` 0.59375 :`G` 0.59375 :`B` 0.59375 :`A` 1.0)) "Complete mission objects and return" (make `/Game/ProHUDV2/Blueprints/Structs/S_TextInfo` true (make `SlateFontInfo` "/Game/ProHUDV2/DemoContent/Fonts/BarlowCondensed/F_Barlow_Condensed.F_Barlow_Condensed" null (struct :`OutlineColor` (struct :`A` 1.0)) "FF_BarlowCondensed-Regular" 30) 1.0 (struct :`R` 1.0 :`G` 1.0 :`B` 1.0 :`A` 1.0)) (struct :`Transform` (struct :`Translation` (0.0 0.0) :`Scale` (1.0 1.0) :`Shear` (0.0 0.0)) :`IconColor` (struct)) (struct :`R` 1.0 :`G` 1.0 :`B` 1.0 :`A` 0.7) 5.0))
  (`/Game/ProHUDV2/Blueprints/Libraries/BPi_HUDManagerV2.AddCrosshair` _hud_manager "NewEnumerator0" (make `/Game/ProHUDV2/Blueprints/Structs/S_CrosshairInfo` (96.0 96.0) 12.0 (struct :`R` 1.0 :`G` 1.0 :`B` 1.0 :`A` 1.0) (1.0 1.0) 0.1))
  (`/Game/ProHUDV2/Blueprints/Libraries/BPi_HUDManagerV2.Show HP Bar` _hud_manager))

(event `Mission Complete`
  (`KismetSystemLibrary.K2_SetTimerDelegate` (delegate `Return to setup`) 10.0)
  (bind _returnvalue (`|CreateWidget` "/Game/GProjectBP/Blueprints/WidgetBP/HUD/WB_HUD_Countdown.WB_HUD_Countdown_C"))
  (`UserWidget.AddToViewport` _returnvalue 0))

(event `Return to setup`
  (bind _outactors (`GameplayStatics.GetAllActorsOfClass` "/Game/GProjectBP/Blueprints/BP_PlayerCharacter.BP_PlayerCharacter_C"))
  (for _array_element _outactors
    (`PrimitiveComponent.SetRenderCustomDepth` (`Character.Mesh` _array_element) false))
  (bind (_direction _alpha) (`Timeline|Timeline_0` :!via `PlayFromStart`)
    (:`Update`
      (`KismetMaterialLibrary.SetScalarParameterValue` "/Game/FXAssets/PixelSort/Youtube_Tutorial/PC_PixelData.PC_PixelData" "Alpha" _alpha))
    (:`Finished`
      (`/Game/ProHUDV2/Blueprints/Libraries/BPi_HUDManagerV2.CreateHUDFX_Blackscreen` (`/Game/ProHUDV2/Blueprints/Libraries/BP_PHV2_Functions.GetHUDManager`) 1.0))))

(fn `UserConstructionScript`)