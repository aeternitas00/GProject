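; Player controller for the Motus mocap character, turning input into camera control, locomotion state flags and weapon montages.
; Sprint key presses and timed holds switch jogging and running, alongside crouch and jump flags, with the AnimBP clearing Jumping.
; Movement axes feed constant-scale, control-yaw-relative input with a gamepad angle check for backward strafing, while Tick smoothly rotates the moving character.
; Weapon actions pick aim, fire and swap montages from the character's WeaponState.
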(event `InputAction|SprintOrRoll`
  (params (Key :type "Key Structure"))
  (bind _returnvalue (`self.IsInputKeyDown` (`self.RunKey`)))
  ;[1 1 1] Running/Jogging - Run is a held down key. This logic checks to ensure the key is held down (if currently jogging) long enough to enter run mode. If the key is released during any point before required time, player will leave jog state and not enter run state
  (:`Pressed`
    (`|ExecutionSequence`
      (:`then_0`
        (`/Engine/EditorBlueprintResources/StandardMacros.DoOnce` false ; Only need to set this key once, the first time it's pressed
          (:`Completed`
            (set `self.RunKey` Key))))
      (:`then_1`
        (if (not (`self.bCrouching`))
          (if (`self.bJogging`)
            (`KismetSystemLibrary.Delay` 0.3)
            (if _returnvalue
              (`KismetSystemLibrary.Delay` 0.3)
              (if _returnvalue
                (`KismetSystemLibrary.Delay` 0.3)
                (if (not _returnvalue)
                  (set `self.bJogging` false :!label _label))
                (else
                  (goto _label)))
              (else
                (goto _label)))
            (elif (`self.bRunning`)
              (set `self.bRunning` false)
              (else
                (set `self.bJogging` true)))))))))

(event `InputAction|Jump`
  (params (Key :type "Key Structure"))
  ;[1 1 1] Jumping
  (:`Pressed`
    (if (and (not (`self.bCrouching`)) (not (`self.bJumping`)))
      (set `self.bJumping` true) ; We only Set jumping here. It is set to false via ABP
    )))

(event `self.ReceiveBeginPlay`
  ;[1 1 1] Begin Play
  (set `self.CharacterReference` (cast `/Game/CharactersAssets/MOCAPAnimationPacks/Mobility/ControllerMain/Blueprints/MotusCharacter_BP` (`self.K2_GetPawn`) :!pure true)))

(event `InputAxis|LookUpRate`
  (params (AxisValue :type "Float (single-precision)"))
  ;[1 1 1] Camera Controls - Gamepad
  (`self.AddPitchInput` (* AxisValue (`GameplayStatics.GetWorldDeltaSeconds`) (`self.LookUpRate`))))

(event `InputAction|Crouch`
  (params (Key :type "Key Structure"))
  ;[1 1 1] Crouching
  (:`Pressed`
    (if (not (`self.bRunning`))
      (`/Engine/EditorBlueprintResources/StandardMacros.FlipFlop` :!label _label_2
        (:`A`
          (set `self.bCrouching` true)
          (set `self.bJogging` false)
          (set `self.bRunning` false))
        (:`B`
          (set `self.bCrouching` false)))
      (elif (`KismetMathLibrary.NearlyEqual_FloatFloat` (`KismetMathLibrary.VSize` (`self.GetVelocity` (`self.CharacterReference`))) 0.0 20.0)
        (goto _label_2)))))

(event `InputAxis|TurnRate`
  (params (AxisValue :type "Float (single-precision)"))
  ;[1 1 1] Camera Controls - Gamepad
  (`self.AddYawInput` (* AxisValue (`GameplayStatics.GetWorldDeltaSeconds`) (`self.TurnRate`))))

(event `InputAxis|MouseY`
  (params (AxisValue :type "Float (single-precision)"))
  ;[1 1 1] Camera Controls - Mouse
  (`self.AddPitchInput` AxisValue))

(event `self.ReceiveTick`
  (params (DeltaSeconds :type "Float (single-precision)"))
  (bind _runkey (`self.RunKey`))
  ;[1 1 1] Tick - Checks Run Key Held time and Sets Character Rotation While Moving
  (if (and (`self.IsInputKeyDown` _runkey) (>= (`self.GetInputKeyTimeDown` _runkey) 1.0) (not (`self.bRunning`)))
    (set `self.bRunning` true)
    (set `self.bIsAiming` false)
    (set `self.bJogging` false))
  (if (or (!= (`self.MoveForwardAxis`) 0.0) (!= (`self.MoveRightAxis`) 0.0))
    (`self.RotateYawWhileMoving`) ; Rotate Yaw of Character only while moving
  ))

(event `InputAxis|MouseX`
  (params (AxisValue :type "Float (single-precision)"))
  ;[1 1 1] Camera Controls - Mouse
  (`self.AddYawInput` AxisValue))

(event `InputAxis|MoveForward`
  (params (AxisValue :type "Float (single-precision)"))
  (bind _forwardvector (`self.GetCharacterVectors`))
  (bind _characterreference (`self.CharacterReference`))
  (bind _moveforwardaxis (`self.MoveForwardAxis`))
  (bind _returnvalue (`KismetMathLibrary.Abs` (`KismetMathLibrary.DegAtan2` (`self.MoveRightAxis`) (`self.MoveForwardAxis`))))
  ;[1 1 1] Move Forward/Backward
  (set `self.MoveForwardAxis` AxisValue)
  (if (> _moveforwardaxis 0.0)
    (`Pawn.AddMovementInput` _characterreference _forwardvector 1.0 false :!label _label_3) ; Apply constant scale value if moving forward
    (set `self.bMovingForward` true)
    (set `self.bMovingBackward` false)
    (elif (and (< _moveforwardaxis 0.0) (> _returnvalue 120.0) (<= _returnvalue 180.0))
      (`Pawn.AddMovementInput` _characterreference _forwardvector -1.0 false :!label _label_4) ; Apply constant scale value if moving backward
      (set `self.bMovingForward` false)
      (set `self.bMovingBackward` true)
      (elif (== (`self.MoveRightAxis`) 0.0)
        (if (`self.bMovingForward`)
          (goto _label_3)
          (elif (`self.bMovingBackward`)
            (goto _label_4)))
        (else
          (`Pawn.AddMovementInput` _characterreference _forwardvector 0.0 false :!label _label_5) ; Not moving so set scale to 0
          (set `self.bMovingForward` false)
          (set `self.bMovingBackward` false))))))

(event `StopMoveInputs`
  (`|ExecutionSequence`
    (:`then_0`
      (goto _label_5))
    (:`then_1`
      ;[1 1 1] Move Left/Right
      (`Pawn.AddMovementInput` (`self.CharacterReference`) (`.RightVector` (`self.GetCharacterVectors`)) 0.0 false :!label _label_6) ; Set scale to 0 when not moving Left/Right
      (set `self.bMovingRight` false)
      (set `self.bMovingLeft` false))))

(event `InputAxis|MoveRight`
  (params (AxisValue :type "Float (single-precision)"))
  (bind (_forwardvector _rightvector) (`self.GetCharacterVectors`))
  (bind _characterreference (`self.CharacterReference`))
  (bind _moverightaxis (`self.MoveRightAxis`))
  ;[1 1 1] Move Left/Right
  (set `self.MoveRightAxis` AxisValue)
  (if (> _moverightaxis 0.0)
    (`Pawn.AddMovementInput` _characterreference _rightvector 1.0 false :!label _label_7) ; Apply constant scale to Move Right
    (set `self.bMovingRight` true)
    (set `self.bMovingLeft` false)
    (elif (< _moverightaxis 0.0)
      (`Pawn.AddMovementInput` _characterreference _rightvector -1.0 false :!label _label_8) ; Apply constant scale to Move Left
      (set `self.bMovingRight` false)
      (set `self.bMovingLeft` true)
      (elif (== (`self.MoveForwardAxis`) 0.0)
        (if (`self.bMovingRight`)
          (goto _label_7)
          (elif (`self.bMovingLeft`)
            (goto _label_8)))
        (else
          (goto _label_6))))))

(event `InputAction|Weapon1Select`
  (params (Key :type "Key Structure"))
  (:`Pressed`
    (`self.PlayPreferSwapMontage` "NewEnumerator1")))

(event `InputAction|HandSelect`
  (params (Key :type "Key Structure"))
  (:`Pressed`
    (`self.PlayPreferSwapMontage` "NewEnumerator0")))

(event `InputAction|Weapon2Select`
  (params (Key :type "Key Structure"))
  (:`Pressed`
    (`self.PlayPreferSwapMontage` "NewEnumerator2")))

(event `InputAction|FireWeapon`
  (params (Key :type "Key Structure"))
  (:`Pressed`
    (`self.PlayPreferFireMontage`)))

(event `InputAction|UseOptic`
  (params (Key :type "Key Structure"))
  (bind _bcrouching (`self.bCrouching`))
  (:`Pressed`
    (`Character.PlayAnimMontage` (`self.CharacterReference`) (select `/Game/CharactersAssets/MOCAPAnimationPacks/Mobility/ControllerMain/Blueprints/WeaponState` (`/Game/CharactersAssets/MOCAPAnimationPacks/Mobility/ControllerMain/Blueprints/MotusCharacter_BP.WeaponState` (`self.CharacterReference`)) :`NewEnumerator1` (select `bool` _bcrouching :`false` "/Game/GProjectBP/Animation/Montage/MOCAP/AM_Aim_Stand_W1.AM_Aim_Stand_W1" :`true` "/Game/GProjectBP/Animation/Montage/MOCAP/AM_Aim_Crouch_W1.AM_Aim_Crouch_W1" :!type "AnimMontage Object Reference") :`NewEnumerator2` (select `bool` _bcrouching :`false` "/Game/GProjectBP/Animation/Montage/MOCAP/AM_Aim_Stand_W2.AM_Aim_Stand_W2" :`true` "/Game/GProjectBP/Animation/Montage/MOCAP/AM_Aim_Crouch_W2.AM_Aim_Crouch_W2" :!type "AnimMontage Object Reference")) 1.0 (select `bool` (`self.bIsAiming`) :`false` "Default" :`true` "Reverse" :!type "Name"))))

(fn `GetCharacterVectors`
  (returns (ForwardVector :type "Vector Structure") (RightVector :type "Vector Structure"))
  (bind _returnvalue (`KismetMathLibrary.MakeRotator` 0.0 0.0 (.yaw (`Pawn.GetControlRotation` (`self.CharacterReference`)))))
  (return (`KismetMathLibrary.GetForwardVector` _returnvalue) (`KismetMathLibrary.GetRightVector` _returnvalue)))

(fn `PlayPreferFireMontage`
  (locals (Aimed :type Name))
  (`KismetSystemLibrary.PrintString` "Hello")
  (set `local.Aimed` (select `bool` (`self.bIsAiming`) :`false` "Default" :`true` "Aimed" :!type "Name"))
  (switch `/Game/CharactersAssets/MOCAPAnimationPacks/Mobility/ControllerMain/Blueprints/WeaponState` (`/Game/CharactersAssets/MOCAPAnimationPacks/Mobility/ControllerMain/Blueprints/MotusCharacter_BP.WeaponState` (`self.CharacterReference`))
    (:`NewEnumerator1`
      (`Character.PlayAnimMontage` (`self.CharacterReference`) "/Game/GProjectBP/Animation/Montage/MOCAP/AM_FireWeapon_Stand_W1.AM_FireWeapon_Stand_W1" 1.0 "None"))
    (:`NewEnumerator2`
      (`Character.PlayAnimMontage` (`self.CharacterReference`) "/Game/GProjectBP/Animation/Montage/MOCAP/AM_FireWeapon_Stand_W2.AM_FireWeapon_Stand_W2" 1.0 "None"))))

(fn `PlayPreferSwapMontage`
  (params (To :type "/Game/CharactersAssets/MOCAPAnimationPacks/Mobility/ControllerMain/Blueprints/WeaponState Enum" :default "NewEnumerator0"))
  (locals (Aimed :type Name))
  (bind _characterreference (`self.CharacterReference`))
  (bind _aimed (`local.Aimed`))
  (bind _weaponstate (`/Game/CharactersAssets/MOCAPAnimationPacks/Mobility/ControllerMain/Blueprints/MotusCharacter_BP.WeaponState` (`self.CharacterReference`)))
  (`KismetSystemLibrary.PrintString` "Hello")
  (set `local.Aimed` (select `bool` (`self.bIsAiming`) :`false` "Default" :`true` "Aimed" :!type "Name"))
  (switch `/Game/CharactersAssets/MOCAPAnimationPacks/Mobility/ControllerMain/Blueprints/WeaponState` To
    (:`NewEnumerator0`
      (`Character.PlayAnimMontage` _characterreference (select `/Game/CharactersAssets/MOCAPAnimationPacks/Mobility/ControllerMain/Blueprints/WeaponState` _weaponstate :`NewEnumerator1` "/Game/GProjectBP/Animation/Montage/MOCAP/AM_SwapWeapon_Stand_W1_to_H.AM_SwapWeapon_Stand_W1_to_H" :`NewEnumerator2` "/Game/GProjectBP/Animation/Montage/MOCAP/AM_SwapWeapon_Stand_W2_to_H.AM_SwapWeapon_Stand_W2_to_H" :!type "AnimMontage Object Reference") 1.0 _aimed))
    (:`NewEnumerator1`
      (`Character.PlayAnimMontage` _characterreference (select `/Game/CharactersAssets/MOCAPAnimationPacks/Mobility/ControllerMain/Blueprints/WeaponState` _weaponstate :`NewEnumerator0` "/Game/GProjectBP/Animation/Montage/MOCAP/AM_SwapWeapon_Stand_H_to_W1.AM_SwapWeapon_Stand_H_to_W1" :`NewEnumerator2` "/Game/GProjectBP/Animation/Montage/MOCAP/AM_SwapWeapon_Stand_W2_to_W1.AM_SwapWeapon_Stand_W2_to_W1" :!type "AnimMontage Object Reference") 1.0 _aimed))
    (:`NewEnumerator2`
      (`Character.PlayAnimMontage` (`self.CharacterReference`) (select `/Game/CharactersAssets/MOCAPAnimationPacks/Mobility/ControllerMain/Blueprints/WeaponState` _weaponstate :`NewEnumerator0` "/Game/GProjectBP/Animation/Montage/MOCAP/AM_SwapWeapon_Stand_H_to_W2.AM_SwapWeapon_Stand_H_to_W2" :`NewEnumerator1` "/Game/GProjectBP/Animation/Montage/MOCAP/AM_SwapWeapon_Stand_W1_to_W2.AM_SwapWeapon_Stand_W1_to_W2" :!type "AnimMontage Object Reference") 1.0 _aimed))))

(fn `RotateYawWhileMoving`
  (`self.K2_SetActorRotation` (`self.CharacterReference`) (`KismetMathLibrary.RInterpTo_Constant` (`self.K2_GetActorRotation` (`self.CharacterReference`)) (`KismetMathLibrary.MakeRotator` 0.0 0.0 (.yaw (`self.GetDesiredRotation`))) (`GameplayStatics.GetWorldDeltaSeconds`) (`KismetMathLibrary.SelectFloat` 166.0 100.0 (`self.bMovingTurn`))) false)
  (return))

(fn `UserConstructionScript`)