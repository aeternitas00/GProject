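; BP_CompassArea is a ProHUDV2 demo trigger volume that shows the HUD compass while the player character is inside it.
; Box overlap events filter for HUD_Character and tell the HUD manager to show the compass on entry.
; On exit it hides the compass, removes all compass markers, and calls UpdateMarker(false) on every BP_DemoTrigger_Marker found in the level.
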(event `self.Box.OnComponentBeginOverlap`
  (params (OverlappedComponent :type "PrimitiveComponent Object Reference") (OtherActor :type "Actor Object Reference") (OtherComp :type "PrimitiveComponent Object Reference") (OtherBodyIndex :type Integer) (bFromSweep :type Boolean) (SweepResult :type "HitResult Structure (by ref)"))
  (cast `/Game/ProHUDV2/DemoContent/DemoCharacter/HUD_Character` OtherActor)
  (`/Game/ProHUDV2/Blueprints/Libraries/BPi_HUDManagerV2.ShowCompass` (`/Game/ProHUDV2/Blueprints/Libraries/BP_PHV2_Functions.GetHUDManager`)))

(event `self.Box.OnComponentEndOverlap`
  (params (OverlappedComponent :type "PrimitiveComponent Object Reference") (OtherActor :type "Actor Object Reference") (OtherComp :type "PrimitiveComponent Object Reference") (OtherBodyIndex :type Integer))
  (bind _hud_manager (`/Game/ProHUDV2/Blueprints/Libraries/BP_PHV2_Functions.GetHUDManager`))
  (cast `/Game/ProHUDV2/DemoContent/DemoCharacter/HUD_Character` OtherActor)
  (`/Game/ProHUDV2/Blueprints/Libraries/BPi_HUDManagerV2.HideCompass` _hud_manager)
  (`/Game/ProHUDV2/Blueprints/Libraries/BPi_HUDManagerV2.RemoveAllCompassMarkers` _hud_manager)
  (bind _outactors (`GameplayStatics.GetAllActorsOfClass` "/Game/ProHUDV2/DemoContent/DemoRoom/DemoTrigger/BP_DemoTrigger_Marker.BP_DemoTrigger_Marker_C"))
  (for _array_element _outactors
    (`/Engine/EditorBlueprintResources/StandardMacros.IsValid` _array_element
      (:`Is Valid`
        (`/Game/ProHUDV2/DemoContent/DemoRoom/DemoTrigger/BP_DemoTrigger_Marker.UpdateMarker` _array_element false)))))

(fn `UserConstructionScript`)