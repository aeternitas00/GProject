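; BP_Crosshair_Demo is a ProHUDV2 demo actor that switches the player's crosshair when an HUD_Character enters its box.
; The CrosshairV1 flag picks the V1 or current HUD manager API, adding that crosshair and removing the other system's.
; The current branch also updates the crosshair with UseMovementStrength and flashes a point light briefly.
; On exit, it again removes the opposite system's crosshair, leaving the added one active.
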(event `self.Box.OnComponentBeginOverlap`
  (params (OverlappedComponent :type "PrimitiveComponent Object Reference") (OtherActor :type "Actor Object Reference") (OtherComp :type "PrimitiveComponent Object Reference") (OtherBodyIndex :type Integer) (bFromSweep :type Boolean) (SweepResult :type "HitResult Structure (by ref)"))
  (bind _hud_manager (`/Game/ProHUDV2/Blueprints/Libraries/BP_PHV2_Functions.GetHUDManager`))
  (bind _pointlight (`self.PointLight`))
  (cast `/Game/ProHUDV2/DemoContent/DemoCharacter/HUD_Character` OtherActor)
  (if (`self.CrosshairV1`)
    (`/Game/ProHUDV2/Blueprints/Libraries/BPi_HUDManagerV2.V1_AddCrosshair` (`/Game/ProHUDV2/Blueprints/Libraries/BP_PHV2_Functions.GetHUDManager`) (`self.V1_Type`) (`self.V1_Color`) true)
    (`/Game/ProHUDV2/Blueprints/Libraries/BPi_HUDManagerV2.RemoveCrosshair` (`/Game/ProHUDV2/Blueprints/Libraries/BP_PHV2_Functions.GetHUDManager`))
    (else
      (`/Game/ProHUDV2/Blueprints/Libraries/BPi_HUDManagerV2.AddCrosshair` _hud_manager (`self.CrosshairType`) (`self.CrosshairInfo`))
      (`/Game/ProHUDV2/Blueprints/Libraries/BPi_HUDManagerV2.UpdateCrosshair` _hud_manager (`self.UseMovementStrength`))
      (`/Game/ProHUDV2/Blueprints/Libraries/BPi_HUDManagerV2.V1_RemoveCrosshair` (`/Game/ProHUDV2/Blueprints/Libraries/BP_PHV2_Functions.GetHUDManager`))
      (`SceneComponent.SetVisibility` _pointlight true false)
      (`KismetSystemLibrary.Delay` 0.3)
      (`SceneComponent.SetVisibility` _pointlight false false))))

(event `self.Box.OnComponentEndOverlap`
  (params (OverlappedComponent :type "PrimitiveComponent Object Reference") (OtherActor :type "Actor Object Reference") (OtherComp :type "PrimitiveComponent Object Reference") (OtherBodyIndex :type Integer))
  (bind _hud_manager (`/Game/ProHUDV2/Blueprints/Libraries/BP_PHV2_Functions.GetHUDManager`))
  (cast `/Game/ProHUDV2/DemoContent/DemoCharacter/HUD_Character` OtherActor)
  (if (`self.CrosshairV1`)
    (`/Game/ProHUDV2/Blueprints/Libraries/BPi_HUDManagerV2.RemoveCrosshair` _hud_manager)
    (else
      (`/Game/ProHUDV2/Blueprints/Libraries/BPi_HUDManagerV2.V1_RemoveCrosshair` _hud_manager))))

(fn `UserConstructionScript`
  (locals (DynamicMaterial :type "MaterialInstanceDynamic Object Reference")))